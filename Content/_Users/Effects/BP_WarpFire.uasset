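; Animated warp fire effect actor that pulses and spins two components, P1 and P2, alongside two particle systems.
; Each tick, two looping timers feed triangle waves, blended differently per component to drive Z stretch and yaw speed.
; The timers also set each particle system's Alpha parameter.
; Stretch amplitude lerps between min and max as its rate moves linearly toward TargetScaleRate, which is never set here.
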(event EventTick
  (params (DeltaSeconds :type Float%20%28single-precision%29))
  (bind _p1 (Variables|Default|GetP1))
  (bind _p2 (Variables|Default|GetP2))
  (bind _returnvalue (Transformation|GetWorldRotation _p2))
  (bind _returnvalue_2 (Transformation|GetWorldRotation _p1))
  (Variables|Default|Seta (CallFunction|AddValue (Variables|Default|Geta) (Variables|Default|GetAMax)))
  (Variables|Default|Setb (CallFunction|AddValue (Variables|Default|Getb) (Variables|Default|GetBMax)))
  (Transformation|SetWorldScale3D (Variables|Default|GetP1) (+ (Variables|Default|GetDefScale) (Math|Vector|MakeVector 0.0 0.0 (* (Math|Float|MakeLiteralFloat 0.1) (/ (+ (CallFunction|Calculate (Variables|Default|Geta) (Variables|Default|GetAMax)) (CallFunction|Calculate (Variables|Default|Getb) (Variables|Default|GetBMax))) 2.0) (Variables|Default|GetNowScale)))))
  (Transformation|SetWorldScale3D (Variables|Default|GetP2) (+ (Variables|Default|GetDefScale) (Math|Vector|MakeVector 0.0 0.0 (* (Math|Float|MakeLiteralFloat 0.1) (/ (+ (- 1.0 (CallFunction|Calculate (Variables|Default|Geta) (Variables|Default|GetAMax))) (CallFunction|Calculate (Variables|Default|Getb) (Variables|Default|GetBMax))) 2.0) (Variables|Default|GetNowScale)))))
  (Effects|Components|ParticleSystem|SetFloatParameter (Variables|Default|GetParticleSystem1) "Alpha" (+ (Variables|Default|Geta) (Variables|Default|Getb)))
  (Effects|Components|ParticleSystem|SetFloatParameter (Variables|Default|GetParticleSystem2) "Alpha" (CallFunction|Calculate (+ (Variables|Default|Geta) (Variables|Default|Getb)) (+ (Variables|Default|GetAMax) (Variables|Default|GetBMax))))
  (Transformation|SetWorldRotation _p1 (Math|Rotator|MakeRotator (.roll _returnvalue_2) (.pitch _returnvalue_2) (Math|Float|%(Float) (+ (.yaw _returnvalue_2) (* (Utilities|Time|GetWorldDeltaSeconds) (+ (- 1.0 (CallFunction|Calculate (Variables|Default|Geta) (Variables|Default|GetAMax))) (CallFunction|Calculate (Variables|Default|Getb) (Variables|Default|GetBMax))) 1e+02)) 3.6e+02)) false false)
  (Transformation|SetWorldRotation _p2 (Math|Rotator|MakeRotator (.roll _returnvalue) (.pitch _returnvalue) (Math|Float|%(Float) (+ (.yaw _returnvalue) (* (Utilities|Time|GetWorldDeltaSeconds) (CallFunction|Calculate (+ (Variables|Default|Geta) (Variables|Default|Getb)) (+ (Variables|Default|GetAMax) (Variables|Default|GetBMax))) 2e+02)) 3.6e+02)) false false)
  (CallFunction|UpdateRate)
  (Variables|Default|SetNowScale (Math|Float|Lerp (Variables|Default|GetMinScale) (Variables|Default|GetMaxScale) (Variables|Default|GetNowScaleRate))))

(event EventBeginPlay
  (Variables|Default|SetDefScale (Transformation|GetActorScale3D)))

(fn ConstructionScript)

(fn AddValue
  (params (NowValue :type Float%20%28single-precision%29) (Max :type Float%20%28single-precision%29))
  (return (Math|Float|%(Float) (+ NowValue (Utilities|Time|GetWorldDeltaSeconds)) Max)))

(fn Calculate
  (params (Value :type Float%20%28single-precision%29) (Max :type Float%20%28single-precision%29))
  (return (Math|Float|Absolute(Float) (- 1.0 (/ Value (* Max 0.5))))))

(fn UpdateRate
  (if (> (Variables|Default|GetNowScaleRate) (Variables|Default|GetTargetScaleRate))
    (Variables|Default|SetNowScaleRate (Math|Float|Max(Float) (- (Variables|Default|GetNowScaleRate) (/ (Utilities|Time|GetWorldDeltaSeconds) (Variables|Default|GetMaxTime))) 0.0))
    (elif (< (Variables|Default|GetNowScaleRate) (Variables|Default|GetTargetScaleRate))
      (Variables|Default|SetNowScaleRate (Math|Float|Min(Float) (+ (Variables|Default|GetNowScaleRate) (/ (Utilities|Time|GetWorldDeltaSeconds) (Variables|Default|GetMaxTime))) 1.0)))))