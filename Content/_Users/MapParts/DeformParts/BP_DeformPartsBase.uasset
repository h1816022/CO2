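; BP_DeformPartsBase is, by its name, a base Blueprint for deform map parts, with a holographic visual that changes when its room is passed.
; On BeginPlay it creates a dynamic MI_Holo material on the ConflictCheckCollision component and stores the instance.
; The PassedThisRoom event sets that instance's color and opacity to the passed-state values.
; Its construction script only calls the parent implementation.
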(event Custom|PassedThisRoom
  (Rendering|Material|SetVectorParameterValue (Variables|Default|GetMaterials) "Color" (Variables|Default|GetPassedColor) :!class /Script/Engine.MaterialInstanceDynamic)
  (Rendering|Material|SetScalarParameterValue (Variables|Default|GetMaterials) "Opacity" (Variables|Default|GetPassedOpacity) :!class /Script/Engine.MaterialInstanceDynamic))

(event EventBeginPlay
  (bind _returnvalue (Rendering|Material|CreateDynamicMaterialInstance (Variables|Default|GetConflictCheckCollision) 0 "/Game/_Users/Materials/MI_Holo.MI_Holo" "None" :!class /Script/Engine.PrimitiveComponent))
  (Variables|Default|SetMaterials _returnvalue))

(fn ConstructionScript
  (|CallParentFunction))