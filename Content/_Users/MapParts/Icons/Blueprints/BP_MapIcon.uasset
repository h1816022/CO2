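; BP_MapIcon is a map icon built from two plane meshes that can be shown, hidden and switched between active and inactive looks.
; On BeginPlay it creates a second dynamic material instance for Plane1, then runs the parent's BeginPlay.
; ChangeVisibility toggles both planes together.
; ChangeColor sets the IsActive scalar parameter on both Material and Material2 to match the active state.
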(event EventChangeVisibility
  (params (bNewVisibility :type Boolean))
  (Rendering|SetVisibility (Variables|Default|GetPlane) bNewVisibility false)
  (Rendering|SetVisibility (Variables|Default|GetPlane1) bNewVisibility false))

(event EventBeginPlay
  (bind _plane1 (Variables|Default|GetPlane1))
  (bind _returnvalue (Rendering|Material|CreateDynamicMaterialInstance _plane1 0 (Rendering|Material|GetMaterial _plane1 0) "None" :!class /Script/Engine.PrimitiveComponent))
  (Variables|Default|SetMaterial2 _returnvalue)
  (|CallParentFunction))

(event EventChangeColor
  (params (bIsActive :type Boolean))
  (if bIsActive
    (Rendering|Material|SetScalarParameterValue (Variables|Default|GetMaterial) "IsActive" 1.0 :!class /Script/Engine.MaterialInstanceDynamic)
    (Rendering|Material|SetScalarParameterValue (Variables|Default|GetMaterial2) "IsActive" 1.0 :!class /Script/Engine.MaterialInstanceDynamic)
    (else
      (Rendering|Material|SetScalarParameterValue (Variables|Default|GetMaterial) "IsActive" 0.0 :!class /Script/Engine.MaterialInstanceDynamic)
      (Rendering|Material|SetScalarParameterValue (Variables|Default|GetMaterial2) "IsActive" 0.0 :!class /Script/Engine.MaterialInstanceDynamic))))

(fn ConstructionScript
  (|CallParentFunction))