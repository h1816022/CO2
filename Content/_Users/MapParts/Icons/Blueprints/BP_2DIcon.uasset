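; BP_2DIcon is a plane-based icon actor that turns every tick to face a referenced camera.
; Tick applies the camera-to-icon look-at rotation with a 90-degree yaw correction plus RotOffset.
; Rotate starts a timeline that drives RotOffset for a spin, replaying after a five-second pause.
; A dynamic material created on BeginPlay lets ChangeColor toggle the active look, while ChangeVisibility shows or hides the plane.
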(event Custom|Rotate
  (bind _newtrack_0 (Timeline|Timeline_0 PlayFromStart)
    (:Update
      (Variables|Default|SetRotOffset (* _newtrack_0 3.6e+02)))
    (:Finished
      (Utilities|FlowControl|Delay 5.0)
      (Timeline|Timeline_0 PlayFromStart))))

(event EventTick
  (params (DeltaSeconds :type Float%20%28single-precision%29))
  (bind _returnvalue (Transformation|GetActorLocation))
  (bind _camera (Variables|Default|GetCamera))
  (bind _camera_2 (Variables|/Game/_Users/Cameras/Blueprints/BP_MiniMapCamera.BP_MiniMapCamera_C|GetCamera _camera))
  (bind _returnvalue_2 (Transformation|GetWorldLocation _camera_2))
  (bind _returnvalue_3 (Math|Rotator|FindLookatRotation (Math|Vector|MakeVector (.x _returnvalue_2) (.y _returnvalue_2) 0.0) (Math|Vector|MakeVector (.x _returnvalue) (.y _returnvalue) 0.0)))
  (Transformation|SetActorRotation (Math|Rotator|MakeRotator (.roll _returnvalue_3) (.pitch _returnvalue_3) (+ (.yaw _returnvalue_3) 9e+01 (Variables|Default|GetRotOffset)))))

(event EventBeginPlay
  (bind _plane (Variables|Default|GetPlane))
  (|CallParentFunction)
  (bind _returnvalue (Rendering|Material|CreateDynamicMaterialInstance _plane 0 (Rendering|Material|GetMaterial _plane 0) "None" :!class /Script/Engine.PrimitiveComponent))
  (Variables|Default|SetMaterial _returnvalue))

(event EventChangeVisibility
  (params (bNewVisibility :type Boolean))
  (Rendering|SetVisibility (Variables|Default|GetPlane) bNewVisibility false))

(fn ConstructionScript)

(fn ChangeColor
  (params (bIsActive :type Boolean))
  (if bIsActive
    (Rendering|Material|SetScalarParameterValue (Variables|Default|GetMaterial) "bIsActive" 1.0 :!class /Script/Engine.MaterialInstanceDynamic)
    (else
      (Rendering|Material|SetScalarParameterValue (Variables|Default|GetMaterial) "bIsActive" 0.0 :!class /Script/Engine.MaterialInstanceDynamic))))