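; BP_3DIcon is a 3D map icon with a mesh and an arrow that turns to face the camera.
; Each Tick it sets the ArrowRoot world rotation to the look-at yaw toward the camera, with pitch and roll held at zero.
; A ChangeVisibility event shows or hides the Mesh and Arrow together, without propagating to their children.
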(event EventTick
  (params (DeltaSeconds :type Float%20%28single-precision%29))
  (Transformation|SetWorldRotation (Variables|Default|GetArrowRoot) (Math|Rotator|MakeRotator 0.0 0.0 (.yaw (Math|Rotator|FindLookatRotation (Transformation|GetWorldLocation (Variables|Default|GetArrowRoot)) (Transformation|GetWorldLocation (Variables|/Game/_Users/Cameras/Blueprints/BP_MiniMapCamera.BP_MiniMapCamera_C|GetCamera (Variables|Default|GetCamera)))))) false false))

(event EventChangeVisibility
  (params (bNewVisibility :type Boolean))
  (Rendering|SetVisibility (Variables|Default|GetMesh) bNewVisibility false)
  (Rendering|SetVisibility (Variables|Default|GetArrow) bNewVisibility false))

(fn ConstructionScript
  (|CallParentFunction))