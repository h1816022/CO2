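; BP_MiniMap is a 3D miniature map that the player views through a dedicated camera and can rotate and pan within clamped limits.
; Registered map parts are recentered on init, and world offsets scaled by 0.003 place player, enemy and device icons on them.
; A capped player trail of linked markers fades through material parameters, skipping spawns that overlap the previous marker.
; ConnectMap reveals parts and icons.
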(event Custom|AddParts
  (params (NewParts :type BP%20Map%20Parts%20Base%20Object%20Reference))
  (Utilities|Array|Add (Variables|Default|GetPartsArray) NewParts)
  (Utilities|Array|Add (Variables|Default|GetLocationDeff) (- (Transformation|GetActorLocation NewParts) (Transformation|GetActorLocation))))

(event Custom|EndView
  (Variables|Default|SetOffset "0, 0, 0")
  (Transformation|SetActorLocation (Variables|Default|GetDefaultLocation) false false)
  (Transformation|SetActorRotation "0, 0, 0")
  (Variables|Default|SetbIsView false))

(event Custom|StartView
  (params (Player :type BP%20Player%20Object%20Reference))
  (Variables|Default|SetbIsView true)
  (CallFunction|SetViewTarget)
  (CallFunction|AdjustRotation Player)
  (Variables|Default|SetOffset (- (Transformation|GetActorLocation) (Transformation|GetActorLocation (Variables|Default|GetPlayerIcon))))
  (CallFunction|AddOffset))

(event Custom|FirstInitMiniMap
  (CallFunction|AdjustDeff)
  (Utilities|FlowControl|Delay 0.2)
  (Variables|Default|SetbCanView true)
  (CallFunction|StartIconsRotate))

(fn ConstructionScript)

(fn AdjustDeff
  (LocalVariables|SetDiff (* (Math|Vector|GetVectorArrayAverage (Variables|Default|GetLocationDeff)) -1.0))
  (for _array_element (Variables|Default|GetPartsArray)
    (Transformation|AddActorWorldOffset _array_element (LocalVariables|GetDiff))
    (Variables|Default|SetDefaultLocation (Transformation|GetActorLocation))))

(fn UpdatePlayerLocation
  (params (Parts :type BP%20Map%20Parts%20Base%20Object%20Reference) (Diff :type Vector))
  (Transformation|SetWorldLocation (Variables|/Game/_Users/MapParts/Icons/Blueprints/BP_3DIcon.BP_3DIcon_C|GetMeshRoot (Variables|Default|GetPlayerIcon)) (+ (* Diff 0.003) (Transformation|GetActorLocation Parts)) false false))

(fn UpdateEnemyLocation
  (LocalVariables|SetPlayerLocation (Transformation|GetActorLocation (Game|Player|GetPlayerPawn 0)))
  (LocalVariables|SetPlayerIconLocation (Transformation|GetWorldLocation (Variables|/Game/_Users/MapParts/Icons/Blueprints/BP_3DIcon.BP_3DIcon_C|GetMeshRoot (Variables|Default|GetPlayerIcon))))
  (bind _outactors (Actor|GetAllActorsOfClass "/Game/_Users/Enemies/General/Blueprints/BP_Enemy.BP_Enemy_C"))
  (for (_array_element _array_index) _outactors
    (Transformation|SetWorldLocation (Variables|/Game/_Users/MapParts/Icons/Blueprints/BP_TankIcon.BP_TankIcon_C|GetMeshRoot (Utilities|Array|Get(acopy) (Variables|Default|GetEnemyIcons) _array_index)) (+ (* (- (Transformation|GetActorLocation _array_element) (LocalVariables|GetPlayerLocation)) 0.003) (LocalVariables|GetPlayerIconLocation)) false false)))

(fn SpawnIcon
  (params (MapParts :type BP%20Map%20Parts%20Base%20Object%20Reference) (Type :type ESpawnActorType%20Enum :default "NewEnumerator0") (MatchPoint :type BP%20Can%20Spawn%20Point%20Object%20Reference) (Device :type BP%20Device%20Base%20Object%20Reference))
  (bind _relativelocation (CallFunction|GetRelativeDeformLocation MapParts (Transformation|GetWorldLocation MatchPoint)))
  (switch Utilities|FlowControl|Switch|SwitchonESpawnActorType Type
    (:NewEnumerator0
      (bind _returnvalue (Game|SpawnActorfromClass "/Game/_Users/MapParts/Icons/Blueprints/BP_WaterSupplyIcon.BP_WaterSupplyIcon_C" (Math|Transform|MakeTransform _relativelocation "0, 0, 0" "1,1,1") "Undefined" 0 (Variables|Default|GetMiniMapCamera) 0))
      (Utilities|Array|Add (Variables|Default|GetIcons) _returnvalue)
      (bind _output_get (Variables|/Game/_Users/Blueprints/BP_DeviceBase.BP_DeviceBase_C|SetMyIcon Device _returnvalue))
      (Transformation|AttachActorToActor _output_get (Variables|/Game/_Users/MapParts/Parts/BP_MapPartsBase.BP_MapPartsBase_C|GetMyDeformParts MapParts) "None" "KeepWorld" "KeepWorld" "KeepRelative" true))
    (:NewEnumerator1
      (bind _returnvalue_2 (Game|SpawnActorfromClass "/Game/_Users/MapParts/Icons/Blueprints/BP_WarpIcon.BP_WarpIcon_C" (Math|Transform|MakeTransform _relativelocation "0, 0, 0" "1,1,1") "Undefined" 0 (Variables|Default|GetMiniMapCamera) 0))
      (Utilities|Array|Add (Variables|Default|GetIcons) _returnvalue_2)
      (bind _output_get_2 (Variables|/Game/_Users/Blueprints/BP_DeviceBase.BP_DeviceBase_C|SetMyIcon Device _returnvalue_2))
      (Transformation|AttachActorToActor _output_get_2 (Variables|/Game/_Users/MapParts/Parts/BP_MapPartsBase.BP_MapPartsBase_C|GetMyDeformParts MapParts) "None" "KeepWorld" "KeepWorld" "KeepRelative" true))
    (:NewEnumerator4
      (bind _returnvalue_3 (Game|SpawnActorfromClass "/Game/_Users/MapParts/Icons/Blueprints/BP_MapIcon.BP_MapIcon_C" (Math|Transform|MakeTransform _relativelocation "0, 0, 0" "1,1,1") "Undefined" 0 (Variables|Default|GetMiniMapCamera) 0))
      (Utilities|Array|Add (Variables|Default|GetIcons) _returnvalue_3)
      (bind _output_get_3 (Variables|/Game/_Users/Blueprints/BP_DeviceBase.BP_DeviceBase_C|SetMyIcon Device _returnvalue_3))
      (Transformation|AttachActorToActor _output_get_3 (Variables|/Game/_Users/MapParts/Parts/BP_MapPartsBase.BP_MapPartsBase_C|GetMyDeformParts MapParts) "None" "KeepWorld" "KeepWorld" "KeepRelative" true))))

(fn Rotate
  (params (Value :type Float%20%28single-precision%29))
  (bind _returnvalue (Transformation|GetActorRotation))
  (if (Variables|Default|GetbIsView)
    (Transformation|SetActorRotation (Math|Rotator|MakeRotator (.roll _returnvalue) (.pitch _returnvalue) (+ (.yaw _returnvalue) Value)))))

(fn MoveForward
  (params (Value :type Float%20%28single-precision%29))
  (if (Variables|Default|GetbIsView)
    (Variables|Default|SetOffset (Math|Vector|MakeVector (.x (Variables|Default|GetOffset)) (Math|Float|Clamp(Float) (+ (.y (Variables|Default|GetOffset)) (* Value 0.05)) -1e+01 1e+01) (.z (Variables|Default|GetOffset))))
    (CallFunction|AddOffset)))

(fn MoveRight
  (params (Value :type Float%20%28single-precision%29))
  (if (Variables|Default|GetbIsView)
    (Variables|Default|SetOffset (Math|Vector|MakeVector (Math|Float|Clamp(Float) (- (.x (Variables|Default|GetOffset)) (* Value 0.05)) -1e+01 1e+01) (.y (Variables|Default|GetOffset)) (.z (Variables|Default|GetOffset))))
    (CallFunction|AddOffset)))

(fn AddOffset
  (Transformation|SetActorLocation (+ (Variables|Default|GetDefaultLocation) (Variables|Default|GetOffset)) false false))

(fn UpdatePlayerTrajectory
  (params (Parts :type BP%20Map%20Parts%20Base%20Object%20Reference) (Diff :type Vector))
  (bind _returnvalue (Game|Player|GetPlayerPawn 0))
  (bind _trajectories (Variables|Default|GetTrajectories))
  (bind _asbp_player (Utilities|Casting|CastToBP_Player _returnvalue))
  (Utilities|IsValid (Variables|/Game/_Users/Players/Blueprints/BP_Player.BP_Player_C|GetCamera (.AsBP%20Player (Utilities|Casting|CastToBP_Player (Game|Player|GetPlayerPawn 0))))
    (:Is%20Valid
      (bind _returnvalue_2 (Game|SpawnActorfromClass "/Game/_Users/MapParts/BP_PlayerTrajectory.BP_PlayerTrajectory_C" (Math|Transform|MakeTransform (+ (Transformation|GetActorLocation Parts) (* Diff 0.003)) (Math|Rotator|MakeRotator 0.0 0.0 (+ (.yaw (Math|Conversions|RotationFromXVector (Variables|/Game/_Users/Players/Blueprints/BP_Player.BP_Player_C|GetInputVec _asbp_player))) (.yaw (Transformation|GetWorldRotation (Variables|/Game/_Users/Cameras/Blueprints/BP_PlayerCamera.BP_PlayerCamera_C|GetThirdCameraArm (Variables|/Game/_Users/Players/Blueprints/BP_Player.BP_Player_C|GetCamera _asbp_player)))))) "0.002000,0.002000,0.002000") "Undefined" 0 (Variables|Default|GetNewTrajectory) 0 0))
      (if (not (CallFunction|CheckCollision _returnvalue_2))
        (Utilities|IsValid (Variables|Default|GetNewTrajectory)
          (:Is%20Valid
            (Variables|/Game/_Users/MapParts/BP_PlayerTrajectory.BP_PlayerTrajectory_C|SetNext (Variables|Default|GetNewTrajectory) _returnvalue_2))
          (:Is%20Not%20Valid
            _))
        (Variables|Default|SetNewTrajectory _returnvalue_2)
        (Transformation|AttachActorToActor (Variables|Default|GetNewTrajectory) self "None" "KeepWorld" "KeepWorld" "KeepRelative" true)
        (for _array_element (Variables|Default|GetTrajectories)
          (bind _returnvalue_3 (Rendering|Material|GetScalarParameterValue (Variables|/Game/_Users/MapParts/BP_PlayerTrajectory.BP_PlayerTrajectory_C|GetMaterial _array_element) "Opacity" :!class /Script/Engine.MaterialInstanceDynamic))
          (Rendering|Material|SetScalarParameterValue (Variables|/Game/_Users/MapParts/BP_PlayerTrajectory.BP_PlayerTrajectory_C|GetMaterial _array_element) "Opacity" (- _returnvalue_3 (/ 1.0 (Math|Conversions|ToFloat(Integer) (LocalVariables|GetMaxNum)))) :!class /Script/Engine.MaterialInstanceDynamic)
          (bind _returnvalue_4 (Rendering|Material|GetScalarParameterValue (Variables|/Game/_Users/MapParts/BP_PlayerTrajectory.BP_PlayerTrajectory_C|GetMaterial _array_element) "Rate" :!class /Script/Engine.MaterialInstanceDynamic))
          (Rendering|Material|SetScalarParameterValue (Variables|/Game/_Users/MapParts/BP_PlayerTrajectory.BP_PlayerTrajectory_C|GetMaterial _array_element) "Rate" (* _returnvalue_4 0.995) :!class /Script/Engine.MaterialInstanceDynamic)
          (bind _returnvalue_5 (Rendering|Material|GetScalarParameterValue (Variables|/Game/_Users/MapParts/BP_PlayerTrajectory.BP_PlayerTrajectory_C|GetMaterial _array_element) "IsActive" :!class /Script/Engine.MaterialInstanceDynamic))
          (Rendering|Material|SetScalarParameterValue (Variables|/Game/_Users/MapParts/BP_PlayerTrajectory.BP_PlayerTrajectory_C|GetMaterial _array_element) "IsActive" (Math|Float|Clamp(Float) (- _returnvalue_5 (/ 1.0 (Math|Conversions|ToFloat(Integer) (LocalVariables|GetMaxNum))))) :!class /Script/Engine.MaterialInstanceDynamic))
        (if (> (Utilities|Array|Length (Variables|Default|GetTrajectories)) (LocalVariables|GetMaxNum))
          (Actor|DestroyActor (Utilities|Array|Get(acopy) _trajectories))
          (Utilities|Array|RemoveIndex _trajectories))
        (Utilities|Array|Add (Variables|Default|GetTrajectories) (Variables|Default|GetNewTrajectory))
        (else
          (Actor|DestroyActor _returnvalue_2))))))

(fn SetViewTarget
  (Game|Player|SetViewTargetwithBlend (Game|GetPlayerController 0) (Variables|Default|GetMiniMapCamera) 0.0 "VTBlend_Linear" 0.0 false))

(fn AdjustRotation
  (params (Player :type BP%20Player%20Object%20Reference))
  (Transformation|SetActorRotation (Math|Rotator|MakeRotator 0.0 0.0 (- (.yaw (Transformation|GetActorRotation (Variables|Default|GetMiniMapCamera))) (.yaw (Transformation|GetWorldRotation (Variables|/Game/_Users/Cameras/Blueprints/BP_PlayerCamera.BP_PlayerCamera_C|GetThirdCamera (Variables|/Game/_Users/Players/Blueprints/BP_Player.BP_Player_C|GetCamera Player))))))))

(fn CheckCollision
  (params (CheckTrajectory :type BP%20Player%20Trajectory%20Object%20Reference))
  (bind _array_element (Utilities|Array|ForEachLoopwithBreak (Collision|GetOverlappingActors (Variables|/Game/_Users/MapParts/BP_PlayerTrajectory.BP_PlayerTrajectory_C|GetSphere CheckTrajectory) 0 :!class /Script/Engine.PrimitiveComponent) :!label _label)
    (:LoopBody
      (bind _asbp_player_trajectory (Utilities|Casting|CastToBP_PlayerTrajectory _array_element))
      (if (== _asbp_player_trajectory (Variables|/Game/_Users/MapParts/BP_PlayerTrajectory.BP_PlayerTrajectory_C|GetPrev CheckTrajectory))
        (LocalVariables|SetbReturn true)
        (goto _label Break)))
    (:Completed
      (return (LocalVariables|GetbReturn)))))

(fn StartIconsRotate
  (for _array_element (Variables|Default|GetIcons)
    (Default|Rotate _array_element)))

(fn ConnectMap
  (for _array_element (Variables|Default|GetPartsArray)
    (Utilities|IsValid (.AsBP%20Deform%20Parts%20Base (Utilities|Casting|CastToBP_DeformPartsBase _array_element))
      (:Is%20Valid
        (Default|ChangeTypeVisibility (.AsBP%20Deform%20Parts%20Base (Utilities|Casting|CastToBP_DeformPartsBase _array_element)) true))))
  (for _array_element_2 (Variables|Default|GetIcons)
    (Default|ChangeVisibility _array_element_2 true)))

(fn GetRelativeDeformLocation
  (params (Parts :type BP%20Map%20Parts%20Base%20Object%20Reference) (targetLocation :type Vector))
  (return (- (Transformation|GetActorLocation (Variables|/Game/_Users/MapParts/Parts/BP_MapPartsBase.BP_MapPartsBase_C|GetMyDeformParts Parts)) (* (- (Transformation|GetActorLocation Parts) targetLocation) 0.003))))