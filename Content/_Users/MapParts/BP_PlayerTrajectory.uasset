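; BP_PlayerTrajectory is one linked marker in a player trajectory, with a player-icon arrow material, that animates its mesh height on a looping timeline.
; On BeginPlay it creates the dynamic material, then polls each tick until IsMove is set or it has no valid Prev.
; After its first cycle it sets IsMove on Next following a short delay and clears that link, staggering the motion along the chain.
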(event EventBeginPlay
  (bind _returnvalue (Rendering|Material|CreateDynamicMaterialInstance (Variables|Default|GetMesh) 0 "/Game/_Users/MapParts/Icons/Materials/MI_PlayerIconArrow.MI_PlayerIconArrow" "None" :!class /Script/Engine.PrimitiveComponent))
  (Variables|Default|SetMaterial _returnvalue)
  (if (or (Variables|Default|GetbIsMove) (not (Utilities|IsValid (Variables|Default|GetPrev)))) :!label _label
    (bind _newtrack_0 (Timeline|Timeline_0 PlayFromStart)
      (:Update
        (Transformation|SetRelativeLocation (Variables|Default|GetMesh) (Math|Vector|MakeVector 0.0 0.0 (* _newtrack_0 5e+01)) false false))
      (:Finished
        (Utilities|FlowControl|Delay 0.0)
        (Utilities|IsValid (Variables|Default|GetNext)
          (:Is%20Valid
            (Utilities|FlowControl|Sequence
              (:then_0
                (Utilities|FlowControl|Delay 0.1)
                (Variables|BP_PlayerTrajectory_C|SetbIsMove (Variables|Default|GetNext) true)
                (Variables|Default|SetNext 0))
              (:then_1
                (Timeline|Timeline_0 PlayFromStart))))
          (:Is%20Not%20Valid
            (Timeline|Timeline_0 PlayFromStart)))))
    (else
      (Utilities|FlowControl|Delay 0.0)
      (goto _label))))

(fn ConstructionScript)