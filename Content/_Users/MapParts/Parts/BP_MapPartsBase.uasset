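; Base actor for generated map parts, which tracks player presence and is paired with a deform part.
; Unless it is a deform part itself, it waits for MapGenerator to finish, then polls ConflictCheckCollision in a Delay loop, notifying its deform part on the player's first pass.
; WaitDestroy disables that collision, then shortly destroys both actors.
; Helpers display connection generation numbers, find the lowest one and return the player's offset.
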(event Custom|WaitDestroy
  (bind _mydeformparts (Variables|Default|GetMyDeformParts))
  (Collision|SetCollisionEnabled (Variables|Default|GetConflictCheckCollision) "NoCollision")
  (Utilities|FlowControl|Delay 0.1)
  (Utilities|IsValid _mydeformparts
    (:Is%20Valid
      (Actor|DestroyActor _mydeformparts))
    (:Is%20Not%20Valid
      _))
  (Actor|DestroyActor))

(event Custom|ShowNum
  (for _array_element (Actor|GetComponentsByClass "/Game/_Users/MapParts/Parts/BP_ConnectionParts.BP_ConnectionParts_C")
    (bind _returnvalue (Game|SpawnActorfromClass "/Game/_Users/MapParts/BP_ShowText.BP_ShowText_C" (Math|Transform|MakeTransform (+ (Transformation|GetWorldLocation _array_element) "0, 0,100.000000") "0, 0, 0" "1,1,1") "Undefined" 0 0))
    (Rendering|Components|TextRender|SetText (Variables|/Game/_Users/MapParts/BP_ShowText.BP_ShowText_C|GetTextRender _returnvalue) (Utilities|Text|ToText(Integer) (Variables|/Game/_Users/MapParts/Parts/BP_ConnectionParts.BP_ConnectionParts_C|GetGenerationNum _array_element)))))

(event Custom|ChasePlayerLocation
  (Utilities|IsValid (Variables|Default|GetMapGenerator) :!label _label
    (:Is%20Valid
      (if (Variables|/Game/_Users/MapParts/BP_MapManager.BP_MapManager_C|GetbIsGenerated (Variables|Default|GetMapGenerator))
        (Variables|Default|SetbPlayerOverlapping false :!label _label_2)
        (bind _array_element (Utilities|Array|ForEachLoopwithBreak (Collision|GetOverlappingActors (Variables|Default|GetConflictCheckCollision) "/Game/_Users/Players/Blueprints/BP_Player.BP_Player_C" :!class /Script/Engine.PrimitiveComponent) :!label _label_3)
          (:LoopBody
            (Utilities|Casting|CastToBP_Player _array_element)
            (Variables|Default|SetbPlayerOverlapping true)
            (if (not (Variables|Default|GetbIsPassed))
              (Variables|Default|SetbIsPassed true)
              (Default|PassedThisRoom (.AsBP%20Deform%20Parts%20Base (Utilities|Casting|CastToBP_DeformPartsBase (Variables|Default|GetMyDeformParts))))
              (goto _label_3 Break)))
          (:Completed
            (Utilities|FlowControl|Delay 0.2)
            (goto _label_2)))
        (else
          (Utilities|FlowControl|Delay 0.2 :!label _label_4)
          (goto _label))))
    (:Is%20Not%20Valid
      (goto _label_4))))

(event EventBeginPlay
  (Utilities|Casting|CastToBP_DeformPartsBase self
    (:CastFailed
      (CallFunction|ChasePlayerLocation))))

(fn ConstructionScript)

(fn GetYoungestGenerationNum
  (for _array_element (Actor|GetComponentsByClass "/Game/_Users/MapParts/Parts/BP_ConnectionParts.BP_ConnectionParts_C")
    (if (> (LocalVariables|GetReturnNum) (Variables|/Game/_Users/MapParts/Parts/BP_ConnectionParts.BP_ConnectionParts_C|GetGenerationNum _array_element))
      (LocalVariables|SetReturnNum (Variables|/Game/_Users/MapParts/Parts/BP_ConnectionParts.BP_ConnectionParts_C|GetGenerationNum _array_element))))
  (return (LocalVariables|GetReturnNum)))

(fn GetCurrentPlayerLocationDiff
  (return (- (Transformation|GetActorLocation (Game|Player|GetPlayerPawn 0)) (Transformation|GetActorLocation))))