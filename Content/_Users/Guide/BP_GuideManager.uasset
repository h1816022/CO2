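; Manager Blueprint for on-screen guides: named button prompts plus a single guide message, both created as viewport widgets.
; Adding a button guide sorts the list by descending button type, keeping one per type, and spreads widgets horizontally; removal by name only re-sorts.
; New messages replace the current one unless it is fixed, optionally playing a bell sound.
; Once-only messages are tracked by name to prevent repeats.
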(fn ConstructionScript)

(fn AdjustGuideLocation
  (bind _buttonguidewidgets (Variables|Default|GetButtonGuideWidgets))
  (CallFunction|SortButtonGuides)
  (LocalVariables|SetRate (- 1.3 (/ (Math|Conversions|ToFloat(Integer) (Utilities|Array|Length (Variables|Default|GetButtonGuideWidgets))) 2e+01)))
  (for (_array_element _array_index) _buttonguidewidgets
    (Class|UserWidget|SetPositioninViewport (.widget _array_element) (Math|Vector2D|MakeVector2D (- (* 3.6e+02 (LocalVariables|GetRate)) (* (* (+ _array_index 1) (/ 7.2e+02 (Math|Conversions|ToFloat(Integer) (+ (Utilities|Array|Length _buttonguidewidgets) 1)))) (LocalVariables|GetRate))) 0.0) true)))

(fn AddButtonGuide
  (params (ButtonType :type EButtonTypes%20Enum :default "NewEnumerator0") (Text :type Text) (LifeTime :type Float%20%28single-precision%29) (Name :type Name))
  (bind _returnvalue (UserInterface|CreateWidget "/Game/_Users/Guide/WBP_ButtonGuide.WBP_ButtonGuide_C" 0 ButtonType Text LifeTime))
  (UserInterface|Viewport|AddtoViewport _returnvalue 0)
  (Utilities|Array|Add (Variables|Default|GetButtonGuideWidgets) (Utilities|Struct|MakeSGuideData Name _returnvalue))
  (CallFunction|AdjustGuideLocation))

(fn SortButtonGuides
  (bind _returnvalue (Utilities|Enum|LiteralenumEButtonTypes "NewEnumerator10"))
  (bind _returnvalue_2 (Math|Conversions|ToInteger(Byte) _returnvalue))
  (bind _returnvalue_3 (- _returnvalue_2 1))
  (for _index (range 0 _returnvalue_3)
    (bind _array_element (Utilities|Array|ForEachLoopwithBreak (Variables|Default|GetButtonGuideWidgets) :!label _label)
      (:LoopBody
        (if (== (- _returnvalue_3 _index) (Math|Conversions|ToInteger(Byte) (Variables|/Game/_Users/Guide/WBP_ButtonGuide.WBP_ButtonGuide_C|GetButtonType (.AsWBP%20Button%20Guide (Utilities|Casting|CastToWBP_ButtonGuide (.Widget (Utilities|Struct|BreakSGuideData _array_element)))))))
          (Utilities|Array|Add (LocalVariables|GetNewArray) _array_element)
          (goto _label Break)))))
  (Variables|Default|SetButtonGuideWidgets (LocalVariables|GetNewArray)))

(fn ChangeGuideMessage
  (params (Text :type Text) (LifeTime :type Float%20%28single-precision%29) (bIsBlink :type Boolean) (bMakeSound :type Boolean) (Name :type Name) (bIsFixed :type Boolean) (bIsOnce :type Boolean))
  (if (or (not bIsOnce) (CallFunction|CheckOnceNames Name))
    (Utilities|IsValid (.widget (.guidedata (Variables|Default|GetNowMessage)))
      (:Is%20Valid
        (if (not (.bisfixedmessage (Variables|Default|GetNowMessage)))
          (Default|Remove (.AsWBP%20Guide%20Message (Utilities|Casting|CastToWBP_GuideMessage (.widget (.guidedata (Variables|Default|GetNowMessage))))))
          (bind _returnvalue (UserInterface|CreateWidget "/Game/_Users/Guide/WBP_GuideMessage.WBP_GuideMessage_C" 0 Text LifeTime bIsBlink :!label _label))
          (bind _output_get (Variables|Default|SetNowMessage (Utilities|Struct|MakeSGuideMessageData (Utilities|Struct|MakeSGuideData Name _returnvalue) bIsFixed)))
          (UserInterface|Viewport|AddtoViewport (.widget (.guidedata _output_get)) 0)
          (if bMakeSound
            (Audio|PlaySound2D "/Game/_Users/Sounds/A_Bell2_Cue.A_Bell2_Cue" 1.0 1.0 0.0 0 0))))
      (:Is%20Not%20Valid
        (goto _label)))))

(fn RemoveGuideMessage
  (params (Name :type Name))
  (bind _nowmessage (Variables|Default|GetNowMessage))
  (Utilities|IsValid (.widget (.guidedata _nowmessage))
    (:Is%20Valid
      (if (Utilities|Name|Equal(Name) (.name (.guidedata _nowmessage)) Name)
        (Default|Remove (.AsWBP%20Guide%20Message (Utilities|Casting|CastToWBP_GuideMessage (.widget (.guidedata (Variables|Default|GetNowMessage))))))))))

(fn RemoveButtonGuide
  (params (Name :type Name))
  (bind _faunddata (CallFunction|FindGuidebyName (Variables|Default|GetButtonGuideWidgets) Name))
  (for _array_element _faunddata
    (Default|Remove (.AsWBP%20Button%20Guide (Utilities|Casting|CastToWBP_ButtonGuide (.Widget (Utilities|Struct|BreakSGuideData _array_element)))))
    (Utilities|Array|RemoveItem (Variables|Default|GetButtonGuideWidgets) _array_element))
  (CallFunction|SortButtonGuides))

(fn RemoveButtonGuides
  (params (Names :type Array%20of%20Names))
  (bind _founddata (CallFunction|FindGuidebyNames (Variables|Default|GetButtonGuideWidgets) Names))
  (for _array_element _founddata
    (Default|Remove (.AsWBP%20Button%20Guide (Utilities|Casting|CastToWBP_ButtonGuide (.Widget (Utilities|Struct|BreakSGuideData _array_element)))))
    (Utilities|Array|RemoveItem (Variables|Default|GetButtonGuideWidgets) _array_element))
  (CallFunction|SortButtonGuides))

(fn FindGuidebyName
  (params (Data :type Array%20of%20S%20Guide%20Data%20Structures) (Name :type %20Object%20Reference))
  (for _array_element Data
    (if (Utilities|Name|Equal(Name) (.Name (Utilities|Struct|BreakSGuideData _array_element)) Name)
      (Utilities|Array|Add (LocalVariables|GetReturn) _array_element)))
  (return (LocalVariables|GetReturn)))

(fn FindGuidebyNames
  (params (Data :type Array%20of%20S%20Guide%20Data%20Structures) (Names :type Array%20of%20Names))
  (for _array_element Names
    (bind _faunddata (CallFunction|FindGuidebyName Data _array_element))
    (Utilities|Array|AppendArray (LocalVariables|GetReturn) _faunddata))
  (return (LocalVariables|GetReturn)))

(fn CheckOnceNames
  (params (NewName :type Name))
  (if (== (Utilities|Array|FindItem (Variables|Default|GetOnceMessageNames) NewName) -1)
    (Utilities|Array|Add (Variables|Default|GetOnceMessageNames) NewName)
    (return true)
    (else
      (return false))))