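; BP_Door is an automatic double sliding door that opens while something overlaps its Sensor and closes after a delay.
; BeginPlay caches each panel's closed and open positions along its forward vector; Tick lerps between them using a clamped alpha stepped per frame, independent of delta time.
; An overlap counter and open/close flags set direction, with the delay counting only once fully open and unoccupied.
; The door sound plays on first entry and last exit, before the closing delay.
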(event OnComponentBeginOverlap(Sensor)
  (params (OverlappedComponent :type Primitive%20Component%20Object%20Reference) (OtherActor :type Actor%20Object%20Reference) (OtherComp :type Primitive%20Component%20Object%20Reference) (OtherBodyIndex :type Integer) (bFromSweep :type Boolean) (SweepResult :type Hit%20Result%20Structure%20%28by%20ref%29))
  (CallFunction|Open))

(event OnComponentEndOverlap(Sensor)
  (params (OverlappedComponent :type Primitive%20Component%20Object%20Reference) (OtherActor :type Actor%20Object%20Reference) (OtherComp :type Primitive%20Component%20Object%20Reference) (OtherBodyIndex :type Integer))
  (CallFunction|Close))

(event Custom|Open
  (Variables|Default|SetbIsOpen true)
  (bind _result (Math|Integer|IncrementInt (Variables|Default|GetOverlappingSensorNum))
    (:%20%20
      (if (== _result 1)
        (Audio|PlaySoundatLocation "/Game/_Users/Blueprints/Door/Sounds/A_Door.A_Door" (Transformation|GetActorLocation) "0, 0, 0" 1.0 1.0 0.0 0 0 0)))))

(event Custom|Close
  (bind _overlappingsensornum (Variables|Default|GetOverlappingSensorNum))
  (Math|Integer|DecrementInt _overlappingsensornum
    (:%20%20
      (if (== _overlappingsensornum 0)
        (Variables|Default|SetbIsClose true)
        (Audio|PlaySoundatLocation "/Game/_Users/Blueprints/Door/Sounds/A_Door.A_Door" (Transformation|GetActorLocation) "0, 0, 0" 1.0 1.0 0.0 "/Game/_Users/Sounds/Att_Default.Att_Default" 0 0)))))

(event EventBeginPlay
  (bind _right (Variables|Default|GetRight))
  (bind _left (Variables|Default|GetLeft))
  (bind _returnvalue (Transformation|GetWorldLocation _left))
  (bind _returnvalue_2 (Transformation|GetWorldLocation _right))
  (Variables|Default|SetStartLeftLocation _returnvalue)
  (Variables|Default|SetEndLeftLocation (+ _returnvalue (* (Math|Vector|GetForwardVector _left) (Variables|Default|GetMoveDistance))))
  (Variables|Default|SetStartRightLocation _returnvalue_2)
  (Variables|Default|SetEndRightLocation (+ _returnvalue_2 (* (Math|Vector|GetForwardVector _right) (Variables|Default|GetMoveDistance)))))

(event EventTick
  (params (DeltaSeconds :type Float%20%28single-precision%29))
  (bind _biscontinue (CallFunction|UpdateFlag))
  (if _biscontinue
    (Transformation|SetWorldLocation (Variables|Default|GetLeft) (Math|Vector|Lerp(Vector) (Variables|Default|GetStartLeftLocation) (Variables|Default|GetEndLeftLocation) (Variables|Default|GetNowAlpha)) false false)
    (Transformation|SetWorldLocation (Variables|Default|GetRight) (Math|Vector|Lerp(Vector) (Variables|Default|GetStartRightLocation) (Variables|Default|GetEndRightLocation) (Variables|Default|GetNowAlpha)) false false)
    (CallFunction|UpdateAlpha)))

(fn ConstructionScript)

(fn UpdateFlag
  (if (and (Variables|Default|GetbIsOpen) (== (Variables|Default|GetNowAlpha) 1.0))
    (if (== (Variables|Default|GetOverlappingSensorNum) 0)
      (Variables|Default|SetNowCloseDelayTime (+ (Variables|Default|GetNowCloseDelayTime) (Utilities|Time|GetWorldDeltaSeconds)))
      (if (>= (Variables|Default|GetNowCloseDelayTime) (Variables|Default|GetCloseDelayTime))
        (Variables|Default|SetbIsOpen false))
      (else
        (Variables|Default|SetNowCloseDelayTime 0.0 :!label _label)))
    (elif (and (Variables|Default|GetbIsClose) (== (Variables|Default|GetNowAlpha) 0.0))
      (Variables|Default|SetbIsClose false)
      (goto _label)
      (else
        (goto _label))))
  (return (or (Variables|Default|GetbIsOpen) (Variables|Default|GetbIsClose))))

(fn UpdateAlpha
  (Variables|Default|SetNowAlpha (Math|Float|Clamp(Float) (+ (Variables|Default|GetNowAlpha) (* (Variables|Default|GetLerpAlphaRate) (- 1.0 (* (Math|Conversions|ToFloat(Boolean) (and (not (Variables|Default|GetbIsOpen)) (Variables|Default|GetbIsClose))) 2.0)))))))