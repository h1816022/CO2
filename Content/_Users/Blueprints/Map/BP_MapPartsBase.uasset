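; BP_MapPartsBase is a map piece actor whose BP_ConnectionParts components carry generation numbers, likely serving as a base for generated map parts.
; On BeginPlay it registers itself as the owner of each connection component.
; It can return the lowest generation number among its connections, or spawn BP_ShowText actors above them to display each number.
; WaitDestroy disables the conflict-check collision, then destroys the actor after a short delay.
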(event Custom|WaitDestroy
  (Collision|SetCollisionEnabled (Variables|Default|GetConflictCheckCollision) "NoCollision")
  (Utilities|FlowControl|Delay 0.1)
  (Actor|DestroyActor))

(event Custom|ShowNum
  (for _array_element (Actor|GetComponentsByClass "/Game/_Users/Blueprints/Map/BP_ConnectionParts.BP_ConnectionParts_C")
    (bind _returnvalue (Game|SpawnActorfromClass "/Game/_Users/Blueprints/Map/BP_ShowText.BP_ShowText_C" (Math|Transform|MakeTransform (+ (Transformation|GetWorldLocation _array_element) "0, 0,100.000000") "0, 0, 0" "1,1,1") "Undefined" 0 0))
    (Rendering|Components|TextRender|SetText (Variables|/Game/_Users/Blueprints/Map/BP_ShowText.BP_ShowText_C|GetTextRender _returnvalue) (Utilities|Text|ToText(Integer) (Variables|/Game/_Users/Blueprints/Map/BP_ConnectionParts.BP_ConnectionParts_C|GetGenerationNum _array_element)))))

(event EventBeginPlay
  (for _array_element (Actor|GetComponentsByClass "/Game/_Users/Blueprints/Map/BP_ConnectionParts.BP_ConnectionParts_C")
    (Variables|/Game/_Users/Blueprints/Map/BP_ConnectionParts.BP_ConnectionParts_C|SetMyParts _array_element self)))

(fn ConstructionScript)

(fn GetYoungestGenerationNum
  (for _array_element (Actor|GetComponentsByClass "/Game/_Users/Blueprints/Map/BP_ConnectionParts.BP_ConnectionParts_C")
    (if (> (LocalVariables|GetReturnNum) (Variables|/Game/_Users/Blueprints/Map/BP_ConnectionParts.BP_ConnectionParts_C|GetGenerationNum _array_element))
      (LocalVariables|SetReturnNum (Variables|/Game/_Users/Blueprints/Map/BP_ConnectionParts.BP_ConnectionParts_C|GetGenerationNum _array_element))))
  (return (LocalVariables|GetReturnNum)))