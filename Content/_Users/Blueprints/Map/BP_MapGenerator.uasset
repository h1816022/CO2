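; Procedural map generator that grows a layout outward from the first placed BP_MapPartsBase, in waves of open connection points up to Max.
; Each connection spawns a random part from its DT_MapPartsData row and snaps a complementary P/M connector onto it, facing opposite.
; CheckConflict tests overlaps against some placed parts' collisions, retrying the part's other matching connectors and destroying it when none remain.
; Successful parts supply the next wave's connections.
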(event Custom|AddP
  (Math|Integer|IncrementInt (Variables|Default|GetNum)
    (:%20%20
      (Variables|Default|SetNowConnectionPartsArray (Variables|Default|GetNextConnectionPartsArray))
      (Utilities|Array|Clear (Variables|Default|GetNextConnectionPartsArray))
      (if (< (Variables|Default|GetNum) (Variables|Default|GetMax))
        (CallFunction|CheckAllConnectionParts (Variables|Default|GetNowConnectionPartsArray))
        (else
          (for _array_element (Variables|Default|GetCurrentlyGeneratedPartsArray)
            (if (CallFunction|CheckConflict _array_element)
              _)))))))

(event EventBeginPlay
  ;[1 1 1] 最初のパーツが用意されるまで待つ
  (bind _outactors (Actor|GetAllActorsOfClass "/Game/_Users/Blueprints/Map/BP_MapPartsBase.BP_MapPartsBase_C" :!label _label))
  (if (== (Utilities|Array|Length _outactors) 0)
    (Utilities|FlowControl|Delay 0.0)
    (goto _label)
    (else
      (Utilities|Array|Add (Variables|Default|GetCurrentlyGeneratedPartsArray) (Utilities|Array|Get(acopy) _outactors))
      (for _array_element (Actor|GetComponentsByClass (Utilities|Array|Get(acopy) _outactors) "/Game/_Users/Blueprints/Map/BP_ConnectionParts.BP_ConnectionParts_C")
        (Utilities|Array|Add (Variables|Default|GetNowConnectionPartsArray) _array_element))
      (CallFunction|CheckAllConnectionParts (Variables|Default|GetNowConnectionPartsArray)))))

(fn ConstructionScript)

(fn SpawnNextParts
  (params (OtherConnectionParts :type BP%20Connection%20Parts%20Object%20Reference))
  (bind _tmpnextconnectionpartsarray (LocalVariables|GetTmpNextConnectionPartsArray))
  (bind _returnvalue (Utilities|Array|Length _tmpnextconnectionpartsarray))
  (bind _returnvalue_2 (Transformation|GetWorldRotation OtherConnectionParts))
  (bind _returnvalue_3 (Utilities|GetDataTableRow "/Game/_Users/Blueprints/Map/Data/DT_MapPartsData.DT_MapPartsData" (Utilities|String|StringToName (Utilities|String|EnumtoString (Variables|/Game/_Users/Blueprints/Map/BP_ConnectionParts.BP_ConnectionParts_C|GetOtherMapPartsType OtherConnectionParts))))
    (:then
      (LocalVariables|SetNextPartsCandidate (.parts _returnvalue_3))
      (LocalVariables|SetTmpChoiceIndex (Math|Random|RandomInteger (Utilities|Array|Length (LocalVariables|GetNextPartsCandidate))))
      (bind _returnvalue_4 (Game|SpawnActorfromClass (Utilities|Array|Get(acopy) (LocalVariables|GetNextPartsCandidate) (LocalVariables|GetTmpChoiceIndex)) (Math|Transform|MakeTransform "0, 0, 0" "0, 0, 0" "1,1,1") "Undefined" 0 0))
      (LocalVariables|SetNextParts _returnvalue_4)
      (Utilities|Array|RemoveIndex (LocalVariables|GetNextPartsCandidate) (LocalVariables|GetTmpChoiceIndex))
      (for _array_element (Actor|GetComponentsByClass (LocalVariables|GetNextParts) "/Game/_Users/Blueprints/Map/BP_ConnectionParts.BP_ConnectionParts_C")
        (if (CallFunction|CheckMapPartsTypeCombo (Variables|/Game/_Users/Blueprints/Map/BP_ConnectionParts.BP_ConnectionParts_C|GetOtherMapPartsType OtherConnectionParts) (Variables|/Game/_Users/Blueprints/Map/BP_ConnectionParts.BP_ConnectionParts_C|GetOtherMapPartsType _array_element))
          (Utilities|Array|Add (LocalVariables|GetTmpNextConnectionPartsArray) _array_element)))
      (if (!= _returnvalue 0) :!label _label
        (LocalVariables|SetTmpChoiceIndex (Math|Random|RandomInteger _returnvalue))
        (LocalVariables|SetNextConnectionParts (Utilities|Array|Get(acopy) (LocalVariables|GetTmpNextConnectionPartsArray) (LocalVariables|GetTmpChoiceIndex)))
        (Utilities|Array|RemoveIndex (LocalVariables|GetTmpNextConnectionPartsArray) (LocalVariables|GetTmpChoiceIndex))
        (Transformation|SetActorRotation (LocalVariables|GetNextParts) (Math|Rotator|MakeRotator (- (.roll _returnvalue_2) (.roll (Variables|/Script/Engine.SceneComponent|GetRelativeRotation (LocalVariables|GetNextConnectionParts)))) (- (.pitch _returnvalue_2) (.pitch (Variables|/Script/Engine.SceneComponent|GetRelativeRotation (LocalVariables|GetNextConnectionParts)))) (+ (- (.yaw _returnvalue_2) (.yaw (Variables|/Script/Engine.SceneComponent|GetRelativeRotation (LocalVariables|GetNextConnectionParts)))) 1.8e+02)))
        (Transformation|SetActorLocation (LocalVariables|GetNextParts) (+ (- (Transformation|GetActorLocation (LocalVariables|GetNextParts)) (Transformation|GetWorldLocation (LocalVariables|GetNextConnectionParts))) (Transformation|GetWorldLocation OtherConnectionParts)) false false)
        (Variables|/Game/_Users/Blueprints/Map/BP_ConnectionParts.BP_ConnectionParts_C|SetbCanConnest (LocalVariables|GetNextConnectionParts) false)
        (if (CallFunction|CheckConflict (LocalVariables|GetNextParts))
          (goto _label)
          (else
            (for _array_element_2 (Actor|GetComponentsByClass (LocalVariables|GetNextParts) "/Game/_Users/Blueprints/Map/BP_ConnectionParts.BP_ConnectionParts_C")
              (Utilities|Array|Add (Variables|Default|GetNextConnectionPartsArray) _array_element_2))
            (Utilities|Array|Add (Variables|Default|GetCurrentlyGeneratedPartsArray) (LocalVariables|GetNextParts))))
        (else
          (Actor|DestroyActor (LocalVariables|GetNextParts)))))))

(fn CheckAllConnectionParts
  (params (Parts :type Array%20of%20BP%20Connection%20Parts%20Object%20References))
  (for _array_element Parts
    (if (Variables|/Game/_Users/Blueprints/Map/BP_ConnectionParts.BP_ConnectionParts_C|GetbCanConnest _array_element)
      (Variables|/Game/_Users/Blueprints/Map/BP_ConnectionParts.BP_ConnectionParts_C|SetbCanConnest _array_element false)
      (CallFunction|SpawnNextParts _array_element)))
  (CallFunction|AddP))

(fn CheckMapPartsTypeCombo
  (params (Type1 :type EMapPartsType%20Enum :default "NewEnumerator0") (Type2 :type EMapPartsType%20Enum :default "NewEnumerator0"))
  (switch Utilities|FlowControl|Switch|SwitchonEMapPartsType Type1
    (:NewEnumerator0
      (return (Utilities|Enum|Equal(Enum) Type2 "NewEnumerator1")))
    (:NewEnumerator1
      (return (Utilities|Enum|Equal(Enum) Type2 "NewEnumerator0")))
    (:NewEnumerator4
      (return (Utilities|Enum|Equal(Enum) Type2 "NewEnumerator5")))
    (:NewEnumerator5
      (return (Utilities|Enum|Equal(Enum) Type2 "NewEnumerator4")))
    (:NewEnumerator2
      (return (Utilities|Enum|Equal(Enum) Type2 "NewEnumerator3")))
    (:NewEnumerator3
      (return (Utilities|Enum|Equal(Enum) Type2 "NewEnumerator2")))))

(fn CheckConflict
  (params (MapParts :type BP%20Map%20Parts%20Base%20Object%20Reference))
  (LocalVariables|SetTmpCollisions (CallFunction|GetCollisions))
  (bind _array_element (Utilities|Array|ForEachLoopwithBreak (Class|PrimitiveComponent|GetOverlappingComponents (Variables|/Game/_Users/Blueprints/Map/BP_MapPartsBase.BP_MapPartsBase_C|GetConflictCheckCollision MapParts)) :!label _label)
    (:LoopBody
      (if (LocalVariables|GetbReturn)
        (goto _label Break)
        (else
          (bind _array_element_2 (Utilities|Array|ForEachLoopwithBreak (LocalVariables|GetTmpCollisions) :!label _label_2)
            (:LoopBody
              (if (== _array_element_2 _array_element)
                (LocalVariables|SetbReturn true)
                (goto _label_2 Break)
                (else
                  (Development|PrintString (Utilities|String|Append (Utilities|GetDisplayName _array_element_2) "   :   " (Utilities|GetDisplayName _array_element))))))))))
    (:Completed
      (return (LocalVariables|GetbReturn)))))

(fn GetCollisions
  (for _array_element (Variables|Default|GetCurrentlyGeneratedPartsArray)
    (if (Math|Boolean|ORBoolean (Utilities|Enum|Equal(Enum) (Variables|/Game/_Users/Blueprints/Map/BP_ConnectionParts.BP_ConnectionParts_C|GetOtherMapPartsType (Actor|GetComponentbyClass _array_element "/Game/_Users/Blueprints/Map/BP_ConnectionParts.BP_ConnectionParts_C")) "NewEnumerator1") (Utilities|Enum|Equal(Enum) (Variables|/Game/_Users/Blueprints/Map/BP_ConnectionParts.BP_ConnectionParts_C|GetOtherMapPartsType (Actor|GetComponentbyClass _array_element "/Game/_Users/Blueprints/Map/BP_ConnectionParts.BP_ConnectionParts_C")) "NewEnumerator5") (Utilities|Enum|Equal(Enum) (Variables|/Game/_Users/Blueprints/Map/BP_ConnectionParts.BP_ConnectionParts_C|GetOtherMapPartsType (Actor|GetComponentbyClass _array_element "/Game/_Users/Blueprints/Map/BP_ConnectionParts.BP_ConnectionParts_C")) "NewEnumerator3"))
      (Utilities|Array|Add (LocalVariables|GetReturn) (Variables|/Game/_Users/Blueprints/Map/BP_MapPartsBase.BP_MapPartsBase_C|GetConflictCheckCollision _array_element))))
  (return (LocalVariables|GetReturn)))