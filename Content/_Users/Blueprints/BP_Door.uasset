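; BP_Door is a two-panel door that slides Left and Right along their forward vectors by MoveDistance.
; Open and Close events maintain an overlapping-sensor count, requesting a close when it reaches zero.
; While opening or closing is flagged, Tick lerps both panels, stepping a clamped alpha by a fixed per-frame rate.
; UpdateFlag holds the fully open door until no sensors overlap for CloseDelayTime, then lets it close.
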(event Custom|Open
  (Variables|Default|SetbIsOpen true)
  (Math|Integer|IncrementInt (Variables|Default|GetOverlappingSensorNum)))

(event Custom|Close
  (bind _overlappingsensornum (Variables|Default|GetOverlappingSensorNum))
  (Math|Integer|DecrementInt _overlappingsensornum
    (:%20%20
      (if (== _overlappingsensornum 0)
        (Variables|Default|SetbIsClose true)))))

(event EventBeginPlay
  (bind _right (Variables|Default|GetRight))
  (bind _left (Variables|Default|GetLeft))
  (bind _returnvalue (Transformation|GetWorldLocation _left))
  (bind _returnvalue_2 (Transformation|GetWorldLocation _right))
  (Variables|Default|SetStartLeftLocation _returnvalue)
  (Variables|Default|SetEndLeftLocation (+ _returnvalue (* (Math|Vector|GetForwardVector _left) (Variables|Default|GetMoveDistance))))
  (Variables|Default|SetStartRightLocation _returnvalue_2)
  (Variables|Default|SetEndRightLocation (+ _returnvalue_2 (* (Math|Vector|GetForwardVector _right) (Variables|Default|GetMoveDistance)))))

(event EventTick
  (params (DeltaSeconds :type Float%20%28single-precision%29))
  (bind _biscontinue (CallFunction|UpdateFlag))
  (if _biscontinue
    (Transformation|SetWorldLocation (Variables|Default|GetLeft) (Math|Vector|Lerp(Vector) (Variables|Default|GetStartLeftLocation) (Variables|Default|GetEndLeftLocation) (Variables|Default|GetNowAlpha)) false false)
    (Transformation|SetWorldLocation (Variables|Default|GetRight) (Math|Vector|Lerp(Vector) (Variables|Default|GetStartRightLocation) (Variables|Default|GetEndRightLocation) (Variables|Default|GetNowAlpha)) false false)
    (CallFunction|UpdateAlpha)))

(fn ConstructionScript)

(fn UpdateFlag
  (if (and (Variables|Default|GetbIsOpen) (== (Variables|Default|GetNowAlpha) 1.0))
    (if (== (Variables|Default|GetOverlappingSensorNum) 0)
      (Variables|Default|SetNowCloseDelayTime (+ (Variables|Default|GetNowCloseDelayTime) (Utilities|Time|GetWorldDeltaSeconds)))
      (if (>= (Variables|Default|GetNowCloseDelayTime) (Variables|Default|GetCloseDelayTime))
        (Variables|Default|SetbIsOpen false))
      (else
        (Variables|Default|SetNowCloseDelayTime 0.0 :!label _label)))
    (elif (and (Variables|Default|GetbIsClose) (== (Variables|Default|GetNowAlpha) 0.0))
      (Variables|Default|SetbIsClose false)
      (goto _label)
      (else
        (goto _label))))
  (return (or (Variables|Default|GetbIsOpen) (Variables|Default|GetbIsClose))))

(fn UpdateAlpha
  (Variables|Default|SetNowAlpha (Math|Float|Clamp(Float) (+ (Variables|Default|GetNowAlpha) (* (Variables|Default|GetLerpAlphaRate) (- 1.0 (* (Math|Conversions|ToFloat(Boolean) (and (not (Variables|Default|GetbIsOpen)) (Variables|Default|GetbIsClose))) 2.0)))))))