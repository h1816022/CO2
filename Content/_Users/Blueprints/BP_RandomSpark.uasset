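; BP_RandomSpark is an actor that repeatedly emits a spark burst with a light flash at its location.
; A looping BeginPlay chain waits on a random-range delay whose equal bounds make it constant, then spawns a sparkler particle effect and plays a 2D spark sound.
; After a brief pause, a timeline scales the point light's intensity, playing forward and then reversing to form each flash.
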(event Custom|UpdateLight
  (params (bIsReverse :type Boolean))
  (if bIsReverse
    (bind _newtrack_0 (Timeline|Timeline_0 ReverseFromEnd)
      (:Update
        (Rendering|Components|Light|SetIntensity (Variables|Default|GetPointLight) (* _newtrack_0 (Variables|Default|GetIntensity))))
      (:Finished
        (if (not bIsReverse)
          (CallFunction|UpdateLight true))))
    (else
      (Timeline|Timeline_0 PlayFromStart))))

(event EventBeginPlay
  (Utilities|FlowControl|Delay (Math|Random|RandomFloatinRange 5.0 5.0) :!label _label)
  (Effects|SpawnEmitteratLocation "/Game/BallisticsVFX/Particles/Impacts/DynamicImpacts/Lava/Lava_impact_Sparklers.Lava_impact_Sparklers" (Transformation|GetActorLocation) (.rotation (Transformation|GetActorTransform)))
  (Audio|PlaySound2D "/Game/_Users/Sounds/Title/A_Spark_Cue.A_Spark_Cue" 0.2 1.0 3.7 0 0)
  (Utilities|FlowControl|Delay 0.05)
  (CallFunction|UpdateLight false)
  (goto _label))

(fn ConstructionScript)