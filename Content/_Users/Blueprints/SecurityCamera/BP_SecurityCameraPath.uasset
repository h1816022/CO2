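; Security camera path actor that computes a world position travelling back and forth along a spline.
; On BeginPlay it caches the spline length and starts a loop where a FlipFlop alternates a timeline between reverse and forward playback, beginning in reverse.
; Timeline updates scale the track value by the length and store the resulting point in NowLocation.
; Each finished pass waits briefly before switching direction.
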(event Custom|Move
  (Utilities|FlowControl|FlipFlop :!label _label
    (:A
      (bind _newtrack_0 (Timeline|Timeline_0 ReverseFromEnd)
        (:Update
          (Variables|Default|SetNowLocation (Spline|GetLocationatDistanceAlongSpline (Variables|Default|GetSpline) (* _newtrack_0 (Variables|Default|GetLength)) "World")))
        (:Finished
          (Utilities|FlowControl|Delay 1.0)
          (goto _label))))
    (:B
      (Timeline|Timeline_0 PlayFromStart))))

(event EventBeginPlay
  (Variables|Default|SetLength (Spline|GetSplineLength (Variables|Default|GetSpline)))
  (CallFunction|Move))

(fn ConstructionScript)