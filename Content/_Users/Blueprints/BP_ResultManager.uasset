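; Result screen manager that creates the WBP_Result widget and steps it through a short staged reveal.
; Next advances the widget by index, switching on ClearSeg and briefly blocking further advances during the second step.
; ForceNext loops on a zero-second Delay as a per-frame timer, auto-advancing after MaxTime.
; Once the sequence ends, GuideManager shows a blinking A-button prompt, and a further Next fires CallEnd once.
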(event Custom|Next
  (if (not (Variables|Default|GetbIsEnd))
    (if (Variables|Default|GetbCanNext)
      (Variables|Default|SetNowTime 0.0)
      (switch int (Variables|Default|GetNowIndex)
        (:0
          (Default|Next (Variables|Default|GetResultWidget))
          (Math|Integer|IncrementInt (Variables|Default|GetNowIndex) :!label _label))
        (:1
          (Variables|/Game/_Users/Seg/Blueprints/BP_SegBase.BP_SegBase_C|SetbIsOn (Variables|Default|GetClearSeg) true)
          (Default|Next (Variables|Default|GetResultWidget))
          (Variables|Default|SetbCanNext false)
          (Utilities|FlowControl|Delay 1.0)
          (Variables|Default|SetbCanNext true)
          (Variables|/Game/_Users/Seg/Blueprints/BP_SegBase.BP_SegBase_C|SetNowType (Variables|Default|GetClearSeg) "NewEnumerator0")
          (goto _label))
        (:2
          (Variables|Default|SetbIsEnd true))))
    (else
      (Utilities|FlowControl|DoOnce false
        (:Completed
          (Default|CallEnd))))))

(event Custom|ForceNext
  (if (Variables|Default|GetbCanNext) :!label _label
    (bind _output_get (Variables|Default|SetNowTime (+ (Variables|Default|GetNowTime) (Utilities|Time|GetWorldDeltaSeconds))))
    (if (< _output_get (Variables|Default|GetMaxTime))
      _
      (else
        (CallFunction|Next))))
  (if (not (Variables|Default|GetbIsEnd))
    (Utilities|FlowControl|Delay 0.0)
    (goto _label)
    (else
      (Default|ChangeGuideMessage (Variables|Default|GetGuideManager) "Aボタンで次へ" 0.0 true))))

(event EventBeginPlay
  (bind _returnvalue (UserInterface|CreateWidget "/Game/_Users/Widgets/WBP_Result.WBP_Result_C"))
  (bind _output_get (Variables|Default|SetResultWidget _returnvalue))
  (UserInterface|Viewport|AddtoViewport _output_get 0)
  (CallFunction|Next)
  (CallFunction|ForceNext))

(fn ConstructionScript)