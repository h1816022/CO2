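; BP_FadeCube is a cube actor that fades to transparent and destroys itself when its FadeOut event is called.
; BeginPlay creates a dynamic instance of MI_FadeColor on the cube.
; After a short delay, FadeOut lowers the Opacity parameter at a rate set by Time, using a zero-length Delay loop as a per-frame update instead of Tick or a Timeline.
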(event Custom|FadeOut
  (Utilities|FlowControl|Delay 1.0)
  (bind _output_get (Variables|Default|SetValue (Math|Float|Max(Float) (- (Variables|Default|GetValue) (/ (Utilities|Time|GetWorldDeltaSeconds) (Variables|Default|GetTime))) 0.0) :!label _label))
  (if (> _output_get 0.0)
    (Rendering|Material|SetScalarParameterValue (Variables|Default|GetMaterial) "Opacity" (Variables|Default|GetValue) :!class /Script/Engine.MaterialInstanceDynamic)
    (Utilities|FlowControl|Delay 0.0)
    (goto _label)
    (else
      (Actor|DestroyActor))))

(event EventBeginPlay
  (bind _returnvalue (Rendering|Material|CreateDynamicMaterialInstance (Variables|Default|GetCube) 0 "/Game/_Users/Materials/MI_FadeColor.MI_FadeColor" "None" :!class /Script/Engine.PrimitiveComponent))
  (Variables|Default|SetMaterial _returnvalue))

(fn ConstructionScript)