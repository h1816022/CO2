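; BP_Title is a title screen backdrop actor that adds parallax and light flicker behind the title camera.
; Each tick it offsets two planes by the BP_TitleCamera yaw and pitch at different strengths to fake depth.
; The camera's vertical input also drives the Opacity of both planes' dynamic materials.
; A looping delay briefly hides the planes and dims the spotlight at random intervals.
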(event Custom|UpdateLightVisibility
  (Utilities|FlowControl|Delay (Math|Random|RandomFloatinRange 0.5 15.0) :!label _label)
  (Rendering|SetVisibility (Variables|Default|GetPlane1) false false)
  (Rendering|SetVisibility (Variables|Default|GetPlane2) false false)
  (Rendering|Components|Light|SetIntensity (Variables|Default|GetSpotLight1) (/ (Variables|Default|GetDefaultIntensity) 1e+01))
  (Utilities|FlowControl|Delay 0.1)
  (Rendering|SetVisibility (Variables|Default|GetPlane1) true false)
  (Rendering|SetVisibility (Variables|Default|GetPlane2) true false)
  (Rendering|Components|Light|SetIntensity (Variables|Default|GetSpotLight1) (Variables|Default|GetDefaultIntensity))
  (goto _label))

(event EventBeginPlay
  (bind _outactors (Actor|GetAllActorsOfClass "/Game/_Users/Cameras/Blueprints/BP_TitleCamera.BP_TitleCamera_C"))
  (Variables|Default|SetCamera (Utilities|Array|Get(acopy) _outactors))
  (Variables|Default|SetDefaultLocation (Variables|/Script/Engine.SceneComponent|GetRelativeLocation (Variables|Default|GetPlane1)))
  (bind _returnvalue (Rendering|Material|CreateDynamicMaterialInstance (Variables|Default|GetPlane1) 0 "/Game/_Users/Materials/MI_TitleBack.MI_TitleBack" "None" :!class /Script/Engine.PrimitiveComponent))
  (Utilities|Array|Add (Variables|Default|GetMaterials) _returnvalue)
  (bind _returnvalue_2 (Rendering|Material|CreateDynamicMaterialInstance (Variables|Default|GetPlane2) 0 "/Game/_Users/Materials/MI_TitleBack_2.MI_TitleBack_2" "None" :!class /Script/Engine.PrimitiveComponent))
  (Utilities|Array|Add (Variables|Default|GetMaterials) _returnvalue_2)
  (CallFunction|UpdateLightVisibility)
  (Variables|Default|SetDefaultIntensity (Variables|/Script/Engine.LightComponentBase|GetIntensity (Variables|Default|GetSpotLight1))))

(event EventTick
  (params (DeltaSeconds :type Float%20%28single-precision%29))
  (bind _camera (Variables|Default|GetCamera))
  (bind _camera_2 (Variables|Default|GetCamera))
  (bind _returnvalue (Transformation|GetActorRotation _camera))
  (bind _returnvalue_2 (Transformation|GetActorRotation _camera_2))
  (Transformation|SetRelativeLocation (Variables|Default|GetPlane1) (+ (Math|Vector|MakeVector 0.0 (* (.yaw _returnvalue_2) 0.1) (* (.pitch _returnvalue_2) 0.1)) (Variables|Default|GetDefaultLocation)) false false)
  (Transformation|SetRelativeLocation (Variables|Default|GetPlane2) (+ (Math|Vector|MakeVector 0.0 (* (.yaw _returnvalue) 0.3) (* (.pitch _returnvalue) 0.3)) (Variables|Default|GetDefaultLocation)) false false)
  (for _array_element (Variables|Default|GetMaterials)
    (Rendering|Material|SetScalarParameterValue _array_element "Opacity" (/ (+ (* (Variables|/Game/_Users/Cameras/Blueprints/BP_TitleCamera.BP_TitleCamera_C|GetInputValueY (Variables|Default|GetCamera)) -1.0) 1.0) 4.0) :!class /Script/Engine.MaterialInstanceDynamic)))

(fn ConstructionScript)