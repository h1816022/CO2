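; BP_SoundManager is a Blueprint that plays and switches between a default background music track and a dash track.
; On BeginPlay it spawns both 2D sounds, keeps their references, stops them, then fades in the default track.
; ChangeBGM picks the track by a bool, waiting a given delay before fading it in.
; The default track stops abruptly, while the dash track gets a FadeOut call targeting full volume rather than silence.
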(event Custom|ChangeBGM
  (params (bDefault :type Boolean) (DelayTime :type Float%20%28single-precision%29))
  (if bDefault
    (Audio|Components|Audio|FadeOut (Variables|Default|GetDashBGM) 1.0 1.0 :!class /Script/Engine.AudioComponent)
    (Utilities|FlowControl|Delay DelayTime)
    (Audio|Components|Audio|FadeIn (Variables|Default|GetDefaultBGM) 2.0 1.0 0.0 :!class /Script/Engine.AudioComponent)
    (else
      (Audio|Components|Audio|Stop (Variables|Default|GetDefaultBGM))
      (Utilities|FlowControl|Delay DelayTime)
      (Audio|Components|Audio|FadeIn (Variables|Default|GetDashBGM) 2.0 1.0 0.0 :!class /Script/Engine.AudioComponent))))

(event EventBeginPlay
  (bind _returnvalue (Audio|SpawnSound2D "/Game/_Users/Sounds/A_BGM5_Cue.A_BGM5_Cue" 1.0 0.9 0.0 0 false false))
  (bind _output_get (Variables|Default|SetDefaultBGM _returnvalue))
  (Audio|Components|Audio|Stop _output_get)
  (bind _returnvalue_2 (Audio|SpawnSound2D "/Game/_Users/Sounds/A_Dash1_Cue.A_Dash1_Cue" 1.0 1.0 0.0 0 false false))
  (bind _output_get_2 (Variables|Default|SetDashBGM _returnvalue_2))
  (Audio|Components|Audio|Stop _output_get_2)
  (Audio|Components|Audio|FadeIn (Variables|Default|GetDefaultBGM) 1.0 1.0 0.0 :!class /Script/Engine.AudioComponent))

(fn ConstructionScript)