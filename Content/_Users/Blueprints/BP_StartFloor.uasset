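; BP_StartFloor is a start-area floor with two door-like cubes that slide along their own splines when play begins.
; BeginPlay snaps both cubes to their spline ends, waits briefly, then calls Move in reverse.
; Move plays a door sound and runs one timeline forward or backward, scaling each spline's length by the track value to position both cubes.
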(event Custom|Move
  (params (bIsReverse :type Boolean))
  (bind _spline1 (Variables|Default|GetSpline1))
  (bind _spline (Variables|Default|GetSpline))
  (Audio|PlaySoundatLocation "/Game/_Users/Blueprints/Door/Sounds/A_StartDoor_Cue.A_StartDoor_Cue" (Transformation|GetActorLocation) "0, 0, 0" 1.0 1.0 0.0 0 0 0)
  (if bIsReverse
    (bind _newtrack_0 (Timeline|Timeline_0 ReverseFromEnd)
      (:Update
        (Transformation|SetWorldLocation (Variables|Default|GetCube) (Spline|GetLocationatDistanceAlongSpline _spline (* (Spline|GetSplineLength _spline) _newtrack_0) "World") false false)
        (Transformation|SetWorldLocation (Variables|Default|GetCube1) (Spline|GetLocationatDistanceAlongSpline _spline1 (* (Spline|GetSplineLength _spline1) _newtrack_0) "World") false false)))
    (else
      (Timeline|Timeline_0 PlayFromStart))))

(event EventBeginPlay
  (bind _spline (Variables|Default|GetSpline))
  (bind _spline1 (Variables|Default|GetSpline1))
  (Transformation|SetWorldLocation (Variables|Default|GetCube) (Spline|GetLocationatDistanceAlongSpline _spline (Spline|GetSplineLength _spline) "World") false false)
  (Transformation|SetWorldLocation (Variables|Default|GetCube1) (Spline|GetLocationatDistanceAlongSpline _spline1 (Spline|GetSplineLength _spline1) "World") false false)
  (Utilities|FlowControl|Delay 0.8)
  (CallFunction|Move true))

(fn ConstructionScript)