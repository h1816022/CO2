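; Game state Blueprint that tracks how many enemies are in chase mode and signals when the chase is over.
; Increment and decrement functions maintain the count and the Chasing flag.
; When the count drops to zero, it plays a release alert and tells the first BP_SoundManager found to restore default BGM.
; The alert cue is briefly played, cut, then replayed with a fade-out.
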(event Custom|ReleaseAlert
  (bind _returnvalue (Audio|SpawnSound2D "/Game/_Users/A_ReleaseAlert_Cue.A_ReleaseAlert_Cue" 1.0 1.0 0.0 0))
  (Utilities|FlowControl|Delay 0.1)
  (Components|DestroyComponent _returnvalue)
  (Utilities|FlowControl|Delay 0.05)
  (bind _returnvalue_2 (Audio|SpawnSound2D "/Game/_Users/A_ReleaseAlert_Cue.A_ReleaseAlert_Cue" 1.0 1.0 0.0 0))
  (Audio|Components|Audio|FadeOut _returnvalue_2 2.0 0.0 :!class /Script/Engine.AudioComponent))

(fn ConstructionScript)

(fn IncrementChaseModeEnemiesNum
  (Math|Integer|IncrementInt (Variables|Default|GetChaseModeEnemiesNum)
    (:%20%20
      (Variables|Default|SetbChasing true))))

(fn DecrementChaseModeEnemiesNum
  (bind _result (Math|Integer|DecrementInt (Variables|Default|GetChaseModeEnemiesNum))
    (:%20%20
      (if (== _result 0)
        (Variables|Default|SetbChasing false)
        (CallFunction|ReleaseAlert)
        (bind _outactors (Actor|GetAllActorsOfClass "/Game/_Users/Blueprints/BP_SoundManager.BP_SoundManager_C"))
        (Default|ChangeBGM (Utilities|Array|Get(acopy) _outactors) true 0.0)))))