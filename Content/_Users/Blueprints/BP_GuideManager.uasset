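; BP_GuideManager manages the on-screen button guide widgets and a guide message.
; Adding a guide creates a timed WBP_ButtonGuide, sorts the list by descending button type, keeping one entry per type, and spreads the widgets horizontally with spacing scaled by count.
; Removing guides re-sorts the list without repositioning the remaining widgets.
; Only one WBP_GuideMessage is tracked, and a new message replaces the current one.
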(fn ConstructionScript)

(fn AdjustGuideLocation
  (bind _buttonguidewidgets (Variables|Default|GetButtonGuideWidgets))
  (CallFunction|SortGuideWidgets)
  (LocalVariables|SetRate (- 1.3 (/ (Math|Conversions|ToFloat(Integer) (Utilities|Array|Length (Variables|Default|GetButtonGuideWidgets))) 2e+01)))
  (for (_array_element _array_index) _buttonguidewidgets
    (Class|UserWidget|SetPositioninViewport _array_element (Math|Vector2D|MakeVector2D (- (* 3.6e+02 (LocalVariables|GetRate)) (* (* (+ _array_index 1) (/ 7.2e+02 (Math|Conversions|ToFloat(Integer) (+ (Utilities|Array|Length _buttonguidewidgets) 1)))) (LocalVariables|GetRate))) 0.0) true)))

(fn AddButtonGuide
  (params (ButtonType :type EButtonTypes%20Enum :default "NewEnumerator0") (Text :type Text) (LifeTime :type Float%20%28single-precision%29))
  (bind _returnvalue (UserInterface|CreateWidget "/Game/_Users/Widgets/Blueprints/WBP_ButtonGuide.WBP_ButtonGuide_C" 0 ButtonType Text LifeTime))
  (UserInterface|Viewport|AddtoViewport _returnvalue 0)
  (Utilities|Array|Add (Variables|Default|GetButtonGuideWidgets) _returnvalue)
  (CallFunction|AdjustGuideLocation)
  (return _returnvalue))

(fn SortGuideWidgets
  (bind _returnvalue (Utilities|Enum|LiteralenumEButtonTypes "NewEnumerator10"))
  (bind _returnvalue_2 (Math|Conversions|ToInteger(Byte) _returnvalue))
  (bind _returnvalue_3 (- _returnvalue_2 1))
  (for _index (range 0 _returnvalue_3)
    (bind _array_element (Utilities|Array|ForEachLoopwithBreak (Variables|Default|GetButtonGuideWidgets) :!label _label)
      (:LoopBody
        (if (== (- _returnvalue_3 _index) (Math|Conversions|ToInteger(Byte) (Variables|/Game/_Users/Widgets/Blueprints/WBP_ButtonGuide.WBP_ButtonGuide_C|GetButtonType _array_element)))
          (Utilities|Array|Add (LocalVariables|GetNewArray) _array_element)
          (goto _label Break)))))
  (Variables|Default|SetButtonGuideWidgets (LocalVariables|GetNewArray)))

(fn RemoveButtonGuide
  (params (TargetWidget :type WBP%20Button%20Guide%20Object%20Reference))
  (Utilities|Array|RemoveItem (Variables|Default|GetButtonGuideWidgets) TargetWidget)
  (Default|Remove TargetWidget)
  (CallFunction|SortGuideWidgets))

(fn RemoveButtonGuides
  (params (Target%20Widgets :type Array%20of%20WBP%20Button%20Guide%20Object%20References))
  (for _array_element Target%20Widgets
    (Utilities|Array|RemoveItem (Variables|Default|GetButtonGuideWidgets) _array_element)
    (Default|Remove _array_element))
  (CallFunction|SortGuideWidgets))

(fn ChangeGuideMessage
  (params (Text :type Text) (LifeTime :type Float%20%28single-precision%29))
  (Utilities|IsValid (Variables|Default|GetNowMessage)
    (:Is%20Valid
      (Default|Remove (Variables|Default|GetNowMessage)))
    (:Is%20Not%20Valid
      _))
  (bind _returnvalue (UserInterface|CreateWidget "/Game/_Users/Widgets/Blueprints/WBP_GuideMessage.WBP_GuideMessage_C" 0 Text LifeTime))
  (bind _output_get (Variables|Default|SetNowMessage _returnvalue))
  (UserInterface|Viewport|AddtoViewport _output_get 0))

(fn RemoveGuideMessage
  (Utilities|IsValid (Variables|Default|GetNowMessage)
    (:Is%20Valid
      (Default|Remove (Variables|Default|GetNowMessage)))))