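; BP_Next is an actor that bobs vertically around its placed location until the player's goal event removes it.
; A timeline scales Length into a Z offset from the saved start location, and a FlipFlop re-entered on each finish alternates forward and reverse playback endlessly.
; After the first pass, a DoOnce binds Goal_Event to BP_Player's goal event, which destroys the actor.
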(event Custom|Goal_Event
  (Actor|DestroyActor))

(event EventBeginPlay
  (Variables|Default|SetDefaultLocation (Transformation|GetActorLocation))
  (Utilities|FlowControl|FlipFlop :!label _label
    (:A
      (bind _newtrack_0 (Timeline|Timeline_0 PlayFromStart)
        (:Update
          (Transformation|SetActorLocation (+ (* (Math|Vector|MakeVector 0.0 0.0 (Variables|Default|GetLength)) _newtrack_0) (Variables|Default|GetDefaultLocation)) false false))
        (:Finished
          (Utilities|FlowControl|Delay 0.0)
          (Utilities|FlowControl|Sequence
            (:then_0
              (goto _label))
            (:then_1
              (Utilities|FlowControl|DoOnce false
                (:Completed
                  (EventDispatchers|BindEventtoGoal (.AsBP%20Player (Utilities|Casting|CastToBP_Player (Game|Player|GetPlayerPawn 0))) (delegate Custom|Goal_Event)))))))))
    (:B
      (Timeline|Timeline_0 ReverseFromEnd))))

(fn ConstructionScript)