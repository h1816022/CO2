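; Door sensor Blueprint that opens and closes a referenced Door based on overlaps with its Box component.
; Begin overlap calls Open and end overlap calls Close directly, without filtering the actor or checking whether others remain inside.
; A CheckOverlapping function scans the box for any BP_Player or BP_Enemy, but neither overlap event calls it.
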(event OnComponentBeginOverlap(Box)
  (params (OverlappedComponent :type Primitive%20Component%20Object%20Reference) (OtherActor :type Actor%20Object%20Reference) (OtherComp :type Primitive%20Component%20Object%20Reference) (OtherBodyIndex :type Integer) (bFromSweep :type Boolean) (SweepResult :type Hit%20Result%20Structure%20%28by%20ref%29))
  (Default|Open (Variables|Default|GetDoor)))

(event OnComponentEndOverlap(Box)
  (params (OverlappedComponent :type Primitive%20Component%20Object%20Reference) (OtherActor :type Actor%20Object%20Reference) (OtherComp :type Primitive%20Component%20Object%20Reference) (OtherBodyIndex :type Integer))
  (Default|Close (Variables|Default|GetDoor)))

(fn ConstructionScript)

(fn CheckOverlapping
  (bind _array_element (Utilities|Array|ForEachLoopwithBreak (Collision|GetOverlappingActors (Variables|Default|GetBox) 0 :!class /Script/Engine.PrimitiveComponent) :!label _label)
    (:LoopBody
      (Utilities|Casting|CastToBP_Player _array_element
        (:then
          _)
        (:CastFailed
          (Utilities|Casting|CastToBP_Enemy _array_element)))
      (LocalVariables|SetbReturn true)
      (goto _label Break))
    (:Completed
      (return (LocalVariables|GetbReturn)))))