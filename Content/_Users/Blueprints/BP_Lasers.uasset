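; Laser hazard that fires a particle beam along its forward axis and damages the player's bottle or any BP_Bottle it hits.
; Emit resets and activates the beam; Tick grows its end up to MaxLength, and while EmitStop is set advances the start too, deactivating at near-zero length.
; A per-tick trace clips the beam and places three staggered hit effects on bottle or player hits.
; The EmitStop timer check is unwired.
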(event Custom|ActiveHitEffects
  (bind _bemeffect1 (Variables|Default|GetBemEffect1))
  (if (not (Components|Activation|IsActive _bemeffect1))
    (Components|Activation|Activate _bemeffect1 false)
    (Utilities|FlowControl|Delay 0.05)
    (Components|Activation|Activate (Variables|Default|GetBemEffect2) false)
    (Utilities|FlowControl|Delay 0.03)
    (Components|Activation|Activate (Variables|Default|GetBemEffect3) false)))

(event EventTick
  (params (DeltaSeconds :type Float%20%28single-precision%29))
  (bind _returnvalue (Utilities|Time|GetWorldDeltaSeconds))
  (bind _speed (Variables|Default|GetSpeed))
  (bind _bemeffect (Variables|Default|GetBemEffect))
  (bind _returnvalue_2 (Transformation|GetWorldTransform _bemeffect))
  (bind _returnvalue_3 (* _returnvalue _speed))
  (bind _returnvalue_4 (Math|Vector|GetForwardVector (.rotation _returnvalue_2)))
  (if (Components|Activation|IsActive (Variables|Default|GetBemEffect))
    (Utilities|FlowControl|Sequence
      (:then_0
        (if (Variables|Default|GetbEmitStop)
          ;[1 1 1] ビームの照射が終わってからの処理
          (CallFunction|SetEmitEndDistance (+ (Variables|Default|GetEndDistance) _returnvalue_3))
          (CallFunction|SetEmitStartDistance (+ (Variables|Default|GetStartDistance) _returnvalue_3))
          (else
            ;[1 1 1] ビーム照射中
            (CallFunction|SetEmitEndDistance (+ _returnvalue_3 (Variables|Default|GetEndDistance))))))
      (:then_1
        ;[1 1 1] ビームの長さがほぼ0なら非アクティブにする
        (if (and (Variables|Default|GetbEmitStop) (< (Math|Float|Absolute(Float) (- (Variables|Default|GetStartDistance) (Variables|Default|GetEndDistance))) 1.0))
          (Components|Activation|Deactivate (Variables|Default|GetBemEffect))
          (Components|Activation|Deactivate (Variables|Default|GetBemEffect1))
          (Components|Activation|Deactivate (Variables|Default|GetBemEffect2))
          (Components|Activation|Deactivate (Variables|Default|GetBemEffect3))))
      (:then_2
        (bind _outhit (Collision|LineTraceByChannel (+ (.location _returnvalue_2) (* _returnvalue_4 (Variables|Default|GetStartDistance))) (+ (.location _returnvalue_2) (* _returnvalue_4 (Variables|Default|GetEndDistance))) "TraceTypeQuery1" true 0 "None"))
        (Class|ParticleSystemComponent|SetBeamSourcePoint (Variables|Default|GetBemEffect) 0 (.TraceStart (Collision|BreakHitResult _outhit)))
        (if (.bBlockingHit (Collision|BreakHitResult _outhit))
          ;[1 1 1] 当たっている時
          (Utilities|FlowControl|Sequence
            (:then_0
              (Class|ParticleSystemComponent|SetBeamTargetPoint (Variables|Default|GetBemEffect) 0 (.Location (Collision|BreakHitResult _outhit)))
              (CallFunction|SetEmitEndDistance (Math|Vector|VectorLength (- (Transformation|GetWorldLocation (Variables|Default|GetBemEffect)) (.Location (Collision|BreakHitResult _outhit))))))
            (:then_1
              (bind _asbp_player (Utilities|Casting|CastToBP_Player (.HitActor (Collision|BreakHitResult _outhit)))
                (:then
                  (Default|AddTypeDamage (Variables|/Game/_Users/Players/Blueprints/BP_Player.BP_Player_C|GetBottle _asbp_player) "NewEnumerator4" 1.0)
                  (CallFunction|ActiveHitEffects :!label _label)
                  (Transformation|SetWorldLocation (Variables|Default|GetBemEffect1) (.ImpactPoint (Collision|BreakHitResult _outhit)) false false)
                  (Transformation|SetWorldLocation (Variables|Default|GetBemEffect2) (.ImpactPoint (Collision|BreakHitResult _outhit)) false false)
                  (Transformation|SetWorldLocation (Variables|Default|GetBemEffect3) (.ImpactPoint (Collision|BreakHitResult _outhit)) false false))
                (:CastFailed
                  (bind _asbp_bottle (Utilities|Casting|CastToBP_Bottle (.HitActor (Collision|BreakHitResult _outhit)))
                    (:then
                      (Default|AddTypeDamage _asbp_bottle "NewEnumerator4" 1.0)
                      (goto _label))
                    (:CastFailed
                      (Components|Activation|Deactivate (Variables|Default|GetBemEffect1) :!label _label_2)
                      (Components|Activation|Deactivate (Variables|Default|GetBemEffect2))
                      (Components|Activation|Deactivate (Variables|Default|GetBemEffect3))))))))
          (else
            ;[1 1 1] 当たってない時
            (Class|ParticleSystemComponent|SetBeamTargetPoint (Variables|Default|GetBemEffect) 0 (.TraceEnd (Collision|BreakHitResult _outhit)))
            (goto _label_2)))))))

(fn ConstructionScript)

(fn Emit
  (Variables|Default|SetStartDistance 0.0)
  (Variables|Default|SetEndDistance 0.0)
  (Variables|Default|SetbEmitStop false)
  (Components|Activation|Activate (Variables|Default|GetBemEffect) false)
  (Components|Activation|Deactivate (Variables|Default|GetBemEffect1)))

(fn SetEmitStartDistance
  (params (InDistance :type Float%20%28single-precision%29))
  (Variables|Default|SetStartDistance (Math|Float|Min(Float) InDistance (Variables|Default|GetEndDistance))))

(fn SetEmitEndDistance
  (params (InDistance :type Float%20%28single-precision%29))
  (Variables|Default|SetEndDistance (Math|Float|Min(Float) InDistance (Variables|Default|GetMaxLength)))
  (CallFunction|SetEmitStartDistance (Variables|Default|GetStartDistance)))