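; BP_GoalDoor is a goal door whose panels show the GameState's RequiredAmount and can switch to an alternate look.
; BeginPlay creates dynamic materials for three "NG" planes and binds SetNum to the MapManager's Generated event.
; SetNum maps RequiredAmount to one of three NumAlpha values on those materials.
; Change reveals three other planes and destroys the NG planes, making the switch one-way.
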(event Custom|SetNum
  (if (== (Variables|/Game/_Users/Blueprints/BP_GameState.BP_GameState_C|GetRequiredAmount (.AsBP%20Game%20State (Utilities|Casting|CastToBP_GameState (Game|GetGameState)))) 0.5)
    (for _array_element (Variables|Default|GetMaterials)
      (Rendering|Material|SetScalarParameterValue _array_element "NumAlpha" 0.0 :!class /Script/Engine.MaterialInstanceDynamic))
    (elif (== (Variables|/Game/_Users/Blueprints/BP_GameState.BP_GameState_C|GetRequiredAmount (.AsBP%20Game%20State (Utilities|Casting|CastToBP_GameState (Game|GetGameState)))) 0.6)
      (for _array_element_2 (Variables|Default|GetMaterials)
        (Rendering|Material|SetScalarParameterValue _array_element_2 "NumAlpha" 0.5 :!class /Script/Engine.MaterialInstanceDynamic))
      (else
        (for _array_element_3 (Variables|Default|GetMaterials)
          (Rendering|Material|SetScalarParameterValue _array_element_3 "NumAlpha" 1.0 :!class /Script/Engine.MaterialInstanceDynamic))))))

(event EventBeginPlay
  (EventDispatchers|BindEventtoGenerated (Variables|Default|GetMapManager) (delegate Custom|SetNum))
  (bind _returnvalue (Rendering|Material|CreateDynamicMaterialInstance (Variables|Default|GetPlane) 0 "/Game/_Users/Materials/MI_GoalDoor_NG1.MI_GoalDoor_NG1" "None" :!class /Script/Engine.PrimitiveComponent))
  (Utilities|Array|Add (Variables|Default|GetMaterials) _returnvalue)
  (bind _returnvalue_2 (Rendering|Material|CreateDynamicMaterialInstance (Variables|Default|GetPlane1) 0 "/Game/_Users/Materials/MI_GoalDoor_NG2.MI_GoalDoor_NG2" "None" :!class /Script/Engine.PrimitiveComponent))
  (Utilities|Array|Add (Variables|Default|GetMaterials) _returnvalue_2)
  (bind _returnvalue_3 (Rendering|Material|CreateDynamicMaterialInstance (Variables|Default|GetPlane2) 0 "/Game/_Users/Materials/MI_GoalDoor_NG3.MI_GoalDoor_NG3" "None" :!class /Script/Engine.PrimitiveComponent))
  (Utilities|Array|Add (Variables|Default|GetMaterials) _returnvalue_3))

(fn ConstructionScript)

(fn Change
  (Rendering|SetVisibility (Variables|Default|GetPlane4) true false)
  (Rendering|SetVisibility (Variables|Default|GetPlane5) true false)
  (Rendering|SetVisibility (Variables|Default|GetPlane3) true false)
  (Components|DestroyComponent (Variables|Default|GetPlane))
  (Components|DestroyComponent (Variables|Default|GetPlane1))
  (Components|DestroyComponent (Variables|Default|GetPlane2)))