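; Temporary decal actor that spawns a decal at its own transform, using its configurable material and size.
; On BeginPlay it creates a dynamic material instance on the spawned decal, then waits for LifeSpan.
; A timeline then animates the material's Opacity parameter and destroys the actor when finished.
; The decal is spawned through SpawnDecalAtLocation, with no explicit removal of that component.
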(event EventBeginPlay
  (bind _returnvalue (Transformation|GetActorTransform))
  (bind _returnvalue_2 (Rendering|Decal|SpawnDecalatLocation (Variables|Default|GetDecalMaterial) (Math|Conversions|ToVector(Float) (Variables|Default|GetSize)) (.location _returnvalue) (.rotation _returnvalue) 0.0))
  (bind _returnvalue_3 (Rendering|Material|CreateDynamicMaterialInstance _returnvalue_2 :!class /Script/Engine.DecalComponent))
  (Variables|Default|SetMat _returnvalue_3)
  (Utilities|FlowControl|Delay (Variables|Default|GetLifeSpan))
  (bind _newtrack_0 (Timeline|Timeline_0 Play)
    (:Update
      (Rendering|Material|SetScalarParameterValue (Variables|Default|GetMat) "Opacity" _newtrack_0 :!class /Script/Engine.MaterialInstanceDynamic))
    (:Finished
      (Actor|DestroyActor))))

(fn ConstructionScript)