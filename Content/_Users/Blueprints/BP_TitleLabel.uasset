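; Title label Blueprint made up of GoGo, Mark and Mark1 components, with a shared visibility toggle.
; BeginPlay creates a dynamic material for GoGo only; the node creating the Base material is disconnected.
; UpdateBaseBrightness computes a clamped triangle-wave pulse from Time for BaseMaterial's Brightness, though nothing here calls it or advances Time.
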(event EventBeginPlay
  (bind _returnvalue (Rendering|Material|CreateDynamicMaterialInstance (Variables|Default|GetGoGo) 0 "/Game/_Users/Players/Label/Materials/MI_TitleLabelGoGo.MI_TitleLabelGoGo" "None" :!class /Script/Engine.PrimitiveComponent))
  (Variables|Materials|SetGoGoMaterial _returnvalue))

(fn ConstructionScript)

(fn UpdateBaseBrightness
  (bind _maxbasebrightness (Variables|Default|GetMaxBaseBrightness))
  (Rendering|Material|SetScalarParameterValue (Variables|Materials|GetBaseMaterial) "Brightness" (Math|Float|Clamp(Float) (* (Math|Float|Absolute(Float) (- (Math|Float|%(Float) (/ (Variables|Default|GetTime) 2.0) 2.0) 1.0)) _maxbasebrightness 1.2) 0.3 _maxbasebrightness) :!class /Script/Engine.MaterialInstanceDynamic))

(fn SetLabelVisibility
  (params (bNewVisibility :type Boolean))
  (Rendering|SetVisibility (Variables|Default|GetMark) bNewVisibility false)
  (Rendering|SetVisibility (Variables|Default|GetGoGo) bNewVisibility false)
  (Rendering|SetVisibility (Variables|Default|GetMark1) bNewVisibility false))