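; BP_WarpDevice is a paired teleporter that moves the player to its PairDevice after they stand in its cylinder for a set time.
; BeginPlay spawns a BP_WarpFire effect and creates dynamic light materials; overlap sets the fire's target scale and starts a per-frame Delay-loop timer.
; Warping triggers a camera fade and disables the destination's CanWarp, re-enabled shortly after the player leaves, preventing an immediate bounce back.
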(event OnComponentBeginOverlap(Cylinder)
  (params (OverlappedComponent :type Primitive%20Component%20Object%20Reference) (OtherActor :type Actor%20Object%20Reference) (OtherComp :type Primitive%20Component%20Object%20Reference) (OtherBodyIndex :type Integer) (bFromSweep :type Boolean) (SweepResult :type Hit%20Result%20Structure%20%28by%20ref%29))
  (if (Variables|Default|GetbCanWarp)
    (bind _asbp_player (Utilities|Casting|CastToBP_Player OtherActor))
    (Utilities|IsValid (Variables|Default|GetPlayer)
      (:Is%20Valid
        _)
      (:Is%20Not%20Valid
        (Variables|Default|SetPlayer _asbp_player)))
    (Variables|Default|SetbIsOverlapping true)
    (CallFunction|UpdateDecisionDelayTime)
    (Variables|/Game/_Users/Effects/BP_WarpFire.BP_WarpFire_C|SetTargetScaleRate (Variables|Default|GetFire) 1.0)))

(event OnComponentEndOverlap(Cylinder)
  (params (OverlappedComponent :type Primitive%20Component%20Object%20Reference) (OtherActor :type Actor%20Object%20Reference) (OtherComp :type Primitive%20Component%20Object%20Reference) (OtherBodyIndex :type Integer))
  (Utilities|Casting|CastToBP_Player OtherActor)
  (Variables|Default|SetbIsOverlapping false)
  (Utilities|FlowControl|Delay 0.2)
  (Variables|Default|SetbCanWarp true)
  (Variables|/Game/_Users/Effects/BP_WarpFire.BP_WarpFire_C|SetTargetScaleRate (Variables|Default|GetFire) 0.0))

(event Custom|UpdateDecisionDelayTime
  (if (Variables|Default|GetbIsOverlapping) :!label _label
    (Variables|Default|SetNowDecisionDelayTime (+ (Variables|Default|GetNowDecisionDelayTime) (Utilities|Time|GetWorldDeltaSeconds)))
    (if (< (Variables|Default|GetNowDecisionDelayTime) (Variables|Default|GetMaxDecisionDelayTime))
      (Utilities|FlowControl|Delay 0.0)
      (goto _label)
      (else
        (Variables|Default|SetNowDecisionDelayTime 0.0)
        (CallFunction|ExecWarp)))
    (else
      (Variables|Default|SetNowDecisionDelayTime 0.0))))

(event Custom|ExecWarp
  (bind _player (Variables|Default|GetPlayer))
  (Variables|BP_WarpDevice_C|SetbCanWarp (Variables|Default|GetPairDevice) false)
  (Transformation|SetActorLocation _player (+ (Transformation|GetActorLocation (Variables|Default|GetPairDevice)) "0, 0,20.000000") false false)
  (Default|Fade (Variables|/Game/_Users/Players/Blueprints/BP_Player.BP_Player_C|GetCamera _player) "NewEnumerator3"))

(event EventBeginPlay
  (bind _returnvalue (Game|SpawnActorfromClass "/Game/_Users/Effects/BP_WarpFire.BP_WarpFire_C" (Math|Transform|MakeTransform (Transformation|GetActorLocation) "0, 0, 0" "0.110000,0.110000,0.110000") "Undefined" 0 (Variables|Default|GetMaxDecisionDelayTime) 0))
  (Variables|Default|SetFire _returnvalue)
  (bind _returnvalue_2 (Rendering|Material|CreateDynamicMaterialInstance (Variables|Default|GetStaticMesh) 1 "/Game/_Users/Blueprints/WarpDevice/MI_warpDeviceLight.MI_WarpDeviceLight" "None" :!class /Script/Engine.PrimitiveComponent))
  (Utilities|Array|Add (Variables|Default|GetLightMaterials) _returnvalue_2)
  (bind _returnvalue_3 (Rendering|Material|CreateDynamicMaterialInstance (Variables|Default|GetFund) 0 "/Game/_Users/Blueprints/WarpDevice/MI_warpDeviceLight.MI_WarpDeviceLight" "None" :!class /Script/Engine.PrimitiveComponent))
  (Utilities|Array|Add (Variables|Default|GetLightMaterials) _returnvalue_3))

(fn ConstructionScript)