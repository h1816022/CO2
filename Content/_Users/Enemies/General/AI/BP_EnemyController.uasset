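; AI controller for BP_Enemy that switches between Patrol and Chase, running the matching tank behavior tree for each.
; Tick drives transitions from the bKnowPlayer blackboard flag and a lose-sight timeout, while state changes update the pawn's status color and patrol point.
; Hearing only prints debug text, and the sight detection logic is disconnected.
; A line-trace helper checks player visibility, looking past other enemies.
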(event OnPerceptionUpdated(Sight)
  (params (UpdatedActors :type Array%20of%20Actor%20Object%20References)))

(event OnPerceptionUpdated(Hearing)
  (params (UpdatedActors :type Array%20of%20Actor%20Object%20References))
  (for _array_element UpdatedActors
    (bind _info (Class|AIPerceptionComponent|GetActorsPerception (Variables|Default|GetHearing) _array_element)) ; 受け取った刺激情報を取り出す
    (if (.bSuccessfullySensed (Utilities|Struct|BreakAIStimulus (Utilities|Array|Get(acopy) (.lastsensedstimuli _info) 1))) ; true 聞こえた\nfalse 忘れた
      (Development|PrintString "Heard")
      (else
        (Development|PrintString "Not Heard")))))

(event EventTick
  (params (DeltaSeconds :type Float%20%28single-precision%29))
  (CallFunction|UpdateActionType)
  (if (Utilities|Enum|Equal(Enum) (Variables|Default|GetActionType) "NewEnumerator0")
    _))

(fn ConstructionScript)

(fn UpdateActionType
  (switch Utilities|FlowControl|Switch|SwitchonEActionType (Variables|Default|GetActionType)
    (:NewEnumerator0
      (if (ScalableFloat|GetValueasBool (AI|GetBlackboard 0) (Utilities|Name|MakeLiteralName "bKnowPlayer"))
        (CallFunction|ChangeActionType "NewEnumerator1")))
    (:NewEnumerator1
      (if (>= (Variables|Default|GetNowLoseSightTime) (Variables|StaticParams|GetMaxLoseSightTime))
        (CallFunction|ChangeActionType "NewEnumerator0")
        (Variables|Default|SetNowLoseSightTime 0.0)
        (AI|Components|Blackboard|SetValueasBool (AI|GetBlackboard 0) (Utilities|Name|MakeLiteralName "bKnowPlayer") false)))))

(fn ChangeActionType
  (params (InType :type EActionType%20Enum :default "NewEnumerator0"))
  (bind _output_get (Variables|Default|SetActionType InType))
  (switch Utilities|FlowControl|Switch|SwitchonEActionType _output_get
    (:NewEnumerator0
      (bind _output_get_2 (Variables|Default|SetNowBehaviorTree "/Game/_Users/Enemies/Tank/AI/BT_Tank_Patrol.BT_Tank_Patrol"))
      (AI|RunBehaviorTree _output_get_2)
      (CallFunction|InitPatrol))
    (:NewEnumerator1
      (bind _output_get_3 (Variables|Default|SetNowBehaviorTree "/Game/_Users/Enemies/Tank/AI/BT_Tank_Chase.BT_Tank_Chase"))
      (AI|RunBehaviorTree _output_get_3)
      (CallFunction|InitChase))))

(fn InitPatrol
  (bind _returnvalue (Pawn|GetControlledPawn))
  (bind _asbp_enemy (Utilities|Casting|CastToBP_Enemy _returnvalue))
  (bind _newparam (Default|GetFirstPathPoint (Variables|/Game/_Users/Enemies/General/Blueprints/BP_Enemy.BP_Enemy_C|GetCurrentPathPoints _asbp_enemy)))
  (Variables|/Game/_Users/Enemies/General/Blueprints/BP_Enemy.BP_Enemy_C|SetCurrentPathPoint _asbp_enemy _newparam)
  (AI|Components|Blackboard|SetValueasVector (Variables|Default|GetBlackboard) (Utilities|Name|MakeLiteralName "CurrentPathPoint") (Transformation|GetActorLocation _newparam))
  (CallFunction|ChangePersonStatus "NewEnumerator0"))

(fn InitChase
  (CallFunction|ChangePersonStatus "NewEnumerator2"))

(fn CheckLineTracetoPlayer
  (bind _outhits (Class|KismetSystemLibrary|LineTraceMultiforObjects (Transformation|GetActorLocation (Pawn|GetControlledPawn)) (Transformation|GetActorLocation (Game|Player|GetPlayerPawn 0)) (Utilities|Array|MakeArray "ObjectTypeQuery1" "ObjectTypeQuery2" "ObjectTypeQuery3" "ObjectTypeQuery4" "ObjectTypeQuery5" "ObjectTypeQuery6") false 0 "None" true))
  (bind _array_element (Utilities|Array|ForEachLoopwithBreak _outhits :!label _label)
    (:LoopBody
      (Utilities|Casting|CastToBP_Enemy (.hitactor _array_element)
        (:CastFailed
          (Utilities|Casting|CastToBP_Player (.hitactor _array_element)
            (:then
              (LocalVariables|SetbReturn true)
              (goto _label Break))
            (:CastFailed
              (goto _label Break))))))
    (:Completed
      (return (LocalVariables|GetbReturn)))))

(fn ChangePersonStatus
  (params (InStatus :type EPersonStatus%20Enum :default "NewEnumerator0"))
  (bind _returnvalue (Pawn|GetControlledPawn))
  (bind _asbp_enemy (Utilities|Casting|CastToBP_Enemy _returnvalue))
  (if (Utilities|Enum|NotEqual(Enum) (Variables|/Game/_Users/Enemies/General/Blueprints/BP_Enemy.BP_Enemy_C|GetPersonStatus _asbp_enemy) InStatus)
    (Variables|/Game/_Users/Enemies/General/Blueprints/BP_Enemy.BP_Enemy_C|SetPersonStatus _asbp_enemy InStatus)
    (Default|UpdateColor _asbp_enemy)))