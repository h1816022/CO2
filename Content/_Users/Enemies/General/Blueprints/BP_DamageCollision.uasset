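; BP_DamageCollision is a short-lived enemy hit sphere that scales over its lifetime and detects overlap with BP_Player.
; A zero-delay loop from BeginPlay advances the timer, lerps the sphere's uniform world scale from its starting size to EndScale, and polls for overlaps.
; It destroys itself when the lifetime ends or the player is hit; a hit only prints a debug string, with no damage applied.
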(event Custom|UpdateTime
  (bind _output_get (Variables|Default|SetNowTime (+ (Variables|Default|GetNowTime) (Utilities|Time|GetWorldDeltaSeconds))))
  (if (>= _output_get (Variables|Default|GetLifeTIme))
    (Variables|Default|SetbIsDie true)))

(event Custom|UpdateSize
  (bind _nowrate (CallFunction|GetTimeRate))
  (bind _endscale (Variables|Default|GetEndScale))
  (bind _startscale (Variables|Default|GetStartScale))
  (bind _returnvalue (Math|Float|Lerp _startscale _endscale _nowrate))
  (Transformation|SetWorldScale3D (Variables|Default|GetSphere) (Math|Vector|MakeVector _returnvalue _returnvalue _returnvalue)))

(event Custom|HitCheck
  (if (!= (Utilities|Array|Length (Collision|GetOverlappingActors (Variables|Default|GetSphere) "/Game/_Users/Players/Blueprints/BP_Player.BP_Player_C" :!class /Script/Engine.PrimitiveComponent)) 0)
    (Development|PrintString "Hit")
    (Variables|Default|SetbIsDie true)))

(event Custom|Destroy
  (Actor|DestroyActor))

(event EventBeginPlay
  (Variables|Default|SetStartScale (.x (Transformation|GetWorldScale (Variables|Default|GetSphere))))
  (CallFunction|UpdateTime :!label _label)
  (CallFunction|UpdateSize)
  (CallFunction|HitCheck)
  (if (not (Variables|Default|GetbIsDie))
    (Utilities|FlowControl|Delay 0.0)
    (goto _label)
    (else
      (Actor|DestroyActor))))

(fn ConstructionScript)

(fn GetTimeRate
  (return (Math|Float|Clamp(Float) (/ (Variables|Default|GetNowTime) (Variables|Default|GetLifeTIme)))))