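; BP_PathPoints is a placeable actor that holds a named array of path points, apparently for enemy movement.
; The construction script shows its Name on a TextRender in the editor.
; On BeginPlay it removes that label, or prints a warning (in Japanese) if the Name is still unset.
; GetFirstPathPoint returns the first entry of the PathPoints array.
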(event EventBeginPlay
  (if (Utilities|Name|Equal(Name) (Variables|Default|GetName) "None")
    (Development|PrintString (Utilities|String|Append (Utilities|GetDisplayName self) "のNameが設定されていません"))
    (else
      (Components|DestroyComponent (Variables|Default|GetTextRender)))))

(fn ConstructionScript
  (Rendering|Components|TextRender|SetText (Variables|Default|GetTextRender) (Utilities|Text|ToText(Name) (Variables|Default|GetName))))

(fn GetFirstPathPoint
  (return (Utilities|Array|Get(acopy) (Variables|Default|GetPathPoints))))