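; BP_Enemy is an enemy character whose head, glow color and walk speed reflect its Patrol, Search or Chase status.
; Each tick it turns the socketed head's yaw toward the player when known or being sighted, otherwise forward, or spins it two turns when flagged.
; Emissive color and eased walk speed come from DT_PersonStatusData, borrowing the Search row during Patrol when the controller reports a sighting or suspicion.
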(event EventTick
  (params (DeltaSeconds :type Float%20%28single-precision%29))
  (CallFunction|UpdateHeadRotation)
  (CallFunction|UpdateColor)
  (CallFunction|UpdateMoveSpeed))

(event EventBeginPlay
  (Transformation|AttachComponentToComponent (Variables|Default|GetHead) (Variables|Character|GetMesh) "HeadLocation" "SnapToTarget" "SnapToTarget" "KeepRelative" true))

(fn ConstructionScript)

(fn UpdateColor
  (switch Utilities|FlowControl|Switch|SwitchonEPersonStatus (Variables|Default|GetPersonStatus)
    (:NewEnumerator0
      (if (!= (Variables|/Game/_Users/Enemies/General/AI/BP_EnemyController.BP_EnemyController_C|GetNowFindSightTime (.AsBP%20Enemy%20Controller (Utilities|Casting|CastToBP_EnemyController (Pawn|GetController)))) 0.0)
        (bind _returnvalue (Utilities|GetDataTableRow "/Game/_Users/Enemies/General/Data/DT_PersonStatusData.DT_PersonStatusData" "Search")
          (:then
            (LocalVariables|SetColor (.emissivecolor _returnvalue))))
        (else
          (bind _returnvalue_2 (Utilities|GetDataTableRow "/Game/_Users/Enemies/General/Data/DT_PersonStatusData.DT_PersonStatusData" (Utilities|String|StringToName (Utilities|String|EnumtoString (Variables|Default|GetPersonStatus))) :!label _label)
            (:then
              (LocalVariables|SetColor (.emissivecolor _returnvalue_2)))))))
    (:NewEnumerator1
      (goto _label))
    (:NewEnumerator2
      (goto _label)))
  (Rendering|Material|SetVectorParameterValue (Variables|Default|GetBodyMat) "EmissiveColor" (LocalVariables|GetColor) :!class /Script/Engine.MaterialInstanceDynamic)
  (Rendering|Material|SetVectorParameterValue (Variables|Default|GetHeadMat) "EmissiveColor" (LocalVariables|GetColor) :!class /Script/Engine.MaterialInstanceDynamic))

(fn UpdateHeadRotation
  (bind _head (Variables|Default|GetHead))
  (if (Variables|Default|GetbIsHeadRotaAround)
    (Variables|Default|SetHeadRotationValue (+ (Variables|Default|GetHeadRotationValue) (* (Utilities|Time|GetWorldDeltaSeconds) 1e+02)))
    (Transformation|SetWorldRotation (Variables|Default|GetHead) (Math|Rotator|MakeRotator (.roll (Variables|Default|GetHeadRotation)) (.pitch (Variables|Default|GetHeadRotation)) (+ (.yaw (Variables|Default|GetHeadRotation)) (Variables|Default|GetHeadRotationValue))) false false)
    (if (>= (Variables|Default|GetHeadRotationValue) 7.2e+02)
      (CallFunction|EndHeadRotaAround))
    (else
      (Transformation|SetWorldRotation (Variables|Default|GetHead) (Variables|Default|GetHeadRotation) false false)
      (if (ScalableFloat|GetValueasBool (AI|GetBlackboard 0) (Utilities|Name|MakeLiteralName "bKnowPlayer"))
        (LocalVariables|SetSpeed 5.0)
        (LocalVariables|SetTargetLocation (Transformation|GetActorLocation (Game|Player|GetPlayerPawn 0)) :!label _label)
        (elif (!= (Variables|/Game/_Users/Enemies/General/AI/BP_EnemyController.BP_EnemyController_C|GetNowFindSightTime (.AsBP%20Enemy%20Controller (Utilities|Casting|CastToBP_EnemyController (Pawn|GetController)))) 0.0)
          (LocalVariables|SetSpeed 1.0)
          (goto _label)
          (else
            (LocalVariables|SetSpeed 1.0)
            (LocalVariables|SetTargetLocation (+ (Transformation|GetActorLocation) (Transformation|GetActorForwardVector))))))
      (Transformation|SetWorldRotation _head (Math|Rotator|MakeRotator 0.0 0.0 (.yaw (Math|Interpolation|RInterpTo (Transformation|GetWorldRotation (Variables|Default|GetHead)) (Math|Rotator|FindLookatRotation (Transformation|GetActorLocation) (LocalVariables|GetTargetLocation)) (Utilities|Time|GetWorldDeltaSeconds) (LocalVariables|GetSpeed)))) false false)
      (Variables|Default|SetHeadRotation (Transformation|GetWorldRotation _head)))))

(fn UpdateMoveSpeed
  (bind _charactermovement (Variables|Character|GetCharacterMovement))
  (switch Utilities|FlowControl|Switch|SwitchonEPersonStatus (Variables|Default|GetPersonStatus)
    (:NewEnumerator0
      (if (Default|CheckSuspicious (.AsBP%20Enemy%20Controller (Utilities|Casting|CastToBP_EnemyController (Pawn|GetController))))
        (bind _returnvalue (Utilities|GetDataTableRow "/Game/_Users/Enemies/General/Data/DT_PersonStatusData.DT_PersonStatusData" "Search")
          (:then
            (if (!= (Variables|Default|GetNowMoveSpeed) (.movespeed _returnvalue))
              (Variables|Default|SetNowMoveSpeed (.movespeed _returnvalue))
              (Variables|Default|SetNowMoveSpeedRate 0.0)
              (else
                (Variables|Default|SetNowMoveSpeedRate (Math|Float|Min(Float) (+ (Variables|Default|GetNowMoveSpeedRate) (Utilities|Time|GetWorldDeltaSeconds)) 1.0))))))
        (else
          (bind _returnvalue_2 (Utilities|GetDataTableRow "/Game/_Users/Enemies/General/Data/DT_PersonStatusData.DT_PersonStatusData" (Utilities|String|StringToName (Utilities|String|EnumtoString (Variables|Default|GetPersonStatus))) :!label _label)
            (:then
              (if (!= (Variables|Default|GetNowMoveSpeed) (.movespeed _returnvalue_2))
                (Variables|Default|SetNowMoveSpeed (.movespeed _returnvalue_2))
                (Variables|Default|SetNowMoveSpeedRate 0.0)
                (else
                  (Variables|Default|SetNowMoveSpeedRate (Math|Float|Min(Float) (+ (Variables|Default|GetNowMoveSpeedRate) (Utilities|Time|GetWorldDeltaSeconds)) 1.0)))))))))
    (:NewEnumerator1
      (goto _label))
    (:NewEnumerator2
      (goto _label)))
  (Variables|/Script/Engine.CharacterMovementComponent|SetMaxWalkSpeed _charactermovement (Math|Float|Lerp (Variables|/Script/Engine.CharacterMovementComponent|GetMaxWalkSpeed _charactermovement) (Variables|Default|GetNowMoveSpeed) (Variables|Default|GetNowMoveSpeedRate))))

(fn EndHeadRotaAround
  (Variables|Default|SetHeadRotationValue 0.0)
  (Variables|Default|SetbIsHeadRotaAround false))