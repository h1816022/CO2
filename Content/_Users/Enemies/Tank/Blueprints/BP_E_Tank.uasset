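; BP_E_Tank is the Tank enemy, a child Blueprint that extends its parent's startup logic.
; On BeginPlay it creates and stores dynamic material instances for the body mesh and head.
; It then has its BP_EnemyController run the BT_Tank_Patrol behavior tree and set an initial action type.
; It also caches the mesh's ABP_Tank animation instance, while the construction script only calls the parent.
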(event EventBeginPlay
  (bind _returnvalue (Pawn|GetController))
  (bind _asbp_enemy_controller (Utilities|Casting|CastToBP_EnemyController _returnvalue))
  (|CallParentFunction)
  (bind _returnvalue_2 (Rendering|Material|CreateDynamicMaterialInstance (Variables|Character|GetMesh) 0 0 "None" :!class /Script/Engine.PrimitiveComponent))
  (Variables|Default|SetBodyMat _returnvalue_2)
  (bind _returnvalue_3 (Rendering|Material|CreateDynamicMaterialInstance (Variables|Default|GetHead) 0 0 "None" :!class /Script/Engine.PrimitiveComponent))
  (Variables|Default|SetHeadMat _returnvalue_3)
  (AI|RunBehaviorTree _asbp_enemy_controller "/Game/_Users/Enemies/Tank/AI/BT_Tank_Patrol.BT_Tank_Patrol")
  (Default|ChangeActionType _asbp_enemy_controller "NewEnumerator0")
  (Variables|Default|SetAnimBlueprint (.AsABP%20Tank (Utilities|Casting|CastToABP_Tank (Components|SkeletalMesh|GetAnimInstance (Variables|Character|GetMesh))))))

(fn ConstructionScript
  (|CallParentFunction))