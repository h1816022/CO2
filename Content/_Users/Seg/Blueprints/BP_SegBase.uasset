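; Base Blueprint for a three-digit seven-segment display that counts toward a target number and colours itself by value range.
; BeginPlay gives each segment a dynamic material, then runs Delay loops that step the number, advance animation state and refresh materials.
; Each refresh sets colour and per-segment Switch parameters from digit bitmasks with leading-zero blanking, random flicker or a figure-eight chase, or turns all segments off.
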(event Custom|UpdateFlags
  (for (_ _array_index) (Variables|Default|GetRandomFlags1) :!label _label
    (if (== (Utilities|Array|Get(acopy) (Variables|Default|GetRandomFlags1) _array_index) 0.0)
      (Utilities|Array|SetArrayElem (Variables|Default|GetRandomFlags1) _array_index (CallFunction|GetRandomNum 6))
      (else
        (Utilities|Array|SetArrayElem (Variables|Default|GetRandomFlags1) _array_index 0.0))))
  (for (_ _array_index_2) (Variables|Default|GetRandomFlags10)
    (if (== (Utilities|Array|Get(acopy) (Variables|Default|GetRandomFlags10) _array_index_2) 0.0)
      (Utilities|Array|SetArrayElem (Variables|Default|GetRandomFlags10) _array_index_2 (CallFunction|GetRandomNum 6))
      (else
        (Utilities|Array|SetArrayElem (Variables|Default|GetRandomFlags10) _array_index_2 0.0))))
  (for (_ _array_index_3) (Variables|Default|GetRandomFlags100)
    (if (== (Utilities|Array|Get(acopy) (Variables|Default|GetRandomFlags100) _array_index_3) 0.0)
      (Utilities|Array|SetArrayElem (Variables|Default|GetRandomFlags100) _array_index_3 (CallFunction|GetRandomNum 6))
      (else
        (Utilities|Array|SetArrayElem (Variables|Default|GetRandomFlags100) _array_index_3 0.0))))
  (Variables|Default|SetNowIndex (Math|Integer|%(Integer) (+ (Variables|Default|GetNowIndex) 1) 8))
  (Utilities|FlowControl|Delay 0.03)
  (goto _label))

(event EventBeginPlay
  (for _array_element (Utilities|Array|MakeArray (Variables|Default|GetSeg0) (Variables|Default|GetSeg1) (Variables|Default|GetSeg2) (Variables|Default|GetSeg3) (Variables|Default|GetSeg4) (Variables|Default|GetSeg5) (Variables|Default|GetSeg6))
    (Utilities|Array|Add (Variables|Default|GetAllSegParts) _array_element)
    (bind _returnvalue (Rendering|Material|CreateDynamicMaterialInstance _array_element 0 "/Game/_Users/Seg/Materials/MI_Seg.MI_Seg" "None" :!class /Script/Engine.PrimitiveComponent))
    (Utilities|Array|Add (Variables|Default|GetSegMaterials1) _returnvalue))
  (for _array_element_2 (Utilities|Array|MakeArray (Variables|Default|GetSeg7) (Variables|Default|GetSeg8) (Variables|Default|GetSeg9) (Variables|Default|GetSeg10) (Variables|Default|GetSeg11) (Variables|Default|GetSeg12) (Variables|Default|GetSeg13))
    (Utilities|Array|Add (Variables|Default|GetAllSegParts) _array_element_2)
    (bind _returnvalue_2 (Rendering|Material|CreateDynamicMaterialInstance _array_element_2 0 "/Game/_Users/Seg/Materials/MI_Seg.MI_Seg" "None" :!class /Script/Engine.PrimitiveComponent))
    (Utilities|Array|Add (Variables|Default|GetSegMaterials10) _returnvalue_2))
  (for _array_element_3 (Utilities|Array|MakeArray (Variables|Default|GetSeg14) (Variables|Default|GetSeg15) (Variables|Default|GetSeg16) (Variables|Default|GetSeg17) (Variables|Default|GetSeg18) (Variables|Default|GetSeg19) (Variables|Default|GetSeg20))
    (Utilities|Array|Add (Variables|Default|GetAllSegParts) _array_element_3)
    (bind _returnvalue_3 (Rendering|Material|CreateDynamicMaterialInstance _array_element_3 0 "/Game/_Users/Seg/Materials/MI_Seg.MI_Seg" "None" :!class /Script/Engine.PrimitiveComponent))
    (Utilities|Array|Add (Variables|Default|GetSegMaterials100) _returnvalue_3))
  (Utilities|Array|Resize (Variables|Default|GetRandomFlags1) (Utilities|Array|Length (Variables|Default|GetSegMaterials1)))
  (Utilities|Array|Resize (Variables|Default|GetRandomFlags10) (Utilities|Array|Length (Variables|Default|GetSegMaterials10)))
  (Utilities|Array|Resize (Variables|Default|GetRandomFlags100) (Utilities|Array|Length (Variables|Default|GetSegMaterials100)))
  (Utilities|FlowControl|Sequence
    (:then_0
      (CallFunction|UpdateNumber :!label _label)
      (Utilities|FlowControl|Delay 0.0)
      (goto _label))
    (:then_1
      (CallFunction|LerpNumber :!label _label_2)
      (Utilities|FlowControl|Delay 0.01)
      (goto _label_2))
    (:then_2
      (CallFunction|UpdateFlags))))

(fn ConstructionScript)

(fn UpdateNumber
  (CallFunction|UpdateColor)
  (if (Variables|Default|GetbIsOn)
    (switch Utilities|FlowControl|Switch|SwitchonESegType (Variables|Default|GetNowType)
      (:NewEnumerator0
        (CallFunction|UpdateNumberDefault (LocalVariables|GetBinaryValues)))
      (:NewEnumerator1
        (CallFunction|UpdateNumberRandom))
      (:NewEnumerator2
        (CallFunction|UpdateNumberEightFigure)))
    (else
      (CallFunction|OffSeg))))

(fn LerpNumber
  (if (> (Variables|Default|GetTargetNum) (Variables|Default|GetNowNum))
    (Math|Integer|IncrementInt (Variables|Default|GetNowNum))
    (elif (< (Variables|Default|GetTargetNum) (Variables|Default|GetNowNum))
      (Math|Integer|DecrementInt (Variables|Default|GetNowNum)))))

(fn UpdateColor
  (LocalVariables|SetColor (CallFunction|GetNowColor))
  (for _array_element (Variables|Default|GetSegMaterials1)
    (Rendering|Material|SetVectorParameterValue _array_element "Color" (LocalVariables|GetColor) :!class /Script/Engine.MaterialInstanceDynamic))
  (for _array_element_2 (Variables|Default|GetSegMaterials10)
    (Rendering|Material|SetVectorParameterValue _array_element_2 "Color" (LocalVariables|GetColor) :!class /Script/Engine.MaterialInstanceDynamic))
  (for _array_element_3 (Variables|Default|GetSegMaterials100)
    (Rendering|Material|SetVectorParameterValue _array_element_3 "Color" (LocalVariables|GetColor) :!class /Script/Engine.MaterialInstanceDynamic)))

(fn SetSegVisibility
  (params (bNewVisibility :type Boolean))
  (for _array_element (Variables|Default|GetAllSegParts)
    (Rendering|SetVisibility _array_element bNewVisibility false)))

(fn GetNowColor
  (if (== (Variables|Default|GetNowNum) 0)
    (LocalVariables|SetColor (Utilities|Array|Get(acopy) (Variables|Default|GetColors) 3))
    (elif (< (Variables|Default|GetNowNum) 30)
      (LocalVariables|SetColor (Utilities|Array|Get(acopy) (Variables|Default|GetColors) 2))
      (elif (< (Variables|Default|GetNowNum) 70)
        (LocalVariables|SetColor (Utilities|Array|Get(acopy) (Variables|Default|GetColors) 1))
        (else
          (LocalVariables|SetColor (Utilities|Array|Get(acopy) (Variables|Default|GetColors)))))))
  (return (LocalVariables|GetColor)))

(fn OffSeg
  (for _array_element (Variables|Default|GetSegMaterials1)
    (Rendering|Material|SetScalarParameterValue _array_element "Switch" 0.0 :!class /Script/Engine.MaterialInstanceDynamic))
  (for _array_element_2 (Variables|Default|GetSegMaterials10)
    (Rendering|Material|SetScalarParameterValue _array_element_2 "Switch" 0.0 :!class /Script/Engine.MaterialInstanceDynamic))
  (for _array_element_3 (Variables|Default|GetSegMaterials100)
    (Rendering|Material|SetScalarParameterValue _array_element_3 "Switch" 0.0 :!class /Script/Engine.MaterialInstanceDynamic)))

(fn GetRandomNum
  (params (Rate :type Integer))
  (if (== (Math|Random|RandomInteger Rate) 0)
    (return 1.0)
    (else
      (return 0.0))))

(fn UpdateNumberDefault
  (params (BinaryValues :type Array%20of%20Integers))
  (LocalVariables|SetNumber (Variables|Default|GetNowNum))
  (for _array_element (Variables|Default|GetSegMaterials1)
    (Rendering|Material|SetScalarParameterValue _array_element "Switch" (select (> (Class|KismetMathLibrary|AndIntInt (Utilities|Array|Get(acopy) BinaryValues (Math|Integer|%(Integer) (LocalVariables|GetNumber) 10)) (LocalVariables|GetPlaseValue)) 0) 1.0 0.0) :!class /Script/Engine.MaterialInstanceDynamic)
    (LocalVariables|SetPlaseValue (* (LocalVariables|GetPlaseValue) 2)))
  (LocalVariables|SetNumber (/ (- (LocalVariables|GetNumber) (Math|Integer|%(Integer) (LocalVariables|GetNumber) 10)) 10))
  (LocalVariables|SetPlaseValue 1)
  (for _array_element_2 (Variables|Default|GetSegMaterials10)
    (if (< (Variables|Default|GetNowNum) 10)
      (Rendering|Material|SetScalarParameterValue _array_element_2 "Switch" 0.0 :!class /Script/Engine.MaterialInstanceDynamic)
      (else
        (Rendering|Material|SetScalarParameterValue _array_element_2 "Switch" (select (> (Class|KismetMathLibrary|AndIntInt (Utilities|Array|Get(acopy) BinaryValues (Math|Integer|%(Integer) (LocalVariables|GetNumber) 10)) (LocalVariables|GetPlaseValue)) 0) 1.0 0.0) :!class /Script/Engine.MaterialInstanceDynamic)))
    (LocalVariables|SetPlaseValue (* (LocalVariables|GetPlaseValue) 2)))
  (LocalVariables|SetNumber (/ (- (LocalVariables|GetNumber) (Math|Integer|%(Integer) (LocalVariables|GetNumber) 10)) 10))
  (LocalVariables|SetPlaseValue 1)
  (for _array_element_3 (Variables|Default|GetSegMaterials100)
    (if (< (Variables|Default|GetNowNum) 100)
      (Rendering|Material|SetScalarParameterValue _array_element_3 "Switch" 0.0 :!class /Script/Engine.MaterialInstanceDynamic)
      (else
        (Rendering|Material|SetScalarParameterValue _array_element_3 "Switch" (select (> (Class|KismetMathLibrary|AndIntInt (Utilities|Array|Get(acopy) BinaryValues (Math|Integer|%(Integer) (LocalVariables|GetNumber) 10)) (LocalVariables|GetPlaseValue)) 0) 1.0 0.0) :!class /Script/Engine.MaterialInstanceDynamic)))
    (LocalVariables|SetPlaseValue (* (LocalVariables|GetPlaseValue) 2))))

(fn UpdateNumberRandom
  (for (_array_element _array_index) (Variables|Default|GetSegMaterials1)
    (Rendering|Material|SetScalarParameterValue _array_element "Switch" (Utilities|Array|Get(acopy) (Variables|Default|GetRandomFlags1) _array_index) :!class /Script/Engine.MaterialInstanceDynamic))
  (for (_array_element_2 _array_index_2) (Variables|Default|GetSegMaterials10)
    (Rendering|Material|SetScalarParameterValue _array_element_2 "Switch" (Utilities|Array|Get(acopy) (Variables|Default|GetRandomFlags10) _array_index_2) :!class /Script/Engine.MaterialInstanceDynamic))
  (for (_array_element_3 _array_index_3) (Variables|Default|GetSegMaterials100)
    (Rendering|Material|SetScalarParameterValue _array_element_3 "Switch" (Utilities|Array|Get(acopy) (Variables|Default|GetRandomFlags100) _array_index_3) :!class /Script/Engine.MaterialInstanceDynamic)))

(fn UpdateNumberEightFigure
  (bind _segmaterials1 (Variables|Default|GetSegMaterials1))
  (bind _segmaterials100 (Variables|Default|GetSegMaterials100))
  (bind _segmaterials10 (Variables|Default|GetSegMaterials10))
  (for _array_element _segmaterials1
    (Rendering|Material|SetScalarParameterValue _array_element "Switch" 0.0 :!class /Script/Engine.MaterialInstanceDynamic))
  (Rendering|Material|SetScalarParameterValue (Utilities|Array|Get(acopy) _segmaterials1 (Utilities|Array|Get(acopy) (Variables|Default|GetEightFigureIndices) (Variables|Default|GetNowIndex))) "Switch" 1.0 :!class /Script/Engine.MaterialInstanceDynamic)
  (for _array_element_2 _segmaterials10
    (Rendering|Material|SetScalarParameterValue _array_element_2 "Switch" 0.0 :!class /Script/Engine.MaterialInstanceDynamic))
  (Rendering|Material|SetScalarParameterValue (Utilities|Array|Get(acopy) _segmaterials10 (Utilities|Array|Get(acopy) (Variables|Default|GetEightFigureIndices) (Variables|Default|GetNowIndex))) "Switch" 1.0 :!class /Script/Engine.MaterialInstanceDynamic)
  (for _array_element_3 _segmaterials100
    (Rendering|Material|SetScalarParameterValue _array_element_3 "Switch" 0.0 :!class /Script/Engine.MaterialInstanceDynamic))
  (Rendering|Material|SetScalarParameterValue (Utilities|Array|Get(acopy) _segmaterials100 (Utilities|Array|Get(acopy) (Variables|Default|GetEightFigureIndices) (Variables|Default|GetNowIndex))) "Switch" 1.0 :!class /Script/Engine.MaterialInstanceDynamic))