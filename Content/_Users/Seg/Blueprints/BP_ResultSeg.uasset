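; Result-segment actor, judging by its name, that takes the game state's cleared-map count as its target number.
; On BeginPlay it sets its pitch from the look-at rotation running from the camera to itself, then calls the parent's BeginPlay.
; It then copies ClearMapNum from BP_GameState into TargetNum; this graph does nothing further with the value.
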(event EventBeginPlay
  (Transformation|SetActorRotation (Math|Rotator|MakeRotator 0.0 (.pitch (Math|Rotator|FindLookatRotation (Transformation|GetWorldLocation (Variables|/Game/_Users/Cameras/Blueprints/BP_ResultCamera.BP_ResultCamera_C|GetCamera (Variables|Default|GetCamera))) (Transformation|GetActorLocation))) 0.0))
  (|CallParentFunction)
  (Variables|Default|SetTargetNum (Variables|/Game/_Users/Blueprints/BP_GameState.BP_GameState_C|GetClearMapNum (.AsBP%20Game%20State (Utilities|Casting|CastToBP_GameState (Game|GetGameState))))))

(fn ConstructionScript)