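; BP_Seg is a child Blueprint that extends its parent's startup and color update, with behavior switched by an OnGame flag.
; When not in game, BeginPlay copies FixedNum into TargetNum before running the parent logic.
; In game, UpdateColor runs the parent update, then pushes the current color into the Color parameter of the Bottle label's material, if that label is valid.
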(event EventUpdateColor
  (|CallParentFunction)
  (if (Variables|Default|GetbOnGame)
    (Utilities|IsValid (Variables|/Game/_Users/Players/Bottle/Blueprints/BP_Bottle.BP_Bottle_C|GetLabel (Variables|Default|GetBottle))
      (:Is%20Valid
        (Rendering|Material|SetVectorParameterValue (Variables|/Game/_Users/Players/Label/Blueprints/BP_Label.BP_Label_C|GetBaseMaterial (Variables|/Game/_Users/Players/Bottle/Blueprints/BP_Bottle.BP_Bottle_C|GetLabel (Variables|Default|GetBottle))) "Color" (CallFunction|GetNowColor) :!class /Script/Engine.MaterialInstanceDynamic)))))

(event EventBeginPlay
  (if (not (Variables|Default|GetbOnGame))
    (Variables|Default|SetTargetNum (Variables|Default|GetFixedNum)))
  (|CallParentFunction))

(fn ConstructionScript)