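; BP_PlayerTrace is a short-lived player trace actor whose sphere scales over its lifetime and which exposes a set of trace points.
; A per-frame Delay(0) loop from BeginPlay, used instead of Tick, advances the timer and lerps the sphere's uniform scale from start to end.
; The actor destroys itself when its lifetime ends or a BP_Enemy begins overlapping the sphere.
; GetTracePoints returns the actor's location plus five child scene component positions.
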(event OnComponentBeginOverlap(Sphere)
  (params (OverlappedComponent :type Primitive%20Component%20Object%20Reference) (OtherActor :type Actor%20Object%20Reference) (OtherComp :type Primitive%20Component%20Object%20Reference) (OtherBodyIndex :type Integer) (bFromSweep :type Boolean) (SweepResult :type Hit%20Result%20Structure%20%28by%20ref%29))
  (if (not (Variables|Default|GetbIsDie))
    (Utilities|Casting|CastToBP_Enemy OtherActor)
    (Variables|Default|SetbIsDie true)))

(event Custom|UpdateTime
  (bind _output_get (Variables|Default|SetNowTime (+ (Variables|Default|GetNowTime) (Utilities|Time|GetWorldDeltaSeconds))))
  (if (>= _output_get (Variables|Default|GetLifeTIme))
    (Variables|Default|SetbIsDie true)))

(event Custom|UpdateSize
  (bind _nowrate (CallFunction|GetTimeRate))
  (bind _endscale (Variables|Default|GetEndScale))
  (bind _startscale (Variables|Default|GetStartScale))
  (bind _returnvalue (Math|Float|Lerp _startscale _endscale _nowrate))
  (Transformation|SetWorldScale3D (Variables|Default|GetSphere) (Math|Vector|MakeVector _returnvalue _returnvalue _returnvalue)))

(event EventBeginPlay
  (Variables|Default|SetStartScale (.x (Transformation|GetWorldScale (Variables|Default|GetSphere))))
  (CallFunction|UpdateTime :!label _label)
  (CallFunction|UpdateSize)
  (if (not (Variables|Default|GetbIsDie))
    (Utilities|FlowControl|Delay 0.0)
    (goto _label)
    (else
      (Actor|DestroyActor))))

(fn ConstructionScript)

(fn GetTimeRate
  (return (Math|Float|Clamp(Float) (/ (Variables|Default|GetNowTime) (Variables|Default|GetLifeTIme)))))

(fn GetTracePoints
  (return (Utilities|Array|MakeArray (Transformation|GetActorLocation) (Transformation|GetWorldLocation (Variables|Default|GetScene1)) (Transformation|GetWorldLocation (Variables|Default|GetScene2)) (Transformation|GetWorldLocation (Variables|Default|GetScene3)) (Transformation|GetWorldLocation (Variables|Default|GetScene4)) (Transformation|GetWorldLocation (Variables|Default|GetScene)))))