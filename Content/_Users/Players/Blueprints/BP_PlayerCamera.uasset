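; Player camera actor that follows control rotation and switches from third to first person while the ChangeCameraMode input is held.
; Entering first person shrinks the camera arm toward the head behind a fade, then attaches water-drop and reticle actors and swaps pitch limits.
; In first person, a forward trace times sighted enemies into the player's FindingEnemies list.
; Damage shakes the camera, and Dying replaces it with an end camera.
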(event Custom|SetFirstCamera_Event
  ;[1 1 1] 一人称視点に切り替えるとき
  (Components|Activation|Deactivate (Variables|Default|GetThirdCamera))
  (Components|Activation|Activate (Variables|Default|GetFirstCamera) false)
  (bind _returnvalue (Game|SpawnActorfromClass "/Game/_Users/Players/Blueprints/BP_WaterDrop.BP_WaterDrop_C" (Math|Transform|MakeTransform "0, 0, 0" "0, 0, 0" "1,1,1") "Undefined" 0 0))
  (Transformation|AttachComponentToComponent _returnvalue (Variables|Default|GetWaterDropSpawnPoint) "None" "SnapToTarget" "SnapToTarget" "KeepRelative" true)
  (Utilities|Array|Add (Variables|Default|GetFirstCameraActors) _returnvalue)
  (bind _returnvalue_2 (Game|SpawnActorfromClass "/Game/_Users/Players/Blueprints/BP_Reticle.BP_Reticle_C" (Math|Transform|MakeTransform "0, 0, 0" "0, 0, 0" "0.060000,0.060000,0.060000") "Undefined" 0 9e+01 false 0))
  (Transformation|AttachComponentToComponent _returnvalue_2 (Variables|Default|GetReticleSpawnPoint) "None" "SnapToTarget" "SnapToTarget" "KeepRelative" true)
  (Utilities|Array|Add (Variables|Default|GetFirstCameraActors) _returnvalue_2)
  (bind _returnvalue_3 (Game|SpawnActorfromClass "/Game/_Users/Players/Blueprints/BP_Reticle.BP_Reticle_C" (Math|Transform|MakeTransform "0, 0, 0" "0, 0, 0" "0.060000,0.060000,0.060000") "Undefined" 0 -45.0 true 0))
  (Transformation|AttachComponentToComponent _returnvalue_3 (Variables|Default|GetReticleSpawnPoint) "None" "SnapToTarget" "SnapToTarget" "KeepRelative" true)
  (Utilities|Array|Add (Variables|Default|GetFirstCameraActors) _returnvalue_3)
  (Variables|Default|SetbIsFirstPerson true)
  (Utilities|FlowControl|Delay 0.3)
  (if (Variables|Default|GetbWaitingChangeTCamera)
    (Variables|Default|SetbWaitingChangeTCamera false)
    (Default|CallSetThirdCamera))
  (Variables|Default|SetbCanChangeCamera true)
  (CallFunction|SetCameraPitch (Variables|Static|GetFCameraPitchMin) (Variables|Static|GetFCameraPitchMax)))

(event Custom|SetThirdCamera_Event
  (bind _fadewidget (Variables|Objects|GetFadeWidget))
  (bind _firstcameraactors (Variables|Default|GetFirstCameraActors))
  ;[1 1 1] 三人称視点に切り替えるとき
  (Components|Activation|Deactivate (Variables|Default|GetFirstCamera))
  (Components|Activation|Activate (Variables|Default|GetThirdCamera) false)
  (for _array_element _firstcameraactors
    (Actor|DestroyActor _array_element))
  (Utilities|Array|Clear _firstcameraactors)
  (Variables|Default|SetbIsFirstPerson false)
  (Variables|Default|SetNowCameraChangeInterval 0.0)
  (UserInterface|Animation|PlayAnimation _fadewidget (Variables|/Game/_Users/Widgets/WBP_Fade.WBP_Fade_C|GetFadeIn _fadewidget) 0.0 1 "Forward" 1.0)
  (CallFunction|SetCameraPitch (Variables|Static|GetTCameraPitchMin) (Variables|Static|GetTCameraPitchMax))
  (Variables|/Script/Engine.SpringArmComponent|SetTargetArmLength (Variables|Default|GetThirdCameraArm) 2e+02))

(event Custom|PreSetFirstCamera
  (params (TCameraLocation :type Vector) (TCameraArmLength :type Float%20%28single-precision%29))
  (bind _thirdcameraarm (Variables|Default|GetThirdCameraArm))
  (bind _fadewidget (Variables|Objects|GetFadeWidget))
  (bind _fadewidget_2 (Variables|Objects|GetFadeWidget))
  ;[1 1 1] 一人称視点のカメラに切り替える、その前の処理
  (Variables|Default|SetbCanChangeCamera false)
  (Variables|/Game/_Users/Players/Blueprints/BP_Player.BP_Player_C|SetbCanMove (Variables|Objects|GetPlayer) false)
  (UserInterface|Animation|PlayAnimation _fadewidget (Variables|/Game/_Users/Widgets/WBP_Fade.WBP_Fade_C|GetFadeOut _fadewidget) 0.0 1 "Forward" 1.0)
  (Variables|/Script/Engine.SpringArmComponent|SetTargetArmLength _thirdcameraarm (Math|Float|Max(Float) (- (Variables|/Script/Engine.SpringArmComponent|GetTargetArmLength _thirdcameraarm) (CallFunction|GetMulDeltaSeconds 1e+03)) 0.0) :!label _label)
  (Transformation|SetWorldLocation (Variables|Default|GetThirdCameraArm) (Math|Vector|Lerp(Vector) (Transformation|GetWorldLocation (Variables|Default|GetHeadLocation)) TCameraLocation (/ (Variables|/Script/Engine.SpringArmComponent|GetTargetArmLength _thirdcameraarm) TCameraArmLength)) false false)
  (if (> (Variables|/Script/Engine.SpringArmComponent|GetTargetArmLength (Variables|Default|GetThirdCameraArm)) 0.0)
    (if (not (Variables|/Game/_Users/Players/Blueprints/BP_Player.BP_Player_C|GetbIsDash (Variables|Objects|GetPlayer)))
      (Utilities|FlowControl|Delay 0.0)
      (goto _label)
      (else
        (Default|CallSetThirdCamera)
        (Variables|Default|SetbCanChangeCamera true)))
    (else
      (Default|CallSetFirstCamera)))
  (Variables|/Game/_Users/Players/Blueprints/BP_Player.BP_Player_C|SetbCanMove (Variables|Objects|GetPlayer) true)
  (UserInterface|Animation|PlayAnimation _fadewidget_2 (Variables|/Game/_Users/Widgets/WBP_Fade.WBP_Fade_C|GetWhite _fadewidget_2) 0.0 1 "Forward" 1.0))

(event Custom|Damage_Event
  (params (DamageType :type EDamageType%20Enum :default "NewEnumerator0"))
  (Class|PlayerController|ClientPlayCameraShake (Game|GetPlayerController 0) "/Game/_Users/Blueprints/BP_CameraShake.BP_CameraShake_C" 1.0 "CameraLocal" "0, 0, 0"))

(event Custom|Dying
  (CallFunction|SpawnEndCamera))

(event EventBeginPlay
  (Game|Player|SetViewTargetwithBlend (Game|GetPlayerController 0) self 0.0 "VTBlend_Linear" 0.0 false)
  (Variables|Objects|SetCameraManager (Variables|/Script/Engine.PlayerController|GetPlayerCameraManager (Game|GetPlayerController 0)))
  (Variables|Objects|SetPlayer (.AsBP%20Player (Utilities|Casting|CastToBP_Player (Game|Player|GetPlayerPawn 0))))
  (EventDispatchers|BindEventtoSetFirstCamera (delegate Custom|SetFirstCamera_Event))
  (EventDispatchers|BindEventtoSetThirdCamera (delegate Custom|SetThirdCamera_Event))
  (EventDispatchers|BindEventtoOnDamage (Variables|Objects|GetPlayer) (delegate Custom|Damage_Event))
  (bind _returnvalue (UserInterface|CreateWidget "/Game/_Users/Widgets/WBP_Fade.WBP_Fade_C"))
  (bind _output_get (Variables|Objects|SetFadeWidget _returnvalue))
  (UserInterface|Viewport|AddtoViewport _output_get 0)
  (Variables|/Script/Engine.PlayerCameraManager|SetViewPitchMin (Variables|Objects|GetCameraManager) (Variables|Static|GetTCameraPitchMin))
  (Variables|/Script/Engine.PlayerCameraManager|SetViewPitchMax (Variables|Objects|GetCameraManager) (Variables|Static|GetTCameraPitchMax)))

(event EventTick
  (params (DeltaSeconds :type Float%20%28single-precision%29))
  (Transformation|SetActorRotation (Pawn|GetControlRotation (Game|Player|GetPlayerPawn 0) :!class /Script/Engine.Pawn))
  (bind (_bishit _hitenemy) (CallFunction|SearchEnemy))
  (CallFunction|UpdateFindingEnemy _bishit _hitenemy)
  (Variables|Default|SetNowCameraChangeInterval (+ (Variables|Default|GetNowCameraChangeInterval) DeltaSeconds))
  (if (and (Variables|Default|GetbIsFirstPerson) (Utilities|Enum|Equal(Enum) (Variables|/Game/_Users/Players/Animations/ABP_CSC.ABP_CSC_C|GetModeType (Variables|/Game/_Users/Players/Blueprints/BP_Player.BP_Player_C|GetAnimBlueprint (Variables|Objects|GetPlayer))) "NewEnumerator2")) ; 主観視点中にタイヤ走行していると歩きに変更
    (Default|ChangeModeType (Variables|Objects|GetPlayer) "NewEnumerator0" false "NewEnumerator0" 0.0)))

(event Input|ActionEvents|InputActionChangeCameraMode
  (params (Key :type Key%20Structure :default "None"))
  (bind _thirdcameraarm (Variables|Default|GetThirdCameraArm))
  ;[1 1 1] 視点切り替え操作
  (:Pressed
    (if (>= (Variables|Default|GetNowCameraChangeInterval) (Variables|Static|GetMaxCameraChangeInterval))
      (if (Variables|Default|GetbCanChangeCamera)
        (if (not (Variables|/Game/_Users/Players/Blueprints/BP_Player.BP_Player_C|GetbIsDash (Variables|Objects|GetPlayer)))
          (CallFunction|PreSetFirstCamera (Transformation|GetWorldLocation _thirdcameraarm) (Variables|/Script/Engine.SpringArmComponent|GetTargetArmLength _thirdcameraarm))
          (else
            (Variables|Default|SetbFailureCameraChange true :!label _label)))
        (else
          (goto _label)))
      (else
        (goto _label))))
  (:Released
    (if (not (Variables|Default|GetbFailureCameraChange))
      (if (Variables|Default|GetbCanChangeCamera)
        (if (Variables|Default|GetbIsFirstPerson)
          (Default|CallSetThirdCamera))
        (else
          (Variables|Default|SetbWaitingChangeTCamera true)))
      (else
        (Variables|Default|SetbFailureCameraChange false)))))

(fn ConstructionScript)

(fn SearchEnemy
  (bind _firstcamera (Variables|Default|GetFirstCamera))
  (bind _returnvalue (Transformation|GetWorldLocation _firstcamera))
  (if (Variables|Default|GetbIsFirstPerson)
    (bind _outhits (Collision|MultiLineTraceByChannel _returnvalue (+ _returnvalue (* (Math|Vector|GetForwardVector _firstcamera) 1e+04)) "TraceTypeQuery2" false 0 "None"))
    (for _array_element _outhits :!label _label
      (Utilities|Casting|CastToBP_Player (.hitactor _array_element)
        (:then
          (goto _label))
        (:CastFailed
          (bind _asbp_enemy (Utilities|Casting|CastToBP_Enemy (.hitactor _array_element)))
          (LocalVariables|SetReturnHitEnemy _asbp_enemy)
          (LocalVariables|SetbReturnIsHIt true))))
    (return (LocalVariables|GetbReturnIsHIt) (LocalVariables|GetReturnHitEnemy))))

(fn UpdateFindingEnemy
  (params (bIsFind :type Boolean) (FindingEnemy :type BP%20Enemy%20Object%20Reference))
  (bind _player (Variables|Objects|GetPlayer))
  (bind _findingenemies (Variables|/Game/_Users/Players/Blueprints/BP_Player.BP_Player_C|GetFindingEnemies _player))
  (if bIsFind
    (if (== (Variables|Default|GetFindingEnemy) FindingEnemy)
      (Variables|Default|SetNowFindingTime (+ (Variables|Default|GetNowFindingTime) (Utilities|Time|GetWorldDeltaSeconds)))
      (if (>= (Variables|Default|GetNowFindingTime) (Variables|Static|GetMaxFindingTime))
        (Variables|Default|SetNowFindingTime 0.0)
        (if (== (Utilities|Array|FindItem _findingenemies FindingEnemy) -1)
          (Utilities|Array|Add _findingenemies FindingEnemy)))
      (else
        (Variables|Default|SetFindingEnemy FindingEnemy)
        (Variables|Default|SetNowFindingTime 0.0)))))

(fn GetMulDeltaSeconds
  (params (Rate :type Float%20%28single-precision%29))
  (return (* Rate (Utilities|Time|GetWorldDeltaSeconds))))

(fn SetCameraPitch
  (params (Min :type Float%20%28single-precision%29) (Max :type Float%20%28single-precision%29))
  (bind _cameramanager (Variables|Objects|GetCameraManager))
  (Variables|/Script/Engine.PlayerCameraManager|SetViewPitchMin _cameramanager Min)
  (Variables|/Script/Engine.PlayerCameraManager|SetViewPitchMax _cameramanager Max))

(fn SpawnEndCamera
  (bind _thirdcamera (Variables|Default|GetThirdCamera))
  (bind _returnvalue (Transformation|GetWorldLocation _thirdcamera))
  (bind _outhit (Collision|LineTraceByChannel _returnvalue (+ _returnvalue "0, 0,-300.000000") "TraceTypeQuery1" false 0 "None"))
  (Game|SpawnActorfromClass "/Game/_Users/Players/Blueprints/BP_EndCamera.BP_EndCamera_C" (Transformation|GetWorldTransform (Variables|Default|GetThirdCamera)) "Undefined" 0 (+ (.z (.impactpoint _outhit)) 2e+01) 0)
  (Actor|DestroyActor))