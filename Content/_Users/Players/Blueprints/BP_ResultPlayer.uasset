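; BP_ResultPlayer is the player actor for the result sequence, holding a bottle and passing Select input to the result manager.
; On BeginPlay it spawns a BP_ResultBottle onto the skeletal mesh's bottlePos socket.
; It also finds the level's BP_ResultCamera and attaches it to CameraLocation, snapping position only, then caches the BP_ResultManager.
; Pressing Select calls Next on that manager.
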(event EventBeginPlay
  (bind _returnvalue (Game|SpawnActorfromClass "/Game/_Users/Players/Bottle/Blueprints/BP_ResultBottle.BP_ResultBottle_C" (Math|Transform|MakeTransform "0, 0, 0" "0, 0, 0" "1,1,1") "Undefined" 0 0))
  (bind _output_get (Variables|Default|SetBottle _returnvalue))
  (Transformation|AttachComponentToComponent (Variables|/Script/Engine.Actor|GetRootComponent _output_get) (Variables|Default|GetSkeletalMesh) "bottlePos" "SnapToTarget" "SnapToTarget" "KeepRelative" true)
  (bind _outactors (Actor|GetAllActorsOfClass "/Game/_Users/Cameras/Blueprints/BP_ResultCamera.BP_ResultCamera_C"))
  (Variables|Default|SetCamera (Utilities|Array|Get(acopy) _outactors))
  (Transformation|AttachComponentToComponent (Variables|Default|GetCamera) (Variables|Default|GetCameraLocation) "None" "SnapToTarget" "KeepRelative" "KeepRelative" true)
  (bind _outactors_2 (Actor|GetAllActorsOfClass "/Game/_Users/BP_ResultManager.BP_ResultManager_C"))
  (Variables|Default|SetResultManager (Utilities|Array|Get(acopy) _outactors_2)))

(event Input|ActionEvents|InputActionSelect
  (params (Key :type Key%20Structure :default "None"))
  (:Pressed
    (Default|Next (Variables|Default|GetResultManager))))

(fn ConstructionScript)