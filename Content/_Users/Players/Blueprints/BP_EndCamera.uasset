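; BP_EndCamera is an end camera that takes over the player's view on BeginPlay and rotates every tick to face the player.
; A timeline moves it vertically toward ZLocation until the player dies, with per-frame polling if the timeline finishes first.
; On death, a zero-delay loop eases its height toward the higher of ZLocation and the player's EndCameraZLocation, using a slowly increasing lerp alpha.
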(event Custom|HomingLocation
  (bind _returnvalue (Transformation|GetActorLocation))
  (Variables|Default|SetAlpha (+ (Variables|Default|GetAlpha) 0.0001) :!label _label)
  (Transformation|SetActorLocation (Math|Vector|Lerp(Vector) (Math|Vector|MakeVector (.x _returnvalue) (.y _returnvalue) (.z _returnvalue)) (Math|Vector|MakeVector (.x _returnvalue) (.y _returnvalue) (Math|Float|Max(Float) (Variables|Default|GetZLocation) (.z (Transformation|GetWorldLocation (Variables|/Game/_Users/Players/Blueprints/BP_Player.BP_Player_C|GetEndCameraZLocation (Variables|Objects|GetPlayer)))))) (Variables|Default|GetAlpha)) false false)
  (Utilities|FlowControl|Delay 0.0)
  (goto _label))

(event EventBeginPlay
  (Game|Player|SetViewTargetwithBlend (Game|GetPlayerController 0) self 0.0 "VTBlend_Linear" 0.0 false)
  (Variables|Objects|SetPlayer (.AsBP%20Player (Utilities|Casting|CastToBP_Player (Game|Player|GetPlayerPawn 0))))
  (Variables|Default|SetStartLocation (Transformation|GetActorLocation))
  (bind _newtrack_0 (Timeline|Timeline_0 Play)
    (:Update
      (Transformation|SetActorLocation (Math|Vector|Lerp(Vector) (Variables|Default|GetStartLocation) (Math|Vector|MakeVector (.x (Variables|Default|GetStartLocation)) (.y (Variables|Default|GetStartLocation)) (Variables|Default|GetZLocation)) _newtrack_0) false false)
      (if (not (Variables|Default|GetbStartHoming))
        (if (not (Default|CheckIsAlive (Variables|Objects|GetPlayer)))
          (Variables|Default|SetbStartHoming true)
          (Timeline|Timeline_0 Stop))))
    (:Finished
      (if (not (Variables|Default|GetbStartHoming))
        (if (Default|CheckIsAlive (Variables|Objects|GetPlayer)) :!label _label
          (Utilities|FlowControl|Delay 0.0)
          (goto _label)
          (else
            (Variables|Default|SetbStartHoming true)))))))

(event EventTick
  (params (DeltaSeconds :type Float%20%28single-precision%29))
  (Transformation|SetActorRotation (Math|Rotator|FindLookatRotation (Transformation|GetActorLocation) (Transformation|GetActorLocation (Variables|Objects|GetPlayer))))
  (if (Variables|Default|GetbStartHoming)
    (Utilities|FlowControl|DoOnce false
      (:Completed
        (CallFunction|HomingLocation)))))

(fn ConstructionScript)