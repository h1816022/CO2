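; Player character Blueprint with camera-relative movement, jumping and a bottle attached to a mesh socket at BeginPlay.
; CanMove gates movement and jump input, which also records an input vector.
; Each tick, AdjustVelocity damps horizontal velocity by up to 5%, scaled by the angle between that input and the mesh's facing relative to camera yaw.
; C selects the follow camera, while B selects first-person and spawns an attached water drop.
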(event EventTick
  (params (DeltaSeconds :type Float%20%28single-precision%29))
  (CallFunction|AdjustVelocity))

(event EventBeginPlay
  (bind _returnvalue (Game|SpawnActorfromClass "/Game/_Users/Bottle/Blueprints/BP_Bottle.BP_Bottle_C" (Math|Transform|MakeTransform "0, 0, 0" "0, 0, 0" "1,1,1") "Undefined" 0 0))
  (Transformation|AttachComponentToComponent (Variables|/Script/Engine.Actor|GetRootComponent _returnvalue) (Variables|Character|GetMesh) "bottlePos" "SnapToTarget" "SnapToTarget" "KeepRelative" true))

(event Input|ActionEvents|InputActionJump
  (params (Key :type Key%20Structure :default "None"))
  ;[1 1 1] Input
  (:Pressed
    (if (Variables|Default|GetbCanMove)
      (Character|Jump)))
  (:Released
    (Character|StopJumping)))

(event Input|AxisEvents|InputAxisLookUp
  (params (AxisValue :type Float%20%28single-precision%29))
  ;[1 1 1] Input
  (Pawn|Input|AddControllerPitchInput AxisValue))

(event Input|AxisEvents|InputAxisTurnRate
  (params (AxisValue :type Float%20%28single-precision%29))
  ;[1 1 1] Input
  (Pawn|Input|AddControllerYawInput (* AxisValue (Variables|Default|GetBaseTurnRate) (Utilities|Time|GetWorldDeltaSeconds))))

(event Input|AxisEvents|InputAxisTurn
  (params (AxisValue :type Float%20%28single-precision%29))
  ;[1 1 1] Input
  (Pawn|Input|AddControllerYawInput AxisValue))

(event Input|AxisEvents|InputAxisLookUpRate
  (params (AxisValue :type Float%20%28single-precision%29))
  ;[1 1 1] Input
  (Pawn|Input|AddControllerPitchInput (* AxisValue (Variables|Default|GetBaseLookUpRate) (Utilities|Time|GetWorldDeltaSeconds))))

(event Input|AxisEvents|InputAxisMoveForward
  (params (AxisValue :type Float%20%28single-precision%29))
  ;[1 1 1] Input
  (if (Variables|Default|GetbCanMove)
    (Variables|Default|SetForwardVal AxisValue)
    (else
      (Variables|Default|SetForwardVal 0.0)))
  (Pawn|Input|AddMovementInput (Math|Vector|GetForwardVector (Math|Rotator|MakeRotator 0.0 0.0 (.Yaw (Math|Rotator|BreakRotator (Pawn|GetControlRotation :!class /Script/Engine.Pawn))))) (Variables|Default|GetForwardVal) false)
  (Variables|Default|SetInputVec (Math|Vector|MakeVector (Variables|Default|GetForwardVal) (.y (Variables|Default|GetInputVec)) 0.0)))

(event Input|AxisEvents|InputAxisMoveRight
  (params (AxisValue :type Float%20%28single-precision%29))
  ;[1 1 1] Input
  (if (Variables|Default|GetbCanMove)
    (Variables|Default|SetRightVal AxisValue)
    (else
      (Variables|Default|SetRightVal 0.0)))
  (Pawn|Input|AddMovementInput (Math|Vector|GetRightVector (Math|Rotator|MakeRotator 0.0 0.0 (.Yaw (Math|Rotator|BreakRotator (Pawn|GetControlRotation :!class /Script/Engine.Pawn))))) (Variables|Default|GetRightVal) false)
  (Variables|Default|SetInputVec (Math|Vector|MakeVector (.x (Variables|Default|GetInputVec)) (Variables|Default|GetRightVal) 0.0)))

(event Input|KeyboardEvents|C
  (params (Key :type Key%20Structure :default "None"))
  (:Pressed
    (Components|Activation|Activate (Variables|MyCharacter|GetFollowCamera) false)
    (Components|Activation|Deactivate (Variables|Default|GetFirstPersonCamera))))

(event Input|KeyboardEvents|B
  (params (Key :type Key%20Structure :default "None"))
  (:Pressed
    (Components|Activation|Deactivate (Variables|MyCharacter|GetFollowCamera))
    (Components|Activation|Activate (Variables|Default|GetFirstPersonCamera) false)
    (bind _returnvalue (Game|SpawnActorfromClass "/Game/_Users/Players/Blueprints/BP_WaterDrop.BP_WaterDrop_C" (Math|Transform|MakeTransform "0, 0, 0" "0, 0, 0" "1,1,1") "Undefined" 0 0))
    (Transformation|AttachComponentToComponent _returnvalue (Variables|Default|GetWaterDropSpawnPoint) "None" "SnapToTarget" "SnapToTarget" "KeepRelative" true)))

(fn ConstructionScript)

(fn AdjustVelocity
  (bind _charactermovement (Variables|Character|GetCharacterMovement))
  (Variables|/Script/Engine.MovementComponent|SetVelocity (Variables|Character|GetCharacterMovement) (Math|Vector|MakeVector (.x (* (Variables|/Script/Engine.MovementComponent|GetVelocity _charactermovement) (- 1.0 (|(((X/180.000000)*5.000000)/100.000000) (Class|KismetMathLibrary|DegAcos (Math|Vector|DotProduct (Variables|Default|GetInputVec) (Math|Vector|RotateVector (Math|Vector|GetForwardVector (Variables|Character|GetMesh)) (Class|KismetMathLibrary|NegateRotator (Math|Rotator|MakeRotator 0.0 0.0 (.yaw (Transformation|GetWorldRotation (Variables|MyCharacter|GetFollowCamera)))))))))))) (.y (* (Variables|/Script/Engine.MovementComponent|GetVelocity _charactermovement) (- 1.0 (|(((X/180.000000)*5.000000)/100.000000) (Class|KismetMathLibrary|DegAcos (Math|Vector|DotProduct (Variables|Default|GetInputVec) (Math|Vector|RotateVector (Math|Vector|GetForwardVector (Variables|Character|GetMesh)) (Class|KismetMathLibrary|NegateRotator (Math|Rotator|MakeRotator 0.0 0.0 (.yaw (Transformation|GetWorldRotation (Variables|MyCharacter|GetFollowCamera)))))))))))) (.z (Variables|/Script/Engine.MovementComponent|GetVelocity _charactermovement)))))