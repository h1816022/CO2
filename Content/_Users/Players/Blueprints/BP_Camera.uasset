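; BP_Camera is the player camera actor that becomes the view target and switches between third-person and first-person views while X is held.
; X press and release fire events that toggle the FirstCamera and ThirdCamera components.
; Entering first person spawns and attaches a water drop and two counter-rotating reticles, which are destroyed on returning to third person.
; Tick matches the actor's rotation to the player pawn's control rotation.
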(event Custom|SetFirstCamera_Event
  (Components|Activation|Deactivate (Variables|Default|GetThirdCamera))
  (Components|Activation|Activate (Variables|Default|GetFirstCamera) false)
  (bind _returnvalue (Game|SpawnActorfromClass "/Game/_Users/Players/Blueprints/BP_WaterDrop.BP_WaterDrop_C" (Math|Transform|MakeTransform "0, 0, 0" "0, 0, 0" "1,1,1") "Undefined" 0 0))
  (Transformation|AttachComponentToComponent _returnvalue (Variables|Default|GetWaterDropSpawnPoint) "None" "SnapToTarget" "SnapToTarget" "KeepRelative" true)
  (Utilities|Array|Add (Variables|Default|GetFirstCameraActors) _returnvalue)
  (bind _returnvalue_2 (Game|SpawnActorfromClass "/Game/_Users/Players/Blueprints/BP_Reticle.BP_Reticle_C" (Math|Transform|MakeTransform "0, 0, 0" "0, 0, 0" "0.070000,0.070000,0.070000") "Undefined" 0 9e+01 false 0))
  (Transformation|AttachComponentToComponent _returnvalue_2 (Variables|Default|GetReticleSpawnPoint) "None" "SnapToTarget" "SnapToTarget" "KeepRelative" true)
  (Utilities|Array|Add (Variables|Default|GetFirstCameraActors) _returnvalue_2)
  (bind _returnvalue_3 (Game|SpawnActorfromClass "/Game/_Users/Players/Blueprints/BP_Reticle.BP_Reticle_C" (Math|Transform|MakeTransform "0, 0, 0" "0, 0, 0" "0.070000,0.070000,0.070000") "Undefined" 0 -45.0 true 0))
  (Transformation|AttachComponentToComponent _returnvalue_3 (Variables|Default|GetReticleSpawnPoint) "None" "SnapToTarget" "SnapToTarget" "KeepRelative" true)
  (Utilities|Array|Add (Variables|Default|GetFirstCameraActors) _returnvalue_3))

(event Custom|SetThirdCamera_Event
  (bind _firstcameraactors (Variables|Default|GetFirstCameraActors))
  (Components|Activation|Deactivate (Variables|Default|GetFirstCamera))
  (Components|Activation|Activate (Variables|Default|GetThirdCamera) false)
  (for _array_element _firstcameraactors
    (Actor|DestroyActor _array_element))
  (Utilities|Array|Clear _firstcameraactors))

(event EventBeginPlay
  (Game|Player|SetViewTargetwithBlend (Game|GetPlayerController 0) self 0.0 "VTBlend_Linear" 0.0 false)
  (EventDispatchers|BindEventtoSetFirstCamera (delegate Custom|SetFirstCamera_Event))
  (EventDispatchers|BindEventtoSetThirdCamera (delegate Custom|SetThirdCamera_Event)))

(event EventTick
  (params (DeltaSeconds :type Float%20%28single-precision%29))
  (Transformation|SetActorRotation (Pawn|GetControlRotation (Game|Player|GetPlayerPawn 0) :!class /Script/Engine.Pawn)))

(event Input|KeyboardEvents|X
  (params (Key :type Key%20Structure :default "None"))
  (:Pressed
    (Variables|Default|SetbIsFirstPerson true)
    (Default|CallSetFirstCamera))
  (:Released
    (Variables|Default|SetbIsFirstPerson false)
    (Default|CallSetThirdCamera)))

(fn ConstructionScript)