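; BP_Bottle is the player's bottle, tracking hit points and collected liquid, and changing the goal door once enough liquid is gathered.
; It spawns bubble spawner, segment display and label actors, and hides itself in first-person view.
; Tick drives liquid materials, speed-based bobbing and mode-dependent health drain, which feeds the display, mask opacity and pinch mode.
; Death empties the liquid before signaling dead; M toggles invincibility.
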(event Custom|InitFirstCamera
  (Rendering|SetActorHiddenInGame true)
  (Default|SetLabelVisibility (Variables|Objects|GetLabel) false)
  (Default|SetSegVisibility (Variables|Objects|GetSeg) false))

(event Custom|InitThirdCamera
  (Rendering|SetActorHiddenInGame false)
  (Default|SetLabelVisibility (Variables|Objects|GetLabel) true)
  (Default|SetSegVisibility (Variables|Objects|GetSeg) true))

(event Custom|Dying_Event
  (Utilities|FlowControl|Delay (Variables|/Game/_Users/Players/Blueprints/BP_Player.BP_Player_C|GetDyingDelay (Variables|Objects|GetPlayer)))
  (bind _bisfinish (CallFunction|Launch :!label _label))
  (if (not _bisfinish)
    (if (not (Variables|Default|GetbIsClear))
      (Utilities|FlowControl|Delay 0.0)
      (goto _label))
    (else
      (Default|CallDead))))

(event Custom|Clear_Event
  (Variables|Default|SetbIsClear true))

(event Custom|Binding
  (bind _returnvalue (Game|Player|GetPlayerPawn 0))
  (bind _asbp_player (Utilities|Casting|CastToBP_Player _returnvalue))
  (bind _camera (Variables|/Game/_Users/Players/Blueprints/BP_Player.BP_Player_C|GetCamera _asbp_player))
  (EventDispatchers|BindEventtoSetFirstCamera _camera (delegate Custom|InitFirstCamera))
  (EventDispatchers|BindEventtoSetThirdCamera _camera (delegate Custom|InitThirdCamera))
  (EventDispatchers|BindEventtoDying (delegate Custom|Dying_Event))
  (EventDispatchers|BindEventtoGoal (Variables|Objects|GetPlayer) (delegate Custom|Goal_Event))
  (EventDispatchers|BindEventtoClear (Variables|Objects|GetPlayer) (delegate Custom|Clear_Event)))

(event Custom|SetDamageInvincible
  (params (InvincibleTime :type Float%20%28single-precision%29))
  (Variables|Default|SetNowDamageInvincibleTime (Math|Float|Max(Float) InvincibleTime (Variables|Default|GetNowDamageInvincibleTime)))
  (if (not (Variables|Default|GetbIsDamageInvincible))
    (Variables|Default|SetbIsDamageInvincible true)
    (bind _output_get (Variables|Default|SetNowDamageInvincibleTime (- (Variables|Default|GetNowDamageInvincibleTime) (Utilities|Time|GetWorldDeltaSeconds)) :!label _label))
    (if (> _output_get 0.0)
      (Utilities|FlowControl|Delay 0.0)
      (goto _label)
      (else
        (Variables|Default|SetbIsDamageInvincible false)))))

(event Custom|Goal_Event
  (Variables|Default|SetbIsContinuousInvincible true))

(event EventBeginPlay
  (CallFunction|InitVariables)
  (CallFunction|Binding)
  (bind _returnvalue (Game|SpawnActorfromClass "/Game/_Users/Blueprints/Bubbles/BP_BubbleSpawner.BP_BubbleSpawner_C" (Math|Transform|MakeTransform "0, 0, 0" "0, 0, 0" "1,1,1") "Undefined" 0 0))
  (bind _output_get (Variables|Objects|SetBubbleSpawner _returnvalue))
  (Transformation|AttachComponentToComponent _output_get (Variables|Default|GetBubbleSpawnerLocation) "None" "SnapToTarget" "SnapToTarget" "KeepRelative" true)
  (bind _returnvalue_2 (Game|SpawnActorfromClass "/Game/_Users/Seg/Blueprints/BP_Seg.BP_Seg_C" (Math|Transform|MakeTransform "0, 0, 0" "0,-90.819183, 0" "0.060000,0.060000,0.060000") "Undefined" 0 self true 0 0))
  (bind _output_get_2 (Variables|Objects|SetSeg _returnvalue_2))
  (Transformation|AttachComponentToComponent _output_get_2 (Variables|Default|GetDisplayTransform) "None" "SnapToTarget" "KeepRelative" "KeepRelative" true)
  (bind _returnvalue_3 (Game|SpawnActorfromClass "/Game/_Users/Players/Label/Blueprints/BP_Label.BP_Label_C" (Math|Transform|MakeTransform "0, 0, 0" "180.000000,180.000000, 0" "1,1,1") "Undefined" 0 0))
  (bind _output_get_3 (Variables|Objects|SetLabel _returnvalue_3))
  (Transformation|AttachComponentToComponent _output_get_3 (Variables|Default|GetDisplayTransform) "None" "SnapToTarget" "KeepRelative" "KeepRelative" true)
  (Utilities|FlowControl|Delay 3.0)
  (Variables|Default|SetbIsContinuousInvincible false))

(event EventTick
  (params (DeltaSeconds :type Float%20%28single-precision%29))
  (Utilities|FlowControl|Sequence
    (:then_0
      (Utilities|FlowControl|DoOnce false
        (:Completed
          (Variables|Default|SetDefRelativeLocation (- (Transformation|GetActorLocation) (Transformation|GetWorldLocation (Variables|/Game/_Users/Players/Blueprints/BP_Player.BP_Player_C|GetFoundationLocation (Variables|Objects|GetPlayer))))))))
    (:then_1
      (CallFunction|Update)
      (Variables|Default|SetNowTime (+ (Variables|Default|GetNowTime) DeltaSeconds))
      (CallFunction|Vibration)
      (if (CallFunction|CheckHitPoint)
        (bind _bisalive (CallFunction|UpdateHitPoint DeltaSeconds))
        (if _bisalive
          (if (not (Variables|/Game/_Users/Players/Blueprints/BP_Player.BP_Player_C|GetbIsGoal (Variables|Objects|GetPlayer)))
            (CallFunction|UpdatePinchMode))
          (else
            (Default|CallDying)))))))

(event Input|KeyboardEvents|M
  (params (Key :type Key%20Structure :default "None"))
  (:Pressed
    (Variables|Default|SetbIsContinuousInvincible (not (Variables|Default|GetbIsContinuousInvincible)))
    (Variables|Default|SetbIsDamageInvincible (not (Variables|Default|GetbIsDamageInvincible)))))

(fn ConstructionScript)

(fn InitVariables
  (Utilities|FlowControl|Sequence
    (:then_0
      (bind _returnvalue (Rendering|Material|CreateDynamicMaterialInstance (Variables|Default|GetLiquid) 1 "/Game/RealLiquidX/M/MI_LiquidX_03.MI_LiquidX_03" "None" :!class /Script/Engine.PrimitiveComponent))
      (Variables|Materials|SetLiquidMat _returnvalue)
      (bind _returnvalue_2 (Rendering|Material|CreateDynamicMaterialInstance (Variables|Default|GetBottleMask) 1 "/Game/_Users/Players/Bottle/Materials/MI_BottleMask.MI_BottleMask" "None" :!class /Script/Engine.PrimitiveComponent))
      (Variables|Materials|SetBottleMaskMat _returnvalue_2)
      (bind _returnvalue_3 (Rendering|Material|CreateDynamicMaterialInstance (Variables|Default|GetScale) 0 "/Game/_Users/Players/Bottle/Materials/MI_Scale.MI_Scale" "None" :!class /Script/Engine.PrimitiveComponent))
      (Variables|Materials|SetScaleMat _returnvalue_3))
    (:then_1
      (Variables|Default|SetNowHitPoint (Variables|Default|GetMaxHItPoint))
      (Variables|Objects|SetPlayer (.AsBP%20Player (Utilities|Casting|CastToBP_Player (Game|Player|GetPlayerPawn 0))))
      (Variables|Default|SetNowDisplayRotation (Transformation|GetWorldRotation (Variables|Default|GetDisplayTransform))))
    (:then_2
      (bind _returnvalue_4 (Audio|SpawnSoundAttached "/Game/_Users/Sounds/A_Soda1_Cue.A_Soda1_Cue" (Variables|Default|GetBody) "None" "0, 0, 0" "0, 0, 0" "KeepRelativeOffset" false 0.1 1.0 0.0 "/Game/_Users/Sounds/Att_Soda.Att_Soda" 0 false))
      (Variables|Default|SetSodaSE _returnvalue_4))))

(fn Update
  (CallFunction|UpdateLiquid)
  (CallFunction|UpdateDisplayRotation)
  (CallFunction|UpdateScale))

(fn ClampHItPoint
  (Variables|Default|SetNowHitPoint (Math|Float|Clamp(Float) (Variables|Default|GetNowHitPoint) 0.0 (Variables|Default|GetMaxHItPoint))))

(fn CheckHitPoint
  (return (> (Variables|Default|GetNowHitPoint) 0.0)))

(fn UpdateHitPoint
  (params (DeltaSeconds :type Float%20%28single-precision%29))
  (if (not (Variables|Default|GetbIsContinuousInvincible))
    (bind _output_get (Variables|Default|SetPlayerModeType (Variables|/Game/_Users/Players/Animations/ABP_CSC.ABP_CSC_C|GetModeType (Variables|/Game/_Users/Players/Blueprints/BP_Player.BP_Player_C|GetAnimBlueprint (Variables|Objects|GetPlayer)))))
    (switch Utilities|FlowControl|Switch|SwitchonEPlayerModeType _output_get
      (:NewEnumerator0
        (LocalVariables|SetSumContinuousDamage (* (Math|Float|Clamp(Float) (Math|Vector|VectorLength (Variables|/Game/_Users/Players/Blueprints/BP_Player.BP_Player_C|GetInputVec (Variables|Objects|GetPlayer))) 0.1) (+ 1.0 (Variables|Default|GetTargetLiquidRate))) :!label _label) ; 移動スピードで減り具合を調整
      )
      (:NewEnumerator1
        _)
      (:NewEnumerator2
        (goto _label))
      (:NewEnumerator3
        _))
    (bind _returnvalue (Utilities|GetDataTableRow "/Game/_Users/Players/Data/DT_PlayerModeTypeData.DT_PlayerModeTypeData" (Utilities|String|StringToName (Utilities|String|EnumtoString (Variables|Default|GetPlayerModeType))))
      (:then
        (LocalVariables|SetSumContinuousDamage (* DeltaSeconds (Variables|Default|GetContinuousDamage) (LocalVariables|GetSumContinuousDamage) (.continuousdamagerate _returnvalue)))
        (Variables|Default|SetNowHitPoint (- (Variables|Default|GetNowHitPoint) (LocalVariables|GetSumContinuousDamage))))))
  (Variables|Default|SetNowHitPoint (- (Variables|Default|GetNowHitPoint) (Variables|Default|GetSumDamage)))
  (LocalVariables|SetRate (Math|Float|Clamp(Float) (/ (Variables|Default|GetNowHitPoint) (Variables|Default|GetMaxHItPoint))))
  (Variables|/Game/_Users/Seg/Blueprints/BP_Seg.BP_Seg_C|SetTargetNum (Variables|Objects|GetSeg) (Math|Float|Truncate (* (- 1.0 (LocalVariables|GetRate)) 1e+02)))
  (Variables|Default|SetSumDamage 0.0)
  (Rendering|Material|SetScalarParameterValue (Variables|Materials|GetBottleMaskMat) "Opacity" (Math|Float|Min(Float) (- 1.0 (LocalVariables|GetRate)) 0.9) :!class /Script/Engine.MaterialInstanceDynamic)
  (return (CallFunction|CheckHitPoint)))

(fn Launch
  (Variables|Default|SetTargetLiquidRate (Math|Float|Max(Float) (- (Variables|Default|GetTargetLiquidRate) (CallFunction|GetMulDeltaSeconds 0.5)) 0.0))
  (return (== (Variables|Default|GetTargetLiquidRate) 0.0)))

(fn AddDamage
  (params (InDamage :type Float%20%28single-precision%29))
  (if (not (Variables|Default|GetbIsDamageInvincible))
    (Variables|Default|SetSumDamage (+ InDamage (Variables|Default|GetSumDamage)))))

(fn AddTypeDamage
  (params (DamageType :type EDamageType%20Enum :default "NewEnumerator0") (Rate :type Float%20%28single-precision%29))
  (bind _returnvalue (Utilities|GetDataTableRow "/Game/_Users/Players/Bottle/Data/DT_DamageAmountData.DT_DamageAmountData" (Utilities|String|StringToName (Utilities|String|EnumtoString DamageType)))
    (:then
      (CallFunction|AddDamage (* (.value _returnvalue) Rate)))))

(fn GetMulDeltaSeconds
  (params (Rate :type Float%20%28single-precision%29))
  (return (* Rate (Utilities|Time|GetWorldDeltaSeconds))))

(fn GetHitPointRate
  (return (/ (Variables|Default|GetNowHitPoint) (Variables|Default|GetMaxHItPoint))))

(fn Vibration
  (bind _returnvalue (Transformation|GetActorLocation))
  (bind _player (Variables|Objects|GetPlayer))
  (bind _player_2 (Variables|Objects|GetPlayer))
  (bind _defrelativelocation (Variables|Default|GetDefRelativeLocation))
  (bind _charactermovement (Variables|/Script/Engine.Character|GetCharacterMovement _player_2))
  (bind _foundationlocation (Variables|/Game/_Users/Players/Blueprints/BP_Player.BP_Player_C|GetFoundationLocation _player))
  (bind _returnvalue_2 (Transformation|GetWorldLocation _foundationlocation))
  (bind _velocity (Variables|/Script/Engine.MovementComponent|GetVelocity _charactermovement))
  (bind _returnvalue_3 (Math|Vector|VectorLengthXY _velocity))
  (bind _returnvalue_4 (+ _defrelativelocation _returnvalue_2))
  (if (Default|CheckIsAlive (Variables|Objects|GetPlayer))
    (switch Utilities|FlowControl|Switch|SwitchonEPlayerModeType (Variables|Default|GetPlayerModeType)
      (:NewEnumerator0
        (LocalVariables|SetVibrationDistance (LocalVariables|GetNormalDistance))
        (LocalVariables|SetTimePerOneRoundTrip (LocalVariables|GetNormalTime))
        (LocalVariables|SetRate (CallFunction|CalculateRate _returnvalue_3 (Variables|/Game/_Users/Players/Blueprints/BP_Player.BP_Player_C|GetTCamWalkSpeed (Variables|Objects|GetPlayer)))))
      (:NewEnumerator1
        (LocalVariables|SetVibrationDistance (LocalVariables|GetDashDistance))
        (LocalVariables|SetTimePerOneRoundTrip (LocalVariables|GetDashTime))
        (LocalVariables|SetRate (CallFunction|CalculateRate _returnvalue_3 (Variables|/Game/_Users/Players/Blueprints/BP_Player.BP_Player_C|GetDashSpeed (Variables|Objects|GetPlayer)))))
      (:NewEnumerator2
        (LocalVariables|SetVibrationDistance (LocalVariables|GetWheelDistance))
        (LocalVariables|SetTimePerOneRoundTrip (LocalVariables|GetWheelTime))
        (LocalVariables|SetRate (CallFunction|CalculateRate _returnvalue_3 (Variables|/Game/_Users/Players/Blueprints/BP_Player.BP_Player_C|GetWheelSpeed (Variables|Objects|GetPlayer)))))
      (:NewEnumerator3
        (LocalVariables|SetVibrationDistance (LocalVariables|GetNormalDistance))
        (LocalVariables|SetTimePerOneRoundTrip (LocalVariables|GetNormalTime))
        (LocalVariables|SetRate 0.0)))
    (Transformation|SetActorLocation (Math|Vector|MakeVector (.x _returnvalue) (.y _returnvalue) (.z (Math|Vector|Lerp(Vector) _returnvalue_4 (+ _returnvalue_4 (Math|Vector|MakeVector 0.0 0.0 (* (LocalVariables|GetVibrationDistance) (LocalVariables|GetRate)))) (Math|Float|Absolute(Float) (- 1.0 (/ (Math|Float|%(Float) (Variables|Default|GetNowTime) (LocalVariables|GetTimePerOneRoundTrip)) (/ (LocalVariables|GetTimePerOneRoundTrip) 2.0))))))) false false)))

(fn UpdatePinchMode
  (if (Variables|/Game/_Users/Players/Blueprints/BP_Player.BP_Player_C|GetbIsPinch (Variables|Objects|GetPlayer))
    (if (>= (CallFunction|GetHitPointRate) 0.1)
      (Default|EndPinchMode (Variables|Objects|GetPlayer)))
    (elif (< (CallFunction|GetHitPointRate) 0.1)
      (Default|OnPinchMode (Variables|Objects|GetPlayer)))))

(fn CalculateRate
  (params (NowValue :type Float%20%28single-precision%29) (MaxValue :type Float%20%28single-precision%29))
  (return (Math|Float|Clamp(Float) (/ NowValue MaxValue))))

(fn UpdateDisplayRotation
  (bind _returnvalue (Utilities|Time|GetWorldDeltaSeconds))
  (bind _player (Variables|Objects|GetPlayer))
  (bind _player_2 (Variables|Objects|GetPlayer))
  (bind _displaytransform (Variables|Default|GetDisplayTransform))
  (bind _displaytransform_2 (Variables|Default|GetDisplayTransform))
  (bind _returnvalue_2 (Transformation|GetWorldRotation _displaytransform_2))
  (bind _returnvalue_3 (Transformation|GetWorldLocation _displaytransform_2))
  (bind _relativerotation (Variables|/Script/Engine.SceneComponent|GetRelativeRotation _displaytransform))
  (bind _camera (Variables|/Game/_Users/Players/Blueprints/BP_Player.BP_Player_C|GetCamera _player_2))
  (bind _returnvalue_4 (* (Math|Vector|MakeVector (.roll _relativerotation) (.pitch _relativerotation) (.yaw _relativerotation)) 0.99))
  (bind _thirdcamera (Variables|/Game/_Users/Cameras/Blueprints/BP_PlayerCamera.BP_PlayerCamera_C|GetThirdCamera _camera))
  (bind _returnvalue_5 (Transformation|GetWorldLocation _thirdcamera))
  (bind _returnvalue_6 (Math|Rotator|FindLookatRotation _returnvalue_3 _returnvalue_5))
  (bind _returnvalue_7 (Math|Interpolation|RInterpTo _returnvalue_2 _returnvalue_6 _returnvalue 3.0))
  (if (and (Variables|/Game/_Users/Players/Blueprints/BP_Player.BP_Player_C|GetbIsPanic _player) (Default|CheckIsAlive _player))
    (Transformation|SetWorldRotation _displaytransform_2 (Variables|Default|GetNowDisplayRotation) false false)
    (Transformation|SetWorldRotation (Variables|Default|GetDisplayTransform) (Math|Rotator|MakeRotator (.roll (Variables|Default|GetNowDisplayRotation)) (.pitch (Variables|Default|GetNowDisplayRotation)) (.yaw _returnvalue_7)) false false)
    (Variables|Default|SetNowDisplayRotation (Math|Rotator|MakeRotator (.roll (Variables|Default|GetNowDisplayRotation)) (.pitch (Variables|Default|GetNowDisplayRotation)) (.yaw _returnvalue_7)))
    (else
      (Transformation|SetRelativeRotation _displaytransform (Math|Rotator|MakeRotator (.x _returnvalue_4) (.y _returnvalue_4) (.z _returnvalue_4)) false false))))

(fn UpdateLiquid
  (bind _player (Variables|Objects|GetPlayer))
  (bind _animblueprint (Variables|/Game/_Users/Players/Blueprints/BP_Player.BP_Player_C|GetAnimBlueprint _player))
  (bind _modetype (Variables|/Game/_Users/Players/Animations/ABP_CSC.ABP_CSC_C|GetModeType _animblueprint))
  (bind _returnvalue (Utilities|GetDataTableRow "/Game/_Users/Players/Bottle/Data/DT_ModeTypeBottleData.DT_ModeTypeBottleData" (Utilities|String|StringToName (Utilities|String|EnumtoString _modetype)))
    (:then
      (switch Utilities|FlowControl|Switch|SwitchonEPlayerModeType _modetype
        (:NewEnumerator0
          (LocalVariables|SetNowMaxSpeed (Variables|/Game/_Users/Players/Blueprints/BP_Player.BP_Player_C|GetTCamWalkSpeed (Variables|Objects|GetPlayer)) :!label _label))
        (:NewEnumerator1
          (LocalVariables|SetNowMaxSpeed (Variables|/Game/_Users/Players/Blueprints/BP_Player.BP_Player_C|GetDashSpeed (Variables|Objects|GetPlayer))))
        (:NewEnumerator2
          (LocalVariables|SetNowMaxSpeed (Variables|/Game/_Users/Players/Blueprints/BP_Player.BP_Player_C|GetWheelSpeed (Variables|Objects|GetPlayer))))
        (:NewEnumerator3
          (goto _label)))
      (LocalVariables|SetVelocity (Variables|/Script/Engine.MovementComponent|GetVelocity (Variables|/Script/Engine.Character|GetCharacterMovement (Variables|Objects|GetPlayer))))
      (LocalVariables|SetSpeedRate (Math|Float|Clamp(Float) (/ (Math|Vector|VectorLengthXY (LocalVariables|GetVelocity)) (LocalVariables|GetNowMaxSpeed))))
      (if (<= (LocalVariables|GetSpeedRate) 0.5)
        (Rendering|Material|SetScalarParameterValue (Variables|Materials|GetLiquidMat) "SineXAmount" (.MinSineAmount (Utilities|Struct|BreakSModeTypeBottleData _returnvalue)) :!class /Script/Engine.MaterialInstanceDynamic)
        (Rendering|Material|SetScalarParameterValue (Variables|Materials|GetLiquidMat) "SineYAmount" (.MinSineAmount (Utilities|Struct|BreakSModeTypeBottleData _returnvalue)) :!class /Script/Engine.MaterialInstanceDynamic)
        (else
          (Rendering|Material|SetScalarParameterValue (Variables|Materials|GetLiquidMat) "SineXAmount" (.MaxSineAmount (Utilities|Struct|BreakSModeTypeBottleData _returnvalue)) :!class /Script/Engine.MaterialInstanceDynamic)
          (Rendering|Material|SetScalarParameterValue (Variables|Materials|GetLiquidMat) "SineYAmount" (.MaxSineAmount (Utilities|Struct|BreakSModeTypeBottleData _returnvalue)) :!class /Script/Engine.MaterialInstanceDynamic)))
      (Rendering|Material|SetScalarParameterValue (Variables|Materials|GetLiquidMat) "Sine_Strength" (Math|Float|Lerp (.MinSineStrength (Utilities|Struct|BreakSModeTypeBottleData _returnvalue)) (.MaxSineStrength (Utilities|Struct|BreakSModeTypeBottleData _returnvalue)) (LocalVariables|GetSpeedRate)) :!class /Script/Engine.MaterialInstanceDynamic)
      (Rendering|Material|SetScalarParameterValue (Variables|Materials|GetLiquidMat) "Liquid_FillHeight" (Math|Float|Lerp -0.5 0.47 (Variables|Default|GetNowLiquidRate)) :!class /Script/Engine.MaterialInstanceDynamic)
      (Variables|Default|SetNowLiquidRate (Math|Float|Lerp (Variables|Default|GetNowLiquidRate) (Variables|Default|GetTargetLiquidRate) 0.02)))))

(fn AddLiquidRate
  (params (Value :type Float%20%28single-precision%29))
  (Variables|Default|SetTargetLiquidRate (Math|Float|Clamp(Float) (+ Value (Variables|Default|GetTargetLiquidRate))))
  (if (not (Variables|Default|GetbCanClear))
    (if (>= (Variables|Default|GetTargetLiquidRate) (Variables|/Game/_Users/Blueprints/BP_GameState.BP_GameState_C|GetRequiredAmount (.AsBP%20Game%20State (Utilities|Casting|CastToBP_GameState (Game|GetGameState)))))
      (Variables|Default|SetbCanClear true)
      (bind _outactors (Actor|GetAllActorsOfClass "/Game/_Users/Blueprints/BP_GoalDoor.BP_GoalDoor_C"))
      (Default|Change (Utilities|Array|Get(acopy) _outactors)))))

(fn UpdateScale
  (bind _returnvalue (Transformation|GetActorRotation))
  (Rendering|Material|SetScalarParameterValue (Variables|Materials|GetScaleMat) "Amount" (Variables|Default|GetNowLiquidRate) :!class /Script/Engine.MaterialInstanceDynamic)
  (Utilities|IsValid (Variables|/Game/_Users/Players/Blueprints/BP_Player.BP_Player_C|GetCamera (Variables|Objects|GetPlayer))
    (:Is%20Valid
      (Transformation|SetWorldRotation (Variables|Default|GetNozzleLocation) (Math|Rotator|MakeRotator (.roll _returnvalue) (.pitch _returnvalue) (+ (.yaw (Transformation|GetWorldRotation (Variables|/Game/_Users/Cameras/Blueprints/BP_PlayerCamera.BP_PlayerCamera_C|GetThirdCamera (Variables|/Game/_Users/Players/Blueprints/BP_Player.BP_Player_C|GetCamera (Variables|Objects|GetPlayer))))) 9e+01)) false false))))