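; BP_TitleBottle is a bottle actor, apparently for the title screen, that assembles its display on BeginPlay.
; It spawns a scaled-down BP_Seg with a fixed number and a BP_TitleLabel, then attaches both to DisplayTransform, snapping location while keeping relative rotation and scale.
; It also creates a dynamic instance of MI_BottleMask on the BottleMask component and sets its opacity to partly transparent.
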(event EventBeginPlay
  (bind _returnvalue (Game|SpawnActorfromClass "/Game/_Users/Players/Seg/BP_Seg.BP_Seg_C" (Math|Transform|MakeTransform "0, 0, 0" "0,-90.819183, 0" "0.060000,0.060000,0.060000") "Undefined" 0 self false 2 0))
  (bind _output_get (Variables|Objects|SetSeg _returnvalue))
  (Transformation|AttachComponentToComponent _output_get (Variables|Default|GetDisplayTransform) "None" "SnapToTarget" "KeepRelative" "KeepRelative" true)
  (bind _returnvalue_2 (Game|SpawnActorfromClass "/Game/_Users/Blueprints/BP_TitleLabel.BP_TitleLabel_C" (Math|Transform|MakeTransform "0, 0, 0" "180.000000,180.000000, 0" "1,1,1") "Undefined" 0 0))
  (bind _output_get_2 (Variables|Objects|SetLabel _returnvalue_2))
  (Transformation|AttachComponentToComponent _output_get_2 (Variables|Default|GetDisplayTransform) "None" "SnapToTarget" "KeepRelative" "KeepRelative" true)
  (bind _returnvalue_3 (Rendering|Material|CreateDynamicMaterialInstance (Variables|Default|GetBottleMask) 1 "/Game/_Users/Players/Bottle/Materials/MI_BottleMask.MI_BottleMask" "None" :!class /Script/Engine.PrimitiveComponent))
  (Rendering|Material|SetScalarParameterValue _returnvalue_3 "Opacity" 0.7 :!class /Script/Engine.MaterialInstanceDynamic))

(fn ConstructionScript)