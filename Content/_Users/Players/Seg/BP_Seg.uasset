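; BP_Seg is a three-digit seven-segment number display built from 21 mesh parts, each with a dynamic material.
; Unless IsResult is set, two endless Delay loops run, one stepping NowNum toward TargetNum, the other redrawing digits.
; Each digit's bitmask from BinaryValues drives the segment "Switch" parameters, blanking leading zeros.
; Value thresholds pick a color shared by the segments and the Bottle's label material.
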(event EventBeginPlay
  (for _array_element (Utilities|Array|MakeArray (Variables|Default|GetSeg0) (Variables|Default|GetSeg1) (Variables|Default|GetSeg2) (Variables|Default|GetSeg3) (Variables|Default|GetSeg4) (Variables|Default|GetSeg5) (Variables|Default|GetSeg6))
    (Utilities|Array|Add (Variables|Default|GetAllSegParts) _array_element)
    (bind _returnvalue (Rendering|Material|CreateDynamicMaterialInstance _array_element 0 "/Game/_Users/Players/Seg/MI_Seg.MI_Seg" "None" :!class /Script/Engine.PrimitiveComponent))
    (Utilities|Array|Add (Variables|Default|GetSegMaterials1) _returnvalue))
  (for _array_element_2 (Utilities|Array|MakeArray (Variables|Default|GetSeg7) (Variables|Default|GetSeg8) (Variables|Default|GetSeg9) (Variables|Default|GetSeg10) (Variables|Default|GetSeg11) (Variables|Default|GetSeg12) (Variables|Default|GetSeg13))
    (Utilities|Array|Add (Variables|Default|GetAllSegParts) _array_element_2)
    (bind _returnvalue_2 (Rendering|Material|CreateDynamicMaterialInstance _array_element_2 0 "/Game/_Users/Players/Seg/MI_Seg.MI_Seg" "None" :!class /Script/Engine.PrimitiveComponent))
    (Utilities|Array|Add (Variables|Default|GetSegMaterials10) _returnvalue_2))
  (for _array_element_3 (Utilities|Array|MakeArray (Variables|Default|GetSeg14) (Variables|Default|GetSeg15) (Variables|Default|GetSeg16) (Variables|Default|GetSeg17) (Variables|Default|GetSeg18) (Variables|Default|GetSeg19) (Variables|Default|GetSeg20))
    (Utilities|Array|Add (Variables|Default|GetAllSegParts) _array_element_3)
    (bind _returnvalue_3 (Rendering|Material|CreateDynamicMaterialInstance _array_element_3 0 "/Game/_Users/Players/Seg/MI_Seg.MI_Seg" "None" :!class /Script/Engine.PrimitiveComponent))
    (Utilities|Array|Add (Variables|Default|GetSegMaterials100) _returnvalue_3))
  (Utilities|FlowControl|Delay 1.0)
  (if (not (Variables|Default|GetbIsResult))
    (Utilities|FlowControl|Sequence
      (:then_0
        (CallFunction|UpdateNumber :!label _label)
        (Utilities|FlowControl|Delay 0.0)
        (goto _label))
      (:then_1
        (CallFunction|LerpNumber :!label _label_2)
        (Utilities|FlowControl|Delay 0.01)
        (goto _label_2)))))

(fn ConstructionScript)

(fn UpdateNumber
  (CallFunction|UpdateColor)
  (LocalVariables|SetNumber (Variables|Default|GetNowNum))
  (for _array_element (Variables|Default|GetSegMaterials1)
    (Rendering|Material|SetScalarParameterValue _array_element "Switch" (select (> (Class|KismetMathLibrary|AndIntInt (Utilities|Array|Get(acopy) (LocalVariables|GetBinaryValues) (Math|Integer|%(Integer) (LocalVariables|GetNumber) 10)) (LocalVariables|GetPlaceValue)) 0) 1.0 0.0) :!class /Script/Engine.MaterialInstanceDynamic)
    (LocalVariables|SetPlaceValue (* (LocalVariables|GetPlaceValue) 2)))
  (LocalVariables|SetNumber (/ (- (LocalVariables|GetNumber) (Math|Integer|%(Integer) (LocalVariables|GetNumber) 10)) 10))
  (LocalVariables|SetPlaceValue 1)
  (for _array_element_2 (Variables|Default|GetSegMaterials10)
    (if (< (Variables|Default|GetNowNum) 10)
      (Rendering|Material|SetScalarParameterValue _array_element_2 "Switch" 0.0 :!class /Script/Engine.MaterialInstanceDynamic)
      (else
        (Rendering|Material|SetScalarParameterValue _array_element_2 "Switch" (select (> (Class|KismetMathLibrary|AndIntInt (Utilities|Array|Get(acopy) (LocalVariables|GetBinaryValues) (Math|Integer|%(Integer) (LocalVariables|GetNumber) 10)) (LocalVariables|GetPlaceValue)) 0) 1.0 0.0) :!class /Script/Engine.MaterialInstanceDynamic)))
    (LocalVariables|SetPlaceValue (* (LocalVariables|GetPlaceValue) 2)))
  (LocalVariables|SetNumber (/ (- (LocalVariables|GetNumber) (Math|Integer|%(Integer) (LocalVariables|GetNumber) 10)) 10))
  (LocalVariables|SetPlaceValue 1)
  (for _array_element_3 (Variables|Default|GetSegMaterials100)
    (if (< (Variables|Default|GetNowNum) 100)
      (Rendering|Material|SetScalarParameterValue _array_element_3 "Switch" 0.0 :!class /Script/Engine.MaterialInstanceDynamic)
      (else
        (Rendering|Material|SetScalarParameterValue _array_element_3 "Switch" (select (> (Class|KismetMathLibrary|AndIntInt (Utilities|Array|Get(acopy) (LocalVariables|GetBinaryValues) (Math|Integer|%(Integer) (LocalVariables|GetNumber) 10)) (LocalVariables|GetPlaceValue)) 0) 1.0 0.0) :!class /Script/Engine.MaterialInstanceDynamic)))
    (LocalVariables|SetPlaceValue (* (LocalVariables|GetPlaceValue) 2))))

(fn LerpNumber
  (if (> (Variables|Default|GetTargetNum) (Variables|Default|GetNowNum))
    (Math|Integer|IncrementInt (Variables|Default|GetNowNum))
    (elif (< (Variables|Default|GetTargetNum) (Variables|Default|GetNowNum))
      (Math|Integer|DecrementInt (Variables|Default|GetNowNum)))))

(fn UpdateColor
  (if (== (Variables|Default|GetNowNum) 0)
    (LocalVariables|SetColor (Utilities|Array|Get(acopy) (Variables|Default|GetColors) 3))
    (elif (< (Variables|Default|GetNowNum) 30)
      (LocalVariables|SetColor (Utilities|Array|Get(acopy) (Variables|Default|GetColors) 2))
      (elif (< (Variables|Default|GetNowNum) 70)
        (LocalVariables|SetColor (Utilities|Array|Get(acopy) (Variables|Default|GetColors) 1))
        (else
          (LocalVariables|SetColor (Utilities|Array|Get(acopy) (Variables|Default|GetColors)))))))
  (for _array_element (Variables|Default|GetSegMaterials1)
    (Rendering|Material|SetVectorParameterValue _array_element "Color" (LocalVariables|GetColor) :!class /Script/Engine.MaterialInstanceDynamic))
  (for _array_element_2 (Variables|Default|GetSegMaterials10)
    (Rendering|Material|SetVectorParameterValue _array_element_2 "Color" (LocalVariables|GetColor) :!class /Script/Engine.MaterialInstanceDynamic))
  (for _array_element_3 (Variables|Default|GetSegMaterials100)
    (Rendering|Material|SetVectorParameterValue _array_element_3 "Color" (LocalVariables|GetColor) :!class /Script/Engine.MaterialInstanceDynamic))
  (Rendering|Material|SetVectorParameterValue (Variables|/Game/_Users/Players/Label/Blueprints/BP_Label.BP_Label_C|GetBaseMaterial (Variables|/Game/_Users/Players/Bottle/Blueprints/BP_Bottle.BP_Bottle_C|GetLabel (Variables|Default|GetBottle))) "Color" (LocalVariables|GetColor) :!class /Script/Engine.MaterialInstanceDynamic))

(fn SetSegVisibility
  (params (bNewVisibility :type Boolean))
  (for _array_element (Variables|Default|GetAllSegParts)
    (Rendering|SetVisibility _array_element bNewVisibility false)))