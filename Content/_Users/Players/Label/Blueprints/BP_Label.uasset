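; BP_Label is a label actor with a pulsing base and a switchable glowing "GoGo" element.
; BeginPlay creates dynamic materials for both, and Tick drives the base's Brightness with a clamped triangle wave over accumulated time.
; ChangeGoGo toggles the GoGo brightness along with two spotlights.
; SetLabelVisibility shows or hides the marks, base and GoGo components, leaving the spotlights untouched.
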(event Custom|ChangeGoGo
  (params (bIsOn :type Boolean))
  (if bIsOn
    (Rendering|Material|SetScalarParameterValue (Variables|Materials|GetGoGoMaterial) "Brightness" 2e+01 :!class /Script/Engine.MaterialInstanceDynamic)
    (Rendering|SetVisibility (Variables|Default|GetSpotLight) true false)
    (Rendering|SetVisibility (Variables|Default|GetSpotLight1) true false)
    (else
      (Rendering|Material|SetScalarParameterValue (Variables|Materials|GetGoGoMaterial) "Brightness" 0.1 :!class /Script/Engine.MaterialInstanceDynamic)
      (Rendering|SetVisibility (Variables|Default|GetSpotLight) false false)
      (Rendering|SetVisibility (Variables|Default|GetSpotLight1) false false))))

(event EventBeginPlay
  (bind _returnvalue (Rendering|Material|CreateDynamicMaterialInstance (Variables|Default|GetBase) 0 "/Game/_Users/Players/Label/Materials/MI_LabelBase.MI_LabelBase" "None" :!class /Script/Engine.PrimitiveComponent))
  (Variables|Materials|SetBaseMaterial _returnvalue)
  (bind _returnvalue_2 (Rendering|Material|CreateDynamicMaterialInstance (Variables|Default|GetGoGo) 0 "/Game/_Users/Players/Label/Materials/MI_LabelGoGo.MI_LabelGoGo" "None" :!class /Script/Engine.PrimitiveComponent))
  (Variables|Materials|SetGoGoMaterial _returnvalue_2))

(event EventTick
  (params (DeltaSeconds :type Float%20%28single-precision%29))
  (Variables|Default|SetTime (+ DeltaSeconds (Variables|Default|GetTime)))
  (CallFunction|UpdateBaseBrightness))

(fn ConstructionScript)

(fn UpdateBaseBrightness
  (bind _maxbasebrightness (Variables|Default|GetMaxBaseBrightness))
  (Rendering|Material|SetScalarParameterValue (Variables|Materials|GetBaseMaterial) "Brightness" (Math|Float|Clamp(Float) (* (Math|Float|Absolute(Float) (- (Math|Float|%(Float) (/ (Variables|Default|GetTime) 2.0) 2.0) 1.0)) _maxbasebrightness 1.2) 0.3 _maxbasebrightness) :!class /Script/Engine.MaterialInstanceDynamic))

(fn SetLabelVisibility
  (params (bNewVisibility :type Boolean))
  (Rendering|SetVisibility (Variables|Default|GetMark) bNewVisibility false)
  (Rendering|SetVisibility (Variables|Default|GetBase) bNewVisibility false)
  (Rendering|SetVisibility (Variables|Default|GetGoGo) bNewVisibility false)
  (Rendering|SetVisibility (Variables|Default|GetMark1) bNewVisibility false))