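; End-sequence camera that takes over the view on BeginPlay and watches the player's dying location.
; A timeline moves it vertically to a set Z until the player dies.
; It then adds the M_Suiteki post-process material, fades in its parameter, and eases height toward the player's end-camera marker, clamped by that Z, until the player's clear event.
; Tick handles look-at; the Tilt event replaces it with a randomly signed, growing roll.
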(event Custom|HomingLocation
  (bind _returnvalue (Transformation|GetActorLocation))
  (bind _returnvalue_2 (Rendering|Material|CreateDynamicMaterialInstance "/Game/_Users/M_Suiteki.M_Suiteki" "None" :!class /Script/Engine.KismetMaterialLibrary))
  (Variables|Default|SetSuitekiMaterial _returnvalue_2)
  (Rendering|Material|SetScalarParameterValue (Variables|Default|GetSuitekiMaterial) "Val" 0.0 :!class /Script/Engine.MaterialInstanceDynamic)
  (Utilities|FlowControl|Delay 0.3)
  (Utilities|Array|SetArrayElem (.array (Utilities|Struct|BreakPostProcessSettings (Variables|/Script/Engine.CameraComponent|GetPostProcessSettings (Variables|Default|GetCamera)))) 0 (Utilities|Struct|MakeWeightedBlendable 1.0 (Variables|Default|GetSuitekiMaterial)))
  (Utilities|FlowControl|Sequence
    (:then_0
      (Variables|Default|SetAlpha (+ (Variables|Default|GetAlpha) 0.0001) :!label _label)
      (Transformation|SetActorLocation (Math|Vector|Lerp(Vector) (Math|Vector|MakeVector (.x _returnvalue) (.y _returnvalue) (.z _returnvalue)) (Math|Vector|MakeVector (.x _returnvalue) (.y _returnvalue) (Math|Float|Max(Float) (Variables|Default|GetZLocation) (.z (Transformation|GetWorldLocation (Variables|/Game/_Users/Players/Blueprints/BP_Player.BP_Player_C|GetEndCameraZLocation (Variables|Objects|GetPlayer)))))) (Variables|Default|GetAlpha)) false false)
      (Utilities|FlowControl|Delay 0.0)
      (if (not (Variables|Default|GetbEndHoming))
        (goto _label)))
    (:then_1
      (bind _newtrack_0 (Timeline|Timeline_1 Play)
        (:Update
          (Rendering|Material|SetScalarParameterValue (Variables|Default|GetSuitekiMaterial) "Val" (Math|Float|Lerp 0.0 0.02 _newtrack_0) :!class /Script/Engine.MaterialInstanceDynamic))))))

(event Custom|Clear_Event
  (Variables|Default|SetbEndHoming true))

(event Custom|Tilt
  (bind _returnvalue (Transformation|GetActorLocation))
  (bind _player (Variables|Objects|GetPlayer))
  (bind _returnvalue_2 (Transformation|GetActorLocation _player))
  (bind _dyinglocation (Variables|/Game/_Users/Players/Blueprints/BP_Player.BP_Player_C|GetDyingLocation _player))
  (bind _returnvalue_3 (Math|Rotator|FindLookatRotation _returnvalue (Math|Vector|MakeVector (.x _dyinglocation) (.y _dyinglocation) (.z _returnvalue_2))))
  (if (== (Math|Random|RandomInteger 1) 0)
    (Variables|Default|SetTiltRate (- (* (Math|Random|RandomInteger 2) 2) 1))
    (Utilities|FlowControl|Delay 0.7)
    (Variables|Default|SetbIsRotation false)
    (Transformation|SetActorRotation (Math|Rotator|MakeRotator (+ (.roll _returnvalue_3) (* (Variables|Default|GetTiltRate) (Variables|Default|GetTiltValue))) (.pitch _returnvalue_3) (.yaw _returnvalue_3)) :!label _label)
    (Variables|Default|SetTiltValue (Math|Float|Min(Float) (+ (Variables|Default|GetTiltValue) (* (Utilities|Time|GetWorldDeltaSeconds) 1e+02)) 15.0))
    (Utilities|FlowControl|Delay 0.0)
    (goto _label)))

(event EventBeginPlay
  (Game|Player|SetViewTargetwithBlend (Game|GetPlayerController 0) self 0.0 "VTBlend_Linear" 0.0 false)
  (Variables|Objects|SetPlayer (.AsBP%20Player (Utilities|Casting|CastToBP_Player (Game|Player|GetPlayerPawn 0))))
  (Variables|Default|SetStartLocation (Transformation|GetActorLocation))
  (EventDispatchers|BindEventtoClear (Variables|Objects|GetPlayer) (delegate Custom|Clear_Event))
  (bind _newtrack_0 (Timeline|Timeline_0 Play)
    (:Update
      (Transformation|SetActorLocation (Math|Vector|Lerp(Vector) (Variables|Default|GetStartLocation) (Math|Vector|MakeVector (.x (Variables|Default|GetStartLocation)) (.y (Variables|Default|GetStartLocation)) (Variables|Default|GetZLocation)) _newtrack_0) false false)
      (if (not (Variables|Default|GetbStartHoming))
        (if (not (Default|CheckIsAlive (Variables|Objects|GetPlayer)))
          (Variables|Default|SetbStartHoming true)
          (Timeline|Timeline_0 Stop))))
    (:Finished
      (if (not (Variables|Default|GetbStartHoming))
        (if (Default|CheckIsAlive (Variables|Objects|GetPlayer)) :!label _label
          (Utilities|FlowControl|Delay 0.0)
          (goto _label)
          (else
            (Variables|Default|SetbStartHoming true)))))))

(event EventTick
  (params (DeltaSeconds :type Float%20%28single-precision%29))
  (bind _player (Variables|Objects|GetPlayer))
  (bind _dyinglocation (Variables|/Game/_Users/Players/Blueprints/BP_Player.BP_Player_C|GetDyingLocation _player))
  (if (Variables|Default|GetbIsRotation)
    (Transformation|SetActorRotation (Math|Rotator|FindLookatRotation (Transformation|GetActorLocation) (Math|Vector|MakeVector (.x _dyinglocation) (.y _dyinglocation) (.z (Transformation|GetActorLocation _player))))))
  (if (Variables|Default|GetbStartHoming)
    (Utilities|FlowControl|DoOnce false
      (:Completed
        (CallFunction|HomingLocation)))))

(fn ConstructionScript)