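; Title screen manager that acts as the view target and drives the intro camera move, audio and input-driven sway.
; On BeginPlay the camera jumps to BP_InitCameraLocation, then a per-frame Delay loop decays its relative transform toward zero alongside a move sound and delayed jingle.
; Tick turns input into clamped, damped actor rotation and normalized input values.
; GoFlat triggers the title player's surprised animation, while LevelTransition fades or suppresses the jingle.
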(event EventBeginPlay
  (bind _camera (Variables|Default|GetCamera))
  (bind _returnvalue (Transformation|GetRelativeTransform _camera))
  (Game|Player|SetViewTargetwithBlend (Game|GetPlayerController 0) self 0.0 "VTBlend_Linear" 0.0 false)
  (Variables|Default|SetMaxRotaValue (/ (Variables|Default|GetSpeed) (- 1.0 (Variables|Default|GetForce))))
  (if (Variables|/Game/_Users/Blueprints/BP_GameInstance.BP_GameInstance_C|GetbIsReplay (.AsBP%20Game%20Instance (Utilities|Casting|CastToBP_GameInstance (Game|GetGameInstance))))
    _
    (else
      _))
  (bind _outactors (Actor|GetAllActorsOfClass "/Game/_Users/Blueprints/BP_InitCameraLocation.BP_InitCameraLocation_C"))
  (Transformation|SetWorldTransform (Variables|Default|GetCamera) (Math|Transform|MakeTransform (.location (Transformation|GetActorTransform (Utilities|Array|Get(acopy) _outactors))) (.rotation (Transformation|GetActorTransform (Utilities|Array|Get(acopy) _outactors))) "1,1,1") false false)
  (Utilities|FlowControl|Sequence
    (:then_0
      (bind _returnvalue_2 (Audio|SpawnSound2D "/Game/_Users/Sounds/Title/A_TitleMove_Cue.A_TitleMove_Cue" 1.0 0.5 0.5 0))
      (Utilities|FlowControl|Delay 0.5)
      (Audio|Components|Audio|FadeOut _returnvalue_2 1.5 0.0 :!class /Script/Engine.AudioComponent))
    (:then_1
      (Transformation|SetRelativeTransform _camera (Math|Transform|MakeTransform (* (.location _returnvalue) 0.98) (Math|Rotator|MakeRotator (* (.roll (.rotation _returnvalue)) 0.98) (* (.pitch (.rotation _returnvalue)) 0.98) (* (.yaw (.rotation _returnvalue)) 0.98)) "1,1,1") false false :!label _label)
      (Utilities|FlowControl|Delay 0.0)
      (goto _label))
    (:then_2
      (Utilities|FlowControl|Delay 1.5)
      (if (not (Variables|Default|GetbLevelTransition))
        (bind _returnvalue_3 (Audio|SpawnSound2D "/Game/_Users/Sounds/Title/A_TitleJingle_Cue.A_TitleJingle_Cue" 1.0 1.0 0.0 0))
        (Variables|Default|SetTitleJingleSE _returnvalue_3)))))

(event EventTick
  (params (DeltaSeconds :type Float%20%28single-precision%29))
  (bind _maxrotavalue (Variables|Default|GetMaxRotaValue))
  (bind _force (Variables|Default|GetForce))
  (CallFunction|UpdateInput)
  (Variables|Default|SetNowRotation (Math|Rotator|MakeRotator (* (.roll (Variables|Default|GetNowRotation)) _force) (* (.pitch (Variables|Default|GetNowRotation)) _force) (* (.yaw (Variables|Default|GetNowRotation)) _force)))
  (Transformation|SetActorRotation (Variables|Default|GetNowRotation))
  (Variables|Default|SetInputValueX (/ (.pitch (Variables|Default|GetNowRotation)) _maxrotavalue))
  (Variables|Default|SetInputValueY (/ (.yaw (Variables|Default|GetNowRotation)) _maxrotavalue)))

(event Input|ActionEvents|InputActionGoFlat
  (params (Key :type Key%20Structure :default "None"))
  (:Pressed
    (bind _outactors (Actor|GetAllActorsOfClass "/Game/_Users/Blueprints/BP_TitlePlayer.BP_TitlePlayer_C"))
    (Default|UpdateSurprised (.AsABP%20Title%20CSC (Utilities|Casting|CastToABP_TitleCSC (Components|SkeletalMesh|GetAnimInstance (Variables|/Game/_Users/Blueprints/BP_TitlePlayer.BP_TitlePlayer_C|GetSkeletalMesh (Utilities|Array|Get(acopy) _outactors))))))))

(fn ConstructionScript)

(fn UpdateInput
  (LocalVariables|SetX (Math|Float|Clamp(Float) (+ (* (Input|AxisValues|GetMoveForward) -1.0) (Input|AxisValues|GetLookUpRate)) -1.0))
  (LocalVariables|SetY (Math|Float|Clamp(Float) (* (+ (Input|AxisValues|GetMoveRight) (Input|AxisValues|GetTurnRate)) -1.0) -1.0))
  (Variables|Default|SetNowRotation (Math|Rotator|MakeRotator (.roll (Variables|Default|GetNowRotation)) (Math|Float|Clamp(Float) (+ (.pitch (Variables|Default|GetNowRotation)) (* (LocalVariables|GetX) (Variables|Default|GetSpeed))) -1e+01 1e+01) (Math|Float|Clamp(Float) (+ (.yaw (Variables|Default|GetNowRotation)) (* (LocalVariables|GetY) (Variables|Default|GetSpeed))) -2e+01 2e+01))))

(fn LevelTransition
  (bind _titlejinglese (Variables|Default|GetTitleJingleSE))
  (Variables|Default|SetbLevelTransition true)
  (Utilities|IsValid _titlejinglese
    (:Is%20Valid
      (Audio|Components|Audio|FadeOut _titlejinglese 0.5 0.0 :!class /Script/Engine.AudioComponent))))