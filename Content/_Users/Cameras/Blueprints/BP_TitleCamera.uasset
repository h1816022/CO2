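; Title-screen camera actor that takes over the player's view and sways with movement and look input.
; Input adds clamped pitch and yaw that decay each tick by Force, also exposed as values normalized against Speed / (1 - Force).
; The camera component starts at BP_InitCameraLocation and eases back to the actor by shrinking its relative transform each tick.
; GoFlat input triggers the surprised reaction in BP_TitlePlayer's anim instance.
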(event EventBeginPlay
  (Game|Player|SetViewTargetwithBlend (Game|GetPlayerController 0) self 0.0 "VTBlend_Linear" 0.0 false)
  (Variables|Default|SetMaxRotaValue (/ (Variables|Default|GetSpeed) (- 1.0 (Variables|Default|GetForce))))
  (bind _outactors (Actor|GetAllActorsOfClass "/Game/_Users/Blueprints/BP_InitCameraLocation.BP_InitCameraLocation_C"))
  (Transformation|SetWorldTransform (Variables|Default|GetCamera) (Math|Transform|MakeTransform (.location (Transformation|GetActorTransform (Utilities|Array|Get(acopy) _outactors))) (.rotation (Transformation|GetActorTransform (Utilities|Array|Get(acopy) _outactors))) "1,1,1") false false))

(event EventTick
  (params (DeltaSeconds :type Float%20%28single-precision%29))
  (bind _maxrotavalue (Variables|Default|GetMaxRotaValue))
  (bind _camera (Variables|Default|GetCamera))
  (bind _force (Variables|Default|GetForce))
  (bind _returnvalue (Transformation|GetRelativeTransform _camera))
  (CallFunction|UpdateInput)
  (Variables|Default|SetNowRotation (Math|Rotator|MakeRotator (* (.roll (Variables|Default|GetNowRotation)) _force) (* (.pitch (Variables|Default|GetNowRotation)) _force) (* (.yaw (Variables|Default|GetNowRotation)) _force)))
  (Transformation|SetActorRotation (Variables|Default|GetNowRotation))
  (Variables|Default|SetInputValueX (/ (.pitch (Variables|Default|GetNowRotation)) _maxrotavalue))
  (Variables|Default|SetInputValueY (/ (.yaw (Variables|Default|GetNowRotation)) _maxrotavalue))
  (Transformation|SetRelativeTransform _camera (Math|Transform|MakeTransform (* (.location _returnvalue) 0.98) (Math|Rotator|MakeRotator (* (.roll (.rotation _returnvalue)) 0.98) (* (.pitch (.rotation _returnvalue)) 0.98) (* (.yaw (.rotation _returnvalue)) 0.98)) "1,1,1") false false))

(event Input|ActionEvents|InputActionGoFlat
  (params (Key :type Key%20Structure))
  (:Pressed
    (bind _outactors (Actor|GetAllActorsOfClass "/Game/_Users/Blueprints/BP_TitlePlayer.BP_TitlePlayer_C"))
    (Default|UpdateSurprised (.AsABP%20Title%20CSC (Utilities|Casting|CastToABP_TitleCSC (Components|SkeletalMesh|GetAnimInstance (Variables|/Game/_Users/Blueprints/BP_TitlePlayer.BP_TitlePlayer_C|GetSkeletalMesh (Utilities|Array|Get(acopy) _outactors))))))))

(fn ConstructionScript)

(fn UpdateInput
  (LocalVariables|SetX (Math|Float|Clamp(Float) (+ (* (Input|AxisValues|GetMoveForward) -1.0) (Input|AxisValues|GetLookUpRate)) -1.0))
  (LocalVariables|SetY (Math|Float|Clamp(Float) (* (+ (Input|AxisValues|GetMoveRight) (Input|AxisValues|GetTurnRate)) -1.0) -1.0))
  (Variables|Default|SetNowRotation (Math|Rotator|MakeRotator (.roll (Variables|Default|GetNowRotation)) (Math|Float|Clamp(Float) (+ (.pitch (Variables|Default|GetNowRotation)) (* (LocalVariables|GetX) (Variables|Default|GetSpeed))) -1e+01 1e+01) (Math|Float|Clamp(Float) (+ (.yaw (Variables|Default|GetNowRotation)) (* (LocalVariables|GetY) (Variables|Default|GetSpeed))) -2e+01 2e+01))))