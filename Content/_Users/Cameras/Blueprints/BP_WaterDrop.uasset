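; BP_WaterDrop is an actor made of glass-blur planes, apparently a water-drop effect that fades over time.
; On BeginPlay it creates a dynamic instance of MI_GlassBlurry for each of its nine planes and collects them in an array.
; Each Tick, OpacityUpdate lowers a shared Value by delta time and writes it to every material's Rate parameter, stopping once Value nears zero.
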(event EventBeginPlay
  (bind _returnvalue (Rendering|Material|CreateDynamicMaterialInstance (Variables|Default|GetPlane) 0 "/Game/Raindrops/MI_GlassBlurry.MI_GlassBlurry" "None" :!class /Script/Engine.PrimitiveComponent))
  (Utilities|Array|Add (Variables|Default|GetMaterials) _returnvalue)
  (bind _returnvalue_2 (Rendering|Material|CreateDynamicMaterialInstance (Variables|Default|GetPlane1) 0 "/Game/Raindrops/MI_GlassBlurry.MI_GlassBlurry" "None" :!class /Script/Engine.PrimitiveComponent))
  (Utilities|Array|Add (Variables|Default|GetMaterials) _returnvalue_2)
  (bind _returnvalue_3 (Rendering|Material|CreateDynamicMaterialInstance (Variables|Default|GetPlane2) 0 "/Game/Raindrops/MI_GlassBlurry.MI_GlassBlurry" "None" :!class /Script/Engine.PrimitiveComponent))
  (Utilities|Array|Add (Variables|Default|GetMaterials) _returnvalue_3)
  (bind _returnvalue_4 (Rendering|Material|CreateDynamicMaterialInstance (Variables|Default|GetPlane3) 0 "/Game/Raindrops/MI_GlassBlurry.MI_GlassBlurry" "None" :!class /Script/Engine.PrimitiveComponent))
  (Utilities|Array|Add (Variables|Default|GetMaterials) _returnvalue_4)
  (bind _returnvalue_5 (Rendering|Material|CreateDynamicMaterialInstance (Variables|Default|GetPlane4) 0 "/Game/Raindrops/MI_GlassBlurry.MI_GlassBlurry" "None" :!class /Script/Engine.PrimitiveComponent))
  (Utilities|Array|Add (Variables|Default|GetMaterials) _returnvalue_5)
  (bind _returnvalue_6 (Rendering|Material|CreateDynamicMaterialInstance (Variables|Default|GetPlane5) 0 "/Game/Raindrops/MI_GlassBlurry.MI_GlassBlurry" "None" :!class /Script/Engine.PrimitiveComponent))
  (Utilities|Array|Add (Variables|Default|GetMaterials) _returnvalue_6)
  (bind _returnvalue_7 (Rendering|Material|CreateDynamicMaterialInstance (Variables|Default|GetPlane6) 0 "/Game/Raindrops/MI_GlassBlurry.MI_GlassBlurry" "None" :!class /Script/Engine.PrimitiveComponent))
  (Utilities|Array|Add (Variables|Default|GetMaterials) _returnvalue_7)
  (bind _returnvalue_8 (Rendering|Material|CreateDynamicMaterialInstance (Variables|Default|GetPlane7) 0 "/Game/Raindrops/MI_GlassBlurry.MI_GlassBlurry" "None" :!class /Script/Engine.PrimitiveComponent))
  (Utilities|Array|Add (Variables|Default|GetMaterials) _returnvalue_8)
  (bind _returnvalue_9 (Rendering|Material|CreateDynamicMaterialInstance (Variables|Default|GetPlane8) 0 "/Game/Raindrops/MI_GlassBlurry.MI_GlassBlurry" "None" :!class /Script/Engine.PrimitiveComponent))
  (Utilities|Array|Add (Variables|Default|GetMaterials) _returnvalue_9))

(event EventTick
  (params (DeltaSeconds :type Float%20%28single-precision%29))
  (if (not (<= (Variables|Default|GetValue) 0.05))
    (CallFunction|OpacityUpdate DeltaSeconds)))

(fn ConstructionScript)

(fn OpacityUpdate
  (params (Rate :type Float%20%28single-precision%29))
  (bind _output_get (Variables|Default|SetValue (- (Variables|Default|GetValue) (/ Rate 1.0))))
  (for _array_element (Variables|Default|GetMaterials)
    (Rendering|Material|SetScalarParameterValue _array_element "Rate" _output_get :!class /Script/Engine.MaterialInstanceDynamic)))