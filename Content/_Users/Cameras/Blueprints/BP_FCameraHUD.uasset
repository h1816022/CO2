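; BP_FCameraHUD is a camera HUD that shows a pressure readout derived from a bottle's hit points.
; On BeginPlay it creates a dynamic instance of MI_FCameraHUD on Base, then refreshes every 0.05 seconds with 100 minus the bottle's current hit points.
; UpdatePRateMaterial splits the value into digits and assigns a digit texture per place to material parameters, using a black texture to blank leading zeros.
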(event Custom|UpdatePressureRate
  (CallFunction|UpdatePRateMaterial (- 1e+02 (Variables|/Game/_Users/Players/Bottle/Blueprints/BP_Bottle.BP_Bottle_C|GetNowHitPoint (Variables|Default|GetBottle))) :!label _label)
  (Utilities|FlowControl|Delay 0.05)
  (goto _label))

(event EventBeginPlay
  (bind _returnvalue (Rendering|Material|CreateDynamicMaterialInstance (Variables|Default|GetBase) 0 "/Game/_Users/Cameras/Materials/MI_FCameraHUD.MI_FCameraHUD" "None" :!class /Script/Engine.PrimitiveComponent))
  (Variables|Default|SetMaterial _returnvalue)
  (CallFunction|UpdatePressureRate))

(fn ConstructionScript)

(fn UpdatePRateMaterial
  (params (InNum :type Float%20%28single-precision%29))
  (bind _output_get (LocalVariables|SetNum InNum))
  (if (> _output_get 99.0)
    (LocalVariables|SetPHundreds (Variables|Default|GetHundredsPlace))
    (else
      (LocalVariables|SetPHundreds "/Game/_Users/Textures/T_Black.T_Black")))
  (if (== (LocalVariables|GetNum) 1e+02)
    (LocalVariables|SetPTens (Utilities|Array|Get(acopy) (Variables|Default|GetTensPlace)))
    (LocalVariables|SetPOnes (Utilities|Array|Get(acopy) (Variables|Default|GetOnesPlace)))
    (else
      (if (== (Math|Float|Truncate (/ (LocalVariables|GetNum) 1e+01)) 0)
        (LocalVariables|SetPTens "/Game/_Users/Textures/T_Black.T_Black")
        (else
          (LocalVariables|SetPTens (Utilities|Array|Get(acopy) (Variables|Default|GetTensPlace) (Math|Float|Truncate (/ (LocalVariables|GetNum) 1e+01))))))
      (LocalVariables|SetPOnes (Utilities|Array|Get(acopy) (Variables|Default|GetOnesPlace) (Math|Float|Truncate (Math|Float|%(Float) (LocalVariables|GetNum) 1e+01))))))
  (Rendering|Material|SetTextureParameterValue (Variables|Default|GetMaterial) "PressureOnes" (LocalVariables|GetPOnes))
  (Rendering|Material|SetTextureParameterValue (Variables|Default|GetMaterial) "PressureTens" (LocalVariables|GetPTens))
  (Rendering|Material|SetTextureParameterValue (Variables|Default|GetMaterial) "PressureHudredss" (LocalVariables|GetPHundreds)))