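; BP_MiniMapCamera is a camera actor for a minimap that can aim at the MiniMap actor and toggle between two zoom positions.
; UpdateRotation turns it toward the MiniMap root using a look-at rotation.
; BeginPlay caches the start location and a short forward offset from the initial rotation.
; Zoom alternates playing and reversing a timeline that lerps between these positions, ignoring calls until the move finishes.
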(event Custom|UpdateRotation
  (Transformation|SetActorRotation (Math|Rotator|FindLookatRotation (Transformation|GetActorLocation) (Transformation|GetWorldLocation (Variables|/Script/Engine.Actor|GetRootComponent (Variables|Default|GetMiniMap))))))

(event Custom|Zoom
  (bind _defaultlocation (Variables|Default|GetDefaultLocation))
  (if (Variables|Default|GetbCanZoom)
    (Variables|Default|SetbCanZoom false)
    (Utilities|FlowControl|FlipFlop
      (:A
        (bind _newtrack_0 (Timeline|Timeline_0 PlayFromStart)
          (:Update
            (Transformation|SetActorLocation (Math|Vector|Lerp(Vector) _defaultlocation (+ _defaultlocation (Variables|Default|GetZoomOffset)) _newtrack_0) false false))
          (:Finished
            (Variables|Default|SetbCanZoom true))))
      (:B
        (Timeline|Timeline_0 ReverseFromEnd)))))

(event EventBeginPlay
  (Variables|Default|SetDefaultLocation (Transformation|GetActorLocation))
  (Variables|Default|SetZoomOffset (* (Math|Rotator|GetRotationXVector (Transformation|GetActorRotation)) 1e+01)))

(fn ConstructionScript)