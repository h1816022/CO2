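; Connectable actor that hands itself to BP_Player for connection when the player overlaps its collision while it is active and accepting.
; Re-accepting waits a second after overlap ends; Connection runs ConnectionProc, which ends the anim squat, then deactivates one-use actors.
; Endless Delay loops drive cues while available: a smoothed light-pillar alpha that grows with player distance, and periodically spawned aura emitters.
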(event OnComponentBeginOverlap(AcceptCollision)
  (params (OverlappedComponent :type Primitive%20Component%20Object%20Reference) (OtherActor :type Actor%20Object%20Reference) (OtherComp :type Primitive%20Component%20Object%20Reference) (OtherBodyIndex :type Integer) (bFromSweep :type Boolean) (SweepResult :type Hit%20Result%20Structure%20%28by%20ref%29))
  (if (Variables|Default|GetbIsActive)
    (if (Variables|Default|GetbCanAccept)
      (bind _asbp_player (Utilities|Casting|CastToBP_Player OtherActor))
      (Variables|Default|SetPlayer _asbp_player)
      (Default|PrepConnection (Variables|Default|GetPlayer) self)
      (Variables|Default|SetbCanAccept false))))

(event OnComponentEndOverlap(AcceptCollision)
  (params (OverlappedComponent :type Primitive%20Component%20Object%20Reference) (OtherActor :type Actor%20Object%20Reference) (OtherComp :type Primitive%20Component%20Object%20Reference) (OtherBodyIndex :type Integer))
  (Utilities|Casting|CastToBP_Player OtherActor)
  (Utilities|FlowControl|Delay 1.0)
  (Variables|Default|SetbCanAccept true))

(event Custom|Connection
  (params (AnimBlueprint :type ABP%20CSC%20Object%20Reference))
  (CallFunction|ConnectionProc AnimBlueprint)
  (if (Variables|Default|GetbIsOnce)
    (CallFunction|SetActivate false)))

(event Custom|UpdateParticle
  (Utilities|FlowControl|Sequence
    (:then_0
      (Utilities|FlowControl|Delay 2.0 :!label _label)
      (if (and (Variables|Default|GetbCanAccept) (Variables|Default|GetbIsActive))
        (Variables|Default|SetTargetAlpha (CallFunction|CalculatePillarAlpha))
        (goto _label)
        (else
          (Variables|Default|SetTargetAlpha 0.0)
          (Variables|Default|SetNowAlpha 0.0)
          (goto _label))))
    (:then_1
      (Variables|Default|SetNowAlpha (Math|Float|Lerp (Variables|Default|GetNowAlpha) (Variables|Default|GetTargetAlpha) 0.05) :!label _label_2)
      (Effects|Components|ParticleSystem|SetFloatParameter (Variables|Default|GetP_Pillar) "Alpha" (Variables|Default|GetNowAlpha))
      (Utilities|FlowControl|Delay 0.0)
      (goto _label_2))
    (:then_2
      (Utilities|FlowControl|Delay 0.5 :!label _label_3)
      (if (and (Variables|Default|GetbCanAccept) (Variables|Default|GetbIsActive))
        (bind _returnvalue (Effects|SpawnEmitteratLocation (Variables|Default|GetAura) (Transformation|GetWorldLocation (Variables|Default|GetConnectLocation))))
        (Effects|Components|ParticleSystem|SetVectorParameter _returnvalue "Velocity" (Math|Vector|MakeVector 0.0 0.0 (* (Variables|Default|GetAuraVelocity) (Variables|Default|GetAuraParamRate))))
        (Effects|Components|ParticleSystem|SetFloatParameter _returnvalue "Num" (* (Variables|Default|GetAuraNum) (Variables|Default|GetAuraParamRate)))
        (Effects|Components|ParticleSystem|SetFloatParameter _returnvalue "Size" (* (Variables|Default|GetAuraSize) (Variables|Default|GetAuraParamRate)))
        (goto _label_3)
        (else
          (goto _label_3))))))

(event Custom|ConnectionProc
  (params (AnimBlueprint :type ABP%20CSC%20Object%20Reference))
  (Default|EndSquat AnimBlueprint))

(event EventBeginPlay
  (CallFunction|UpdateParticle))

(fn ConstructionScript)

(fn CalculatePillarAlpha
  (bind _output_get (LocalVariables|SetLength (Math|Vector|VectorLength (- (Transformation|GetActorLocation) (Transformation|GetActorLocation (Game|Player|GetPlayerPawn 0))))))
  (if (< _output_get (Variables|Default|GetMinPillarLength))
    (LocalVariables|SetReturn 0.0)
    (else
      (LocalVariables|SetReturn (Math|Float|Clamp(Float) (- (/ (LocalVariables|GetLength) (Variables|Default|GetMaxPillarLength)) 0.1) 0.0 0.2))))
  (return (LocalVariables|GetReturn)))