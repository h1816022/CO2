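; BP_WaterSupplyDevice is a connectable actor that adds liquid to the player's bottle.
; On BeginPlay, it derives an aura parameter rate from its refill amount, scaled and clamped to a fixed range.
; Its ConnectionProc event adds that refill amount to the bottle, waits briefly, then ends the squat on the supplied AnimBlueprint.
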(event EventBeginPlay
  (|CallParentFunction)
  (Variables|Default|SetAuraParamRate (Math|Float|Clamp(Float) (* (Variables|Default|GetRateAmount) 5.0) 1.0 3.0)))

(event EventConnectionProc
  (params (AnimBlueprint :type ABP%20CSC%20Object%20Reference))
  (Default|AddLiquidRate (Variables|/Game/_Users/Players/Blueprints/BP_Player.BP_Player_C|GetBottle (Variables|Default|GetPlayer)) (Variables|Default|GetRateAmount))
  (Utilities|FlowControl|Delay 1.0)
  (Default|EndSquat AnimBlueprint))

(fn ConstructionScript
  (|CallParentFunction))