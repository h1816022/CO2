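; BP_Bottle is a bottle actor that acts as the player's health display, creating its own widget and hiding in first-person camera.
; Tick drains hit points by movement input, faster while dashing, and shake or direct damage also reduces them.
; Dynamic materials show the loss through mask, head and emissive opacity.
; At zero it calls dying, then after the player's delay lowers the CO2-driven liquid fill until it calls dead.
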(event Custom|InitFirstCamera
  (Rendering|SetActorHiddenInGame true))

(event Custom|InitThirdCamera
  (Rendering|SetActorHiddenInGame false))

(event Custom|Dying_Event
  (Utilities|FlowControl|Delay (Variables|/Game/_Users/Players/Blueprints/BP_Player.BP_Player_C|GetDyingDelay (Variables|Default|GetPlayer)))
  (bind _bisfinish (CallFunction|UpdateCO2Rate :!label _label))
  (if (not _bisfinish)
    (Utilities|FlowControl|Delay 0.0)
    (goto _label)
    (else
      (Default|CallDead))))

(event Custom|Dead_Event)

(event EventBeginPlay
  (bind _returnvalue (Game|Player|GetPlayerPawn 0))
  (bind _asbp_player (Utilities|Casting|CastToBP_Player _returnvalue))
  (bind _camera (Variables|/Game/_Users/Players/Blueprints/BP_Player.BP_Player_C|GetCamera _asbp_player))
  (CallFunction|InitVariables)
  (EventDispatchers|BindEventtoSetFirstCamera _camera (delegate Custom|InitFirstCamera))
  (EventDispatchers|BindEventtoSetThirdCamera _camera (delegate Custom|InitThirdCamera))
  (EventDispatchers|BindEventtoDying (delegate Custom|Dying_Event))
  (EventDispatchers|BindEventtoDead (delegate Custom|Dead_Event))
  (bind _returnvalue_2 (UserInterface|CreateWidget "/Game/_Users/Players/Widget/WBP_Bottle.WBP_Bottle_C"))
  (Variables|/Game/_Users/Players/Widget/WBP_Bottle.WBP_Bottle_C|SetOwner _returnvalue_2 self)
  (UserInterface|Viewport|AddtoViewport _returnvalue_2 0))

(event EventTick
  (params (DeltaSeconds :type Float%20%28single-precision%29))
  (if (CallFunction|CheckHitPoint)
    (bind _bisalive (CallFunction|UpdateHitPoint DeltaSeconds))
    (if (not _bisalive)
      (Default|CallDying))))

(fn ConstructionScript)

(fn InitVariables
  (Utilities|FlowControl|Sequence
    (:then_0
      (bind _returnvalue (Rendering|Material|CreateDynamicMaterialInstance (Variables|Default|GetLiquid) 1 "/Game/RealLiquidX/M/MI_LiquidX_03.MI_LiquidX_03" "None" :!class /Script/Engine.PrimitiveComponent))
      (Variables|Default|SetLiquidMat _returnvalue)
      (bind _returnvalue_2 (Rendering|Material|CreateDynamicMaterialInstance (Variables|Default|GetHead) 0 "/Game/_Users/Bottle/Materials/MI_LGTBaseColor.MI_LGTBaseColor" "None" :!class /Script/Engine.PrimitiveComponent))
      (Utilities|Array|Add (Variables|Default|GetHeadMats) _returnvalue_2)
      (bind _returnvalue_3 (Rendering|Material|CreateDynamicMaterialInstance (Variables|Default|GetHead4) 0 "/Game/_Users/Bottle/Materials/MI_LGTBaseColor.MI_LGTBaseColor" "None" :!class /Script/Engine.PrimitiveComponent))
      (Utilities|Array|Add (Variables|Default|GetHeadMats) _returnvalue_3)
      (bind _returnvalue_4 (Rendering|Material|CreateDynamicMaterialInstance (Variables|Default|GetBottleMask) 1 "/Game/_Users/Bottle/Materials/MI_BottleMask.MI_BottleMask" "None" :!class /Script/Engine.PrimitiveComponent))
      (Variables|Default|SetBottleMaskMat _returnvalue_4)
      (bind _returnvalue_5 (Rendering|Material|CreateDynamicMaterialInstance (Variables|Default|GetEmissiveLight1) 0 "/Game/_Users/Bottle/Materials/MI_LGTEmissive.MI_LGTEmissive" "None" :!class /Script/Engine.PrimitiveComponent))
      (Utilities|Array|Add (Variables|Default|GetEmissiveLightMats) _returnvalue_5)
      (bind _returnvalue_6 (Rendering|Material|CreateDynamicMaterialInstance (Variables|Default|GetEmissiveLight2) 0 "/Game/_Users/Bottle/Materials/MI_LGTEmissive.MI_LGTEmissive" "None" :!class /Script/Engine.PrimitiveComponent))
      (Utilities|Array|Add (Variables|Default|GetEmissiveLightMats) _returnvalue_6)
      (bind _returnvalue_7 (Rendering|Material|CreateDynamicMaterialInstance (Variables|Default|GetEmissiveLight3) 0 "/Game/_Users/Bottle/Materials/MI_LGTEmissive.MI_LGTEmissive" "None" :!class /Script/Engine.PrimitiveComponent))
      (Utilities|Array|Add (Variables|Default|GetEmissiveLightMats) _returnvalue_7))
    (:then_1
      (Variables|Default|SetNowHitPoint (Variables|Default|GetMaxHItPoint))
      (Variables|Default|SetPlayer (.AsBP%20Player (Utilities|Casting|CastToBP_Player (Game|Player|GetPlayerPawn 0)))))))

(fn ClampHItPoint
  (Variables|Default|SetNowHitPoint (Math|Float|Clamp(Float) (Variables|Default|GetNowHitPoint) 0.0 (Variables|Default|GetMaxHItPoint))))

(fn CheckHitPoint
  (return (> (Variables|Default|GetNowHitPoint) 0.0)))

(fn UpdateHitPoint
  (params (DeltaSeconds :type Float%20%28single-precision%29))
  (if (Variables|/Game/_Users/Players/Blueprints/BP_Player.BP_Player_C|GetbIsDash (Variables|Default|GetPlayer))
    (Variables|Default|SetNowHitPoint (- (Variables|Default|GetNowHitPoint) (* DeltaSeconds (Variables|Default|GetContinuousDamage) 5.0)))
    (else
      (Variables|Default|SetNowHitPoint (- (Variables|Default|GetNowHitPoint) (* DeltaSeconds (Variables|Default|GetContinuousDamage) (Math|Vector|VectorLength (Variables|/Game/_Users/Players/Blueprints/BP_Player.BP_Player_C|GetInputVec (Variables|Default|GetPlayer))))))))
  (Rendering|Material|SetScalarParameterValue (Variables|Default|GetBottleMaskMat) "Opacity" (Math|Float|Min(Float) (- 1.0 (Math|Float|Clamp(Float) (/ (Variables|Default|GetNowHitPoint) (Variables|Default|GetMaxHItPoint)))) 0.98) :!class /Script/Engine.MaterialInstanceDynamic)
  (for _array_element (Variables|Default|GetHeadMats)
    (Rendering|Material|SetScalarParameterValue _array_element "Opacity" (Math|Float|Clamp(Float) (/ (Variables|Default|GetNowHitPoint) (/ (Variables|Default|GetMaxHItPoint) 15.0))) :!class /Script/Engine.MaterialInstanceDynamic))
  (for _array_element_2 (Variables|Default|GetEmissiveLightMats)
    (Rendering|Material|SetScalarParameterValue _array_element_2 "Opacity" (- 1.0 (Math|Float|Clamp(Float) (/ (Variables|Default|GetNowHitPoint) (/ (Variables|Default|GetMaxHItPoint) 15.0)))) :!class /Script/Engine.MaterialInstanceDynamic))
  (Rendering|SetVisibility (Variables|Default|GetEmissiveLight2) true false)
  (Rendering|SetVisibility (Variables|Default|GetEmissiveLight3) true false)
  (return (CallFunction|CheckHitPoint)))

(fn UpdateCO2Rate
  (Variables|Default|SetCO2Rate (- (Variables|Default|GetCO2Rate) (CallFunction|GetMulDeltaSeconds 0.5)))
  (if (<= (Variables|Default|GetCO2Rate) 0.0)
    (Variables|Default|SetCO2Rate 0.0))
  (Rendering|Material|SetScalarParameterValue (Variables|Default|GetLiquidMat) "Liquid_FillHeight" (Math|Float|Lerp -0.5 0.15 (Variables|Default|GetCO2Rate)) :!class /Script/Engine.MaterialInstanceDynamic)
  (return (<= (Variables|Default|GetCO2Rate) 0.0)))

(fn AddShakeDamage
  (if (>= (Variables|Default|GetNowHitPoint) (+ (Variables|Default|GetShakeDamage) 1.0))
    (CallFunction|AddDamage (Variables|Default|GetShakeDamage))))

(fn AddDamage
  (params (InDamage :type Float%20%28single-precision%29))
  (Variables|Default|SetNowHitPoint (- (Variables|Default|GetNowHitPoint) InDamage))
  (CallFunction|ClampHItPoint))

(fn GetMulDeltaSeconds
  (params (Rate :type Float%20%28single-precision%29))
  (return (* Rate (Utilities|Time|GetWorldDeltaSeconds))))