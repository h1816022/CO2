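; Destructible double door in the BallisticsVFX demo map that records when the player's world gets wrecked.
; When either leaf fractures, it flags that side as broken and increments AssholeRating and DoorsDestroyed on the rifle first-person character.
; Slide open and close logic moves unbroken leaves with MoveComponentTo, polling per-side in-motion flags through delays, but no event triggers it.
; The construction script resets both broken flags.
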(event OnComponentFracture(SM_Door_DM_left)
  (bind _output_get (Variables|Default|SetLeft%20Door%20Is%20broken! true))
  (if _output_get
    (bind _asfirst_person_character_rifle_2 (Utilities|Casting|CastToFirstPersonCharacter_rifle_2 (Game|GetPlayerCharacter 0)))
    (Variables|/Game/BallisticsVFX/FirstPersonBPExamples/FirstPersonCharacter_rifle_2.FirstPersonCharacter_rifle_2_C|SetAssholeRating _asfirst_person_character_rifle_2 (+ (Variables|/Game/BallisticsVFX/FirstPersonBPExamples/FirstPersonCharacter_rifle_2.FirstPersonCharacter_rifle_2_C|GetAssholeRating _asfirst_person_character_rifle_2) 1.0))
    (Variables|/Game/BallisticsVFX/FirstPersonBPExamples/FirstPersonCharacter_rifle_2.FirstPersonCharacter_rifle_2_C|SetDoors%20Destroyed? _asfirst_person_character_rifle_2 (+ (Variables|/Game/BallisticsVFX/FirstPersonBPExamples/FirstPersonCharacter_rifle_2.FirstPersonCharacter_rifle_2_C|GetDoors%20Destroyed? _asfirst_person_character_rifle_2) 1.0))))

(event OnComponentFracture(SM_Door_DM_right)
  (bind _output_get (Variables|Default|SetRight%20Door%20Is%20broken! true))
  (if _output_get
    (bind _asfirst_person_character_rifle_2 (Utilities|Casting|CastToFirstPersonCharacter_rifle_2 (Game|GetPlayerCharacter 0)))
    (Variables|/Game/BallisticsVFX/FirstPersonBPExamples/FirstPersonCharacter_rifle_2.FirstPersonCharacter_rifle_2_C|SetAssholeRating _asfirst_person_character_rifle_2 (+ (Variables|/Game/BallisticsVFX/FirstPersonBPExamples/FirstPersonCharacter_rifle_2.FirstPersonCharacter_rifle_2_C|GetAssholeRating _asfirst_person_character_rifle_2) 1.0))
    (Variables|/Game/BallisticsVFX/FirstPersonBPExamples/FirstPersonCharacter_rifle_2.FirstPersonCharacter_rifle_2_C|SetDoors%20Destroyed? _asfirst_person_character_rifle_2 (+ (Variables|/Game/BallisticsVFX/FirstPersonBPExamples/FirstPersonCharacter_rifle_2.FirstPersonCharacter_rifle_2_C|GetDoors%20Destroyed? _asfirst_person_character_rifle_2) 1.0))))

(event EventActorBeginOverlap
  (params (OtherActor :type Actor%20Object%20Reference)))

(event EventTick
  (params (DeltaSeconds :type Float%20%28single-precision%29)))

(fn ConstructionScript
  (Variables|Default|SetLeft%20Door%20Is%20broken! false)
  (Variables|Default|SetRight%20Door%20Is%20broken! false))